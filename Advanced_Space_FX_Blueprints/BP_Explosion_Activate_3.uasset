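; Demo actor that triggers a medium space explosion effect and sound when the V key is pressed.
; BeginPlay enables input from player controller 0.
; Pressing V spawns a non-auto-activating Niagara system attached to ExplosionFx, activates ExplosionFx itself with a reset, and plays a large explosion cue at its location.
; Releasing V deactivates ExplosionFx after a brief delay.
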(event `self.ReceiveBeginPlay`
  (`self.EnableInput` (`GameplayStatics.GetPlayerController` 0)))

(event `Key|V`
  (params (Key :type "Key Structure"))
  (bind _explosion_fx (`self.Explosion_Fx`))
  (:`Pressed`
    (`NiagaraFunctionLibrary.SpawnSystemAttached` "/Game/Advanced_Space_Fx_Pack1/FX/Medium_Explosions/NS_Medium_Explosion_2.NS_Medium_Explosion_2" _explosion_fx "None" (0.0 0.0 0.0) (struct) "KeepRelativeOffset" true false)
    (if true
      (`ActorComponent.Activate` _explosion_fx true)
      (`GameplayStatics.PlaySoundAtLocation` "/Game/Advanced_Space_Fx_Pack1/Sources/Sounds/Explosion_Sounds/Sound_Cue/SW_Explosion_Large_Scale_03_Cue.SW_Explosion_Large_Scale_03_Cue" (`SceneComponent.K2_GetComponentLocation` _explosion_fx) (struct) 1.0 1.0 0.0 null null null)))
  (:`Released`
    (`KismetSystemLibrary.Delay` 0.02)
    (`ActorComponent.Deactivate` _explosion_fx)))

(fn `UserConstructionScript`)