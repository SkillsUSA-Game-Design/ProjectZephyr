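; BP_TargetPawn is a destructible moving target pawn, either friendly with its own material or tagged as an enemy.
; Construction sets walk speed, optionally randomized; on BeginPlay it uses AIMoveTo to head for the MoveTo actor, while Tick yaws its mesh toward LookAtLocation.
; Move completion or failure, Event_Kill, or damage arriving once Health is negative all feed one DoOnce that spawns an explosion and destroys it.
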(event `self.ReceiveTick`
  (params (DeltaSeconds :type "Float (single-precision)"))
  (bind _staticmesh (`self.StaticMesh`))
  ;[1 1 1] Make the Target Look at the center of the map
  (`SceneComponent.K2_SetWorldRotation` _staticmesh (`KismetMathLibrary.MakeRotator` (.roll (`SceneComponent.K2_GetComponentRotation` (`self.Mesh`))) (.pitch (`SceneComponent.K2_GetComponentRotation` (`self.Mesh`))) (.yaw (`KismetMathLibrary.FindLookAtRotation` (`SceneComponent.K2_GetComponentLocation` _staticmesh) (`self.LookAtLocation`)))) false false))

(event `self.ReceiveBeginPlay`
  (`|AIMoveTo` self (`self.K2_GetActorLocation` (`self.MoveTo`)) null 50.0 true
    (:`OnSuccess`
      _)
    (:`OnFail`
      _))
  (`/Engine/EditorBlueprintResources/StandardMacros.DoOnce` false :!label _label
    (:`Completed`
      (bind _returnvalue (`GameplayStatics.SpawnEmitterAtLocation` "/Game/ZEPHYR/TurretPack/Effects/P_Explosion_M.P_Explosion_M" (`SceneComponent.K2_GetComponentLocation` (`self.StaticMesh`))))
      (`SceneComponent.K2_DetachFromComponent` _returnvalue "KeepWorld" "KeepWorld" "KeepWorld" true)
      (`self.SetActorHiddenInGame` true)
      (`self.K2_DestroyActor`))))

(event `Event_Kill`
  (goto _label))

(event `self.ReceiveAnyDamage`
  (params (Damage :type "Float (single-precision)") (DamageType :type "DamageType Object Reference") (InstigatedBy :type "Controller Object Reference") (DamageCauser :type "Actor Object Reference"))
  (bind _health (`self.Health`))
  (if (>= _health 0.0)
    (set `self.Health` (- _health Damage))
    (else
      (goto _label))))

(fn `UserConstructionScript`
  (bind _speed (`self.Speed`))
  (set `CharacterMovementComponent.MaxWalkSpeed` (`KismetMathLibrary.SelectFloat` (`KismetMathLibrary.RandomFloatInRange` (* _speed 0.75) (* _speed 2.0)) _speed (`self.Random Speed?`)) (`self.CharacterMovement`))
  (if (`self.Friendly`)
    (`PrimitiveComponent.SetMaterial` (`self.StaticMesh`) 0 "/Game/ZEPHYR/TurretPack/Materials/Environment/MI_Target_Friendly.MI_Target_Friendly")
    (else
      (set `self.Tags` (`self.EnemyTag`)))))