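; Electricity effect actor from a lightning pack that shows arcs with a spinning Torus mesh.
; Tick adds a small fixed local rotation to the torus every frame, independent of delta time.
; After an initial FirstDelay on BeginPlay, a self-calling event endlessly switches the Arcs component on and off, using delays to time the active and idle phases.
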(event `self.ReceiveTick`
  (params (DeltaSeconds :type "Float (single-precision)"))
  (`SceneComponent.K2_AddLocalRotation` (`self.Torus`) (struct :`Pitch` 0.5 :`Yaw` 0.25 :`Roll` 0.75) false false))

(event `Again`
  (`ActorComponent.Activate` (`self.Arcs`) false :!label _label)
  (`KismetSystemLibrary.Delay` 4.0)
  (`ActorComponent.Deactivate` (`self.Arcs`))
  (`KismetSystemLibrary.Delay` 4.5)
  (`self.Again`))

(event `self.ReceiveBeginPlay`
  (`KismetSystemLibrary.Delay` (`self.FirstDelay`))
  (goto _label))

(fn `UserConstructionScript`)