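; BP_LightningTrail_v1_4 is an actor that plays a looping lightning trail effect through three flash trail Niagara components.
; After a short delay on BeginPlay, it activates the trails at full Deactivate_Scale and holds them.
; A timeline then drives that parameter to fade and deactivate them, while a parallel delay restarts the cycle.
; A movement timeline for offsetting and rotating the actor from its start location exists but is never run.
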(event `Again`
  ;[1 1 1] Activate
  (`ActorComponent.Activate` (`self.FlashTrail`) false :!label _label)
  (`ActorComponent.Activate` (`self.FlashTrail_02`) false)
  (`ActorComponent.Activate` (`self.FlashTrail_StM`) false)
  (`FXSystemComponent.SetFloatParameter` (`self.FlashTrail`) "User.Deactivate_Scale" 1.0)
  (`FXSystemComponent.SetFloatParameter` (`self.FlashTrail_02`) "User.Deactivate_Scale" 1.0)
  (`FXSystemComponent.SetFloatParameter` (`self.FlashTrail_StM`) "User.Deactivate_Scale" 1.0)
  (`KismetSystemLibrary.Delay` 4.0)
  (`|ExecutionSequence`
    (:`then_0`
      (`KismetSystemLibrary.Delay` 2.0)
      (`self.Again`))
    (:`then_1`
      ;[1 1 1] Deactivate
      (bind (_direction _scale) (`Timeline|Deactivate` :!via `PlayFromStart`)
        (:`Update`
          (`FXSystemComponent.SetFloatParameter` (`self.FlashTrail`) "User.Deactivate_Scale" _scale)
          (`FXSystemComponent.SetFloatParameter` (`self.FlashTrail_02`) "User.Deactivate_Scale" _scale)
          (`FXSystemComponent.SetFloatParameter` (`self.FlashTrail_StM`) "User.Deactivate_Scale" _scale))
        (:`Finished`
          (`ActorComponent.Deactivate` (`self.FlashTrail`))
          (`ActorComponent.Deactivate` (`self.FlashTrail_02`))
          (`ActorComponent.Deactivate` (`self.FlashTrail_StM`)))))))

(event `self.ReceiveBeginPlay`
  (set `self.StartLocation` (`self.K2_GetActorLocation`))
  (`KismetSystemLibrary.Delay` 0.5)
  (goto _label))

(fn `UserConstructionScript`)