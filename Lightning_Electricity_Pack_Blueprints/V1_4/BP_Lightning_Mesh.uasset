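; BP_Lightning_Mesh is a lightning effect actor that spans a bolt between its Start and End components.
; Each tick, it passes the Start-to-End vector and distance to the Lightning component's User.Orientation and User.Distance parameters, so the effect follows both endpoints.
; A timeline that would offset both endpoints is present but never runs, and the construction script is empty.
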(event `self.ReceiveTick`
  (params (DeltaSeconds :type "Float (single-precision)"))
  (bind _lightning (`self.Lightning`))
  (bind _returnvalue (`SceneComponent.K2_GetComponentLocation` (`self.End`)))
  (bind _returnvalue_2 (`SceneComponent.K2_GetComponentLocation` (`self.Start`)))
  ;[1 1 1] Update User.End
  (`/Engine/EditorBlueprintResources/StandardMacros.IsValid` _lightning
    (:`Is Valid`
      (`FXSystemComponent.SetVectorParameter` _lightning "User.Orientation" (- _returnvalue _returnvalue_2))
      (`FXSystemComponent.SetFloatParameter` _lightning "User.Distance" (`KismetMathLibrary.Vector_Distance` _returnvalue _returnvalue_2)))))

(fn `UserConstructionScript`)