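; BP_Turret_A_Destroyed is the wrecked version of Turret A, which breaks apart as soon as it begins play.
; BeginPlay applies radius damage to the Mesh, centered on the Sphere component, to fracture it.
; An unconnected Timeline, meant as a workaround for Add Radial Force, would grow the collision Sphere relative to actor scale to push pieces outward, then disable its collision, but it never runs.
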(event `self.ReceiveBeginPlay`
  (`self.ApplyRadiusDamage` (`self.Mesh`) 1000.0 (`SceneComponent.K2_GetComponentLocation` (`self.Sphere`)) 100.0 1.0 true) ; Fracture the mesh
)

(fn `UserConstructionScript`)