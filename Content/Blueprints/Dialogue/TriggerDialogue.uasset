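; One-shot trigger volume that plays dialogue when an overlapping TestCharacter's objective matches its own and it is active.
; It queues DialogueKeys on the character, with Override clearing the cue and forcing the first line, then destroys itself, after LookDelay if a look target is valid.
; The look-at call itself is disconnected.
; The construction script sizes the box from TriggerExtents, or zero for DirectTriggerOnly.
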(event `self.ReceiveActorBeginOverlap`
  (params (OtherActor :type "Actor Object Reference"))
  (bind _override (`self.Override`))
  (if (`self.Active`)
    (bind _astest_character (cast `/Game/TestObjects/TestCharacter` OtherActor))
    (if (`|EnumEquality` (`/Game/TestObjects/TestCharacter.Objective` _astest_character) (`self.Objective`))
      (`/Engine/EditorBlueprintResources/StandardMacros.DoOnce` false
        (:`Completed`
          (if _override
            (`KismetArrayLibrary.Array_Clear` (`/Game/TestObjects/TestCharacter.DialogueCue` _astest_character))
            (`/Game/TestObjects/TestCharacter.PlayDialogue` _astest_character (`|GetArrayItem` (`self.DialogueKeys`)) true))
          (for (_array_element _array_index) (`self.DialogueKeys`)
            (if (not (and _override (== _array_index 0)))
              (`/Game/TestObjects/TestCharacter.PlayDialogue` _astest_character _array_element false)))
          (`/Engine/EditorBlueprintResources/StandardMacros.IsValid` (`self.LookAtTarget`)
            (:`Is Valid`
              (`KismetSystemLibrary.Delay` (`self.LookDelay`)))
            (:`Is Not Valid`
              _))
          (`self.K2_DestroyActor`))))))

(fn `UserConstructionScript`
  (`BoxComponent.SetBoxExtent` (`self.Box`) (`KismetMathLibrary.SelectVector` (0.0 0.0 0.0) (`self.TriggerExtents`) (`self.DirectTriggerOnly`)) true))