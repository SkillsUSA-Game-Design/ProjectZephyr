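; RockGrinder is an environmental hazard that animates grinder meshes and damages the player character on contact.
; A timeline started at BeginPlay drives the roll of two mesh pairs through separate float tracks, keeping yaw at 90.
; Overlapping the box calls GrinderDamageEvent on a TestCharacter.
; A DoOnce that is never reset limits this to one hit per grinder instance.
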(event `self.ReceiveBeginPlay`
  (bind (_direction _newtrack_0 _newtrack_1) (`Timeline|Timeline_0`)
    (:`Update`
      (`SceneComponent.K2_SetRelativeRotation` (`self.StaticMesh1`) (`KismetMathLibrary.MakeRotator` _newtrack_0 0.0 90.0) false false)
      (`SceneComponent.K2_SetRelativeRotation` (`self.StaticMesh2`) (`KismetMathLibrary.MakeRotator` _newtrack_0 0.0 90.0) false false)
      (`SceneComponent.K2_SetRelativeRotation` (`self.StaticMesh3`) (`KismetMathLibrary.MakeRotator` _newtrack_1 0.0 90.0) false false)
      (`SceneComponent.K2_SetRelativeRotation` (`self.StaticMesh4`) (`KismetMathLibrary.MakeRotator` _newtrack_1 0.0 90.0) false false))))

(event `self.ReceiveTick`
  (params (DeltaSeconds :type "Float (single-precision)")))

(event `self.Box.OnComponentBeginOverlap`
  (params (OverlappedComponent :type "PrimitiveComponent Object Reference") (OtherActor :type "Actor Object Reference") (OtherComp :type "PrimitiveComponent Object Reference") (OtherBodyIndex :type Integer) (bFromSweep :type Boolean) (SweepResult :type "HitResult Structure (by ref)"))
  (bind _astest_character (cast `/Game/TestObjects/TestCharacter` OtherActor))
  (`/Engine/EditorBlueprintResources/StandardMacros.DoOnce` false
    (:`Completed`
      (`/Game/TestObjects/TestCharacter.GrinderDamageEvent` _astest_character))))

(fn `UserConstructionScript`)