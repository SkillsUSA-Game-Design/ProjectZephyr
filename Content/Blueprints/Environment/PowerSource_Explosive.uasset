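; An explosive power source that bursts once, then leaves a low-gravity field that launches the player upward.
; It fires after SpawnDelay via Init or BeginPlay when Enabled, or on player overlap with TriggerRadius, with seeded random-radius camera shake, Niagara, sounds and delayed glow.
; The burst opens a gate, so entering the inner sphere sets Flip, cuts gravity and boosts non-crouching players.
; Exiting restores both after a retriggerable delay.
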(event `self.Sphere1.OnComponentBeginOverlap`
  (params (OverlappedComponent :type "PrimitiveComponent Object Reference") (OtherActor :type "Actor Object Reference") (OtherComp :type "PrimitiveComponent Object Reference") (OtherBodyIndex :type Integer) (bFromSweep :type Boolean) (SweepResult :type "HitResult Structure (by ref)"))
  (bind _returnvalue (`self.K2_GetActorLocation`))
  (bind (_scaleminmax_x _scaleminmax_y) (`KismetMathLibrary.BreakVector2D` (`self.ScaleMinMax`)))
  (cast `/Game/TestObjects/TestCharacter` OtherActor)
  (if (`self.Enabled`)
    (`/Engine/EditorBlueprintResources/StandardMacros.DoOnce` false :!label _label
      (:`Completed`
        (bind _output_get (set `self.Radius` (`KismetMathLibrary.RandomFloatInRangeFromStream` _scaleminmax_x _scaleminmax_y (`self.RandomStream`))))
        (`GameplayStatics.PlayWorldCameraShake` "/Game/Blueprints/Character/RMExplosionCameraShake.RMExplosionCameraShake_C" _returnvalue (* _output_get 2.0) (* _output_get 5.0) 1.0 true)
        (`ActorComponent.Activate` (`self.Niagara1`) false)
        (`GameplayStatics.PlaySoundAtLocation` "/Game/SoundEffects/GlassExplodeMetal2_Cue.GlassExplodeMetal2_Cue" _returnvalue (struct) 0.7 0.9 0.0 "/Game/SoundEffects/SoundAttenuation_Loud.SoundAttenuation_Loud" null null)
        (`self.SetActorHiddenInGame` false)
        (`|ExecutionSequence`
          (:`then_0`
            (goto _label_3 :!via `Open`))
          (:`then_1`
            (`KismetSystemLibrary.Delay` 0.5)
            (`SceneComponent.SetVisibility` (`self.Glow`) true false)
            (`SceneComponent.SetVisibility` (`self.Refraction`) true false)
            (`GameplayStatics.PlaySoundAtLocation` "/Game/Advanced_Space_Fx_Pack1/Sources/Sounds/Explosion_Sounds/Sound_Cue/SW_Explosion_Electrical_02_Cue.SW_Explosion_Electrical_02_Cue" _returnvalue (struct) 1.0 0.6 0.0 "/Game/SoundEffects/SoundAttenuation_Loud.SoundAttenuation_Loud" null null)))))))

(event `Init`
  (`KismetSystemLibrary.Delay` (`self.SpawnDelay`) :!label _label_2)
  (goto _label))

(event `self.ReceiveBeginPlay`
  (bind _astest_character (cast `/Game/TestObjects/TestCharacter` (`GameplayStatics.GetPlayerPawn` 0)))
  (set `self.PlayerCharacter` _astest_character)
  (`KismetMathLibrary.SetRandomStreamSeed` (`self.RandomStream`) (`self.RandomSeed`))
  (if (`self.Enabled`)
    (goto _label_2)))

(event `self.Sphere.OnComponentBeginOverlap`
  (params (OverlappedComponent :type "PrimitiveComponent Object Reference") (OtherActor :type "Actor Object Reference") (OtherComp :type "PrimitiveComponent Object Reference") (OtherBodyIndex :type Integer) (bFromSweep :type Boolean) (SweepResult :type "HitResult Structure (by ref)"))
  (`/Engine/EditorBlueprintResources/StandardMacros.Gate` true :!label _label_3
    (:`Exit`
      (bind _astest_character (cast `/Game/TestObjects/TestCharacter` OtherActor))
      (bind _output_get (set `self.PlayerCharacter` _astest_character))
      (set `/Game/TestObjects/TestCharacter.Flip` true _output_get)
      (bind _charactermovement (`Character.CharacterMovement` _output_get))
      (set `CharacterMovementComponent.GravityScale` 0.5 _charactermovement)
      (set `/Game/TestObjects/TestCharacter.HasAirBoosted` false _output_get)
      (if (not (`/Game/TestObjects/TestCharacter.IsCrouching` _output_get))
        (`CharacterMovementComponent.AddImpulse` _charactermovement (0.0 0.0 50000.0) false)))))

(event `self.Sphere.OnComponentEndOverlap`
  (params (OverlappedComponent :type "PrimitiveComponent Object Reference") (OtherActor :type "Actor Object Reference") (OtherComp :type "PrimitiveComponent Object Reference") (OtherBodyIndex :type Integer))
  (bind _astest_character (cast `/Game/TestObjects/TestCharacter` OtherActor))
  (`KismetSystemLibrary.RetriggerableDelay` 1.0)
  (set `/Game/TestObjects/TestCharacter.Flip` false (stale `self.Sphere.OnComponentBeginOverlap` _output_get))
  (set `CharacterMovementComponent.GravityScale` 1.5 (`Character.CharacterMovement` (stale `self.Sphere.OnComponentBeginOverlap` _output_get))))

(fn `UserConstructionScript`
  (`SphereComponent.SetSphereRadius` (`self.Sphere1`) (`self.TriggerRadius`) true))