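; A moving platform actor that slides along the world X axis when a TestCharacter enters its Box trigger.
; The first such overlap passes a DoOnce, which is never reset, and plays a timeline from the start.
; Each timeline update sets the location to the position saved at BeginPlay plus the track value, negated when Reverse is set, without sweeping.
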(event `self.ReceiveBeginPlay`
  (bind _output_get (set `self.OriginalPosition` (`self.K2_GetActorLocation`))))

(event `self.Box.OnComponentBeginOverlap`
  (params (OverlappedComponent :type "PrimitiveComponent Object Reference") (OtherActor :type "Actor Object Reference") (OtherComp :type "PrimitiveComponent Object Reference") (OtherBodyIndex :type Integer) (bFromSweep :type Boolean) (SweepResult :type "HitResult Structure (by ref)"))
  (cast `/Game/TestObjects/TestCharacter` OtherActor)
  (`/Engine/EditorBlueprintResources/StandardMacros.DoOnce` false
    (:`Completed`
      (bind (_direction _newtrack_0) (`Timeline|Timeline_0` :!via `PlayFromStart`)
        (:`Update`
          (`self.K2_SetActorLocation` (+ (stale `self.ReceiveBeginPlay` _output_get) (`KismetMathLibrary.MakeVector` (`KismetMathLibrary.SelectFloat` (* _newtrack_0 -1.0) _newtrack_0 (`self.Reverse`))))))))))

(fn `UserConstructionScript`)