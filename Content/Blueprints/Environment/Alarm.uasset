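; An alarm actor that can be switched on and off, showing a light and playing a security siren at its location.
; AlarmActivate reveals the point light, spawns a loud-attenuated sound without auto-destroy, and plays a timeline that drives light intensity through a scale factor.
; Deactivate stops the stored sound and timeline and hides the light.
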(event `AlarmActivate`
  (`SceneComponent.SetVisibility` (`self.PointLight`) true false)
  (bind _returnvalue (`GameplayStatics.SpawnSoundAtLocation` "/Game/SoundEffects/SecurityAlarm.SecurityAlarm" (`self.K2_GetActorLocation`) (struct) 0.75 1.0 0.0 "/Game/SoundEffects/SoundAttenuation_Loud.SoundAttenuation_Loud" null false))
  (bind (_direction _newtrack_0) (`Timeline|Timeline_0` :!label _label)
    (:`Update`
      (`LightComponent.SetIntensity` (`self.PointLight`) (* _newtrack_0 (`self.IntensityScale`))))))

(event `Deactivate`
  (`AudioComponent.Stop` (stale `AlarmActivate` _returnvalue))
  (`SceneComponent.SetVisibility` (`self.PointLight`) false false)
  (goto _label :!via `Stop`))

(fn `UserConstructionScript`)