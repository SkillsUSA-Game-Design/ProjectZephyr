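; Sliding door that rises when a TestCharacter enters its trigger box, unless locked, and closes after a delay once they exit.
; Separate open and close timelines move a scene component by scaled height, with state flags and DoOnce gates handling re-entry mid-close.
; If destructible, Kill or a fast or boosting character impact swaps it for a destroyed-door actor with Niagara and crash sound.
; Construction script sizes the trigger.
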(event `self.ReceiveTick`
  (params (DeltaSeconds :type "Float (single-precision)")))

(event `self.Box.OnComponentBeginOverlap`
  (params (OverlappedComponent :type "PrimitiveComponent Object Reference") (OtherActor :type "Actor Object Reference") (OtherComp :type "PrimitiveComponent Object Reference") (OtherBodyIndex :type Integer) (bFromSweep :type Boolean) (SweepResult :type "HitResult Structure (by ref)"))
  (bind _returnvalue (`self.K2_GetActorLocation`))
  (bind _returnvalue_2 (`self.K2_GetActorLocation`))
  (bind _scene (`self.Scene`))
  (bind _closedelay (`self.CloseDelay`))
  (bind _returnvalue_3 (* (.z (`self.GetActorScale3D`)) 300.0))
  (cast `/Game/TestObjects/TestCharacter` OtherActor)
  (if (not (`self.Locked`))
    (`/Engine/EditorBlueprintResources/StandardMacros.DoOnce` false :!label _label
      (:`Completed`
        (if (`self.Closing`)
          (set `self.Exited` false)
          (set `self.Closing` false)
          (set `self.Waiting` false)
          (`|ExecutionSequence`
            (:`then_0`
              (bind (_direction _newtrack_0) (`Timeline|Timeline_0` :!via `Stop` :!label _label_2)
                (:`Update`
                  (`SceneComponent.K2_SetRelativeLocation` _scene (`KismetMathLibrary.MakeVector` 0.0 0.0 (* _returnvalue_3 _newtrack_0)) false false))
                (:`Finished`
                  (`GameplayStatics.PlaySoundAtLocation` "/Game/SoundEffects/AmmoFireHit2.AmmoFireHit2" _returnvalue_2 (struct) 0.2 1.2 0.0 null null null)
                  (set `self.Waiting` false)
                  (set `self.Exited` false)
                  (set `self.Closing` false)
                  (`|ExecutionSequence`
                    (:`then_0`
                      (goto _label :!via `Reset`))
                    (:`then_1`
                      (goto _label_5 :!via `Reset`))))))
            (:`then_1`
              (bind (_direction_2 _newtrack_0_2) (`Timeline|Open` :`NewTime` _newtrack_0 :!via `SetNewTime` :!label _label_3)
                (:`Update`
                  (`SceneComponent.K2_SetRelativeLocation` _scene (`KismetMathLibrary.MakeVector` 0.0 0.0 (* _returnvalue_3 _newtrack_0_2)) false false))
                (:`Finished`
                  (`GameplayStatics.PlaySoundAtLocation` "/Game/SoundEffects/AmmoFireHit2.AmmoFireHit2" _returnvalue_2 (struct) 0.2 1.6 0.0 null null null)
                  (if (`self.Exited`)
                    (set `self.Exited` false)
                    (`KismetSystemLibrary.RetriggerableDelay` _closedelay)
                    (set `self.Closing` true :!label _label_4)
                    (`GameplayStatics.PlaySoundAtLocation` "/Game/SoundEffects/SlideDoor_Cue.SlideDoor_Cue" _returnvalue (struct) 0.4 0.7 0.3 "/Game/SoundEffects/SoundAttenuation_SlideDoor.SoundAttenuation_SlideDoor" null null)
                    (`|ExecutionSequence`
                      (:`then_0`
                        (goto _label :!via `Reset`))
                      (:`then_1`
                        (goto _label_5 :!via `Reset`))
                      (:`then_2`
                        (goto _label_2 :!via `ReverseFromEnd`)))
                    (else
                      (set `self.Waiting` true))))))
            (:`then_2`
              (goto _label_3)))
          (else
            (`GameplayStatics.PlaySoundAtLocation` "/Game/SoundEffects/SlideDoor_Cue.SlideDoor_Cue" _returnvalue (struct) 0.8 0.8 0.3 "/Game/SoundEffects/SoundAttenuation_SlideDoor.SoundAttenuation_SlideDoor" null null)
            (goto _label_3 :!via `PlayFromStart`)))))))

(event `self.Box.OnComponentEndOverlap`
  (params (OverlappedComponent :type "PrimitiveComponent Object Reference") (OtherActor :type "Actor Object Reference") (OtherComp :type "PrimitiveComponent Object Reference") (OtherBodyIndex :type Integer))
  (cast `/Game/TestObjects/TestCharacter` OtherActor)
  (`/Engine/EditorBlueprintResources/StandardMacros.DoOnce` false :!label _label_5
    (:`Completed`
      (set `self.Exited` true)
      (if (`self.Waiting`)
        (set `self.Waiting` false)
        (`KismetSystemLibrary.RetriggerableDelay` (`self.CloseDelay`))
        (goto _label_4)))))

(event `Kill`
  (bind _staticmesh (`self.StaticMesh`))
  (if (`self.Destructable`)
    (`|ExecutionSequence` :!label _label_6
      (:`then_0`
        (goto _label_3 :!via `Stop`))
      (:`then_1`
        (`/Engine/EditorBlueprintResources/StandardMacros.DoOnce` false
          (:`Completed`
            (`AddComponent|NODE_AddNiagaraComponent-0`)
            (`PrimitiveComponent.SetSimulatePhysics` (`self.StaticMesh`) true)
            (`GameplayStatics.PlaySoundAtLocation` "/Game/SoundEffects/HeavyCrash.HeavyCrash" (`self.K2_GetActorLocation`) (struct) 1.0 0.8 0.0 null null null)
            (`|SpawnActorFromClass` "/Game/Blueprints/Environment/SlidingDoor_Destroyed.SlidingDoor_Destroyed_C" (`KismetMathLibrary.MakeTransform` (+ (.location (`self.GetTransform`)) (0.0 0.0 175.0)) (.rotation (`self.GetTransform`)) (`SceneComponent.RelativeScale3D` _staticmesh)) "Undefined" "OverrideRootScale" null null)
            (`ActorComponent.K2_DestroyComponent` _staticmesh)
            (`KismetSystemLibrary.Delay` 5.0)
            (`self.K2_DestroyActor`)))))))

(event `self.StaticMesh.OnComponentHit`
  (params (HitComponent :type "PrimitiveComponent Object Reference") (OtherActor :type "Actor Object Reference") (OtherComp :type "PrimitiveComponent Object Reference") (NormalImpulse :type "Vector Structure") (Hit :type "HitResult Structure (by ref)"))
  (bind _astest_character (cast `/Game/TestObjects/TestCharacter` OtherActor))
  (bind _returnvalue (`KismetMathLibrary.VSize` (`MovementComponent.Velocity` (`Character.CharacterMovement` _astest_character))))
  (bind _isboosting (`/Game/TestObjects/TestCharacter.IsBoosting` _astest_character))
  (if (and (`self.Destructable`) (or (> _returnvalue 1100.0) (and (> _returnvalue 150.0) _isboosting)))
    (goto _label_6)
    (elif (or _isboosting (`/Game/TestObjects/TestCharacter.IsRunning` _astest_character) (> _returnvalue 600.0))
      (`/Engine/EditorBlueprintResources/StandardMacros.DoOnce` false :!label _label_7
        (:`Completed`
          (`GameplayStatics.PlaySoundAtLocation` "/Game/TurretPack/Sounds/Damage/S_MetalExplosion_C.S_MetalExplosion_C" (`self.K2_GetActorLocation` _astest_character) (struct) 1.0 0.8 0.0 null null null)
          (`KismetSystemLibrary.Delay` 1.0)
          (goto _label_7 :!via `Reset`))))))

(fn `UserConstructionScript`
  (`BoxComponent.SetBoxExtent` (`self.Box`) (`self.TriggerExtent`) true))