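; Destructible power machine that breaks once, when a TestCharacter first hits its static mesh.
; The hit swaps the mesh to a broken tank, hides the cylinder and plays a small electric shockwave with an explosion sound above the actor.
; After a short delay, a larger shockwave follows with an electrical explosion sound and a radial camera shake.
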(event `self.StaticMesh.OnComponentHit`
  (params (HitComponent :type "PrimitiveComponent Object Reference") (OtherActor :type "Actor Object Reference") (OtherComp :type "PrimitiveComponent Object Reference") (NormalImpulse :type "Vector Structure") (Hit :type "HitResult Structure (by ref)"))
  (bind _returnvalue (+ (`self.K2_GetActorLocation`) (0.0 0.0 500.0)))
  (cast `/Game/TestObjects/TestCharacter` OtherActor)
  (`/Engine/EditorBlueprintResources/StandardMacros.DoOnce` false
    (:`Completed`
      (`NiagaraFunctionLibrary.SpawnSystemAtLocation` "/Game/Blueprints/NS_Electric_Shockwave_Blue_New.NS_Electric_Shockwave_Blue_New" _returnvalue (struct) (0.5 0.5 0.5))
      (`StaticMeshComponent.SetStaticMesh` (`self.StaticMesh`) "/Game/Polar/Meshes/Props/SM_Tank_Broken.SM_Tank_Broken")
      (`SceneComponent.SetHiddenInGame` (`self.Cylinder`) true false)
      (`GameplayStatics.PlaySoundAtLocation` "/Game/SoundEffects/New/SW_Explosion_Laser_02_Cue_New.SW_Explosion_Laser_02_Cue_New" _returnvalue (struct) 1.0 1.0 0.0 "/Game/SoundEffects/SoundAttenuation_Loud.SoundAttenuation_Loud" null null)
      (`KismetSystemLibrary.Delay` 1.0)
      (`NiagaraFunctionLibrary.SpawnSystemAtLocation` "/Game/Blueprints/NS_Electric_Shockwave_Blue_New.NS_Electric_Shockwave_Blue_New" _returnvalue (struct) (2.0 2.0 2.0))
      (`GameplayStatics.PlayWorldCameraShake` "/Game/Blueprints/Character/RMExplosionCameraShake.RMExplosionCameraShake_C" _returnvalue 500.0 1000.0)
      (`GameplayStatics.PlaySoundAtLocation` "/Game/Advanced_Space_Fx_Pack1/Sources/Sounds/Explosion_Sounds/Sound_Cue/SW_Explosion_Electrical_02_Cue.SW_Explosion_Electrical_02_Cue" _returnvalue (struct) 1.0 1.0 0.0 "/Game/SoundEffects/SoundAttenuation_Loud.SoundAttenuation_Loud" null null))))

(fn `UserConstructionScript`)