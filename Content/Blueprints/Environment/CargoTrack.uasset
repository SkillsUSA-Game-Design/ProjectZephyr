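; Cargo track actor that builds a track of spline meshes along an editable spline in the construction script.
; The spline is split into equal segments sized near MeshLength, each a spline mesh with tangents clamped to segment length.
; Optional supports trace down from each segment midpoint and add instanced meshes scaled to hit distance, skipping short drops.
; The event graph holds an unconnected, delayed copy of this logic.
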(event `self.ReceiveBeginPlay`)

(fn `UserConstructionScript`
  (bind _spline (`self.Spline`))
  (bind _returnvalue (`SplineComponent.GetSplineLength` _spline))
  (bind _returnvalue_2 (`KismetMathLibrary.FTrunc` (/ _returnvalue (`self.MeshLength`))))
  (bind _returnvalue_3 (/ _returnvalue (`KismetMathLibrary.Conv_IntToDouble` _returnvalue_2)))
  (for _index (range _returnvalue_2)
    (bind _returnvalue_4 (* _index _returnvalue_3))
    (bind _returnvalue_5 (`SplineComponent.GetLocationAtDistanceAlongSpline` _spline _returnvalue_4 "World"))
    (bind _returnvalue_6 (* (+ _index 1) _returnvalue_3))
    (bind _returnvalue_7 (`SplineComponent.GetLocationAtDistanceAlongSpline` _spline _returnvalue_6 "World"))
    (bind _returnvalue_8 (/ (+ _returnvalue_5 _returnvalue_7) 2.0))
    (bind _returnvalue_9 (`AddComponent|NODE_AddSplineMeshComponent-0` :`RelativeTransform` (`KismetMathLibrary.MakeTransform` _returnvalue_8)))
    (bind _returnvalue_10 (`SceneComponent.K2_GetComponentToWorld` _returnvalue_9))
    (`SplineMeshComponent.SetStartAndEnd` _returnvalue_9 (`KismetMathLibrary.InverseTransformLocation` _returnvalue_10 _returnvalue_5) (`KismetMathLibrary.ClampVectorSize` (`SplineComponent.GetTangentAtDistanceAlongSpline` _spline _returnvalue_4 "World") 20.0 _returnvalue_3) (`KismetMathLibrary.InverseTransformLocation` _returnvalue_10 _returnvalue_7) (`KismetMathLibrary.ClampVectorSize` (`SplineComponent.GetTangentAtDistanceAlongSpline` _spline _returnvalue_6 "World") 20.0 _returnvalue_3) true)
    (if (`self.MakeSupports`)
      (bind _outhit (`KismetSystemLibrary.LineTraceSingle` (- _returnvalue_8 (0.0 0.0 0.0)) (- _returnvalue_8 (`KismetMathLibrary.MakeVector` 0.0 0.0 (`self.MaximumSupportLength`))) "TraceTypeQuery1"))
      (bind (_bblockinghit _binitialoverlap _time _distance) (`GameplayStatics.BreakHitResult` _outhit))
      (if _bblockinghit
        (if (not (< _distance (`self.MinimumSupportLength`)))
          (`InstancedStaticMeshComponent.AddInstanceWorldSpace` (`self.InstancedStaticMesh`) (`KismetMathLibrary.MakeTransform` (- _returnvalue_8 (0.0 0.0 5.0)) (struct :`Pitch` -90.0) (`KismetMathLibrary.MakeVector` (/ _distance 256.0) 2.0 2.0))))))))