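; ObjectiveArrows is a trigger-started guide effect that sends a Niagara system along a spline, likely to point toward an objective.
; The first TestCharacter overlap of the box, sized and placed in the Construction Script, activates the effect.
; A Tick-driven Gate and DoN counter advance it by Speed units per frame, so travel is framerate-dependent.
; At the final step the gate closes and the actor destroys itself after a delay.
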(event `self.ReceiveBeginPlay`)

(event `Init`
  (bind _spline (`self.Spline`))
  (bind _returnvalue (`KismetMathLibrary.FTrunc` (`self.Increment`)))
  (`ActorComponent.Activate` (`self.Niagara`) false)
  (set `self.SplineLength` (`SplineComponent.GetSplineLength` _spline))
  (set `self.Increment` (/ (`self.SplineLength`) (`self.Speed`)))
  (`|ExecutionSequence`
    (:`then_0`
      (goto _label_2 :!via `Reset`))
    (:`then_1`
      (goto _label :!via `Open`))))

(event `self.ReceiveTick`
  (params (DeltaSeconds :type "Float (single-precision)"))
  (bind _returnvalue (`KismetMathLibrary.FTrunc` (`self.Increment`)))
  (`/Engine/EditorBlueprintResources/StandardMacros.Gate` true :!label _label
    (:`Exit`
      (bind _counter (`/Engine/EditorBlueprintResources/StandardMacros.Do N` _returnvalue :!label _label_2)
        (:`Exit`
          (if (== _counter _returnvalue)
            (`|ExecutionSequence`
              (:`then_0`
                (goto _label :!via `Close`))
              (:`then_1`
                (`KismetSystemLibrary.Delay` 5.0)
                (`self.K2_DestroyActor`)))
            (else
              (`SceneComponent.K2_SetRelativeLocation` (`self.Niagara`) (`SplineComponent.GetLocationAtDistanceAlongSpline` (`self.Spline`) (* (`self.Speed`) (`KismetMathLibrary.Conv_IntToDouble` _counter)) "Local") false false))))))))

(event `self.Box.OnComponentBeginOverlap`
  (params (OverlappedComponent :type "PrimitiveComponent Object Reference") (OtherActor :type "Actor Object Reference") (OtherComp :type "PrimitiveComponent Object Reference") (OtherBodyIndex :type Integer) (bFromSweep :type Boolean) (SweepResult :type "HitResult Structure (by ref)"))
  (cast `/Game/TestObjects/TestCharacter` OtherActor)
  (`/Engine/EditorBlueprintResources/StandardMacros.DoOnce` false
    (:`Completed`
      (`self.Init`))))

(fn `UserConstructionScript`
  (bind _box (`self.Box`))
  (`BoxComponent.SetBoxExtent` _box (`self.TriggerExtent`) true)
  (`SceneComponent.K2_SetRelativeLocation` _box (`self.TriggerOffset`) false false))