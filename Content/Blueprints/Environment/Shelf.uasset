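; Destructible shelf prop that fills itself with randomized boxes and collapses when hit.
; The construction script uses a seeded random stream to spawn four levels of box meshes, varying count, yaw and scale and spacing them across the width.
; The first Hit from any actor enables physics on the shelf parts and boxes and spawns a Niagara destruction effect, while a character cast and speed threshold sit unused.
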(event `self.ReceiveHit`
  (params (MyComp :type "PrimitiveComponent Object Reference") (Other :type "Actor Object Reference") (OtherComp :type "PrimitiveComponent Object Reference") (bSelfMoved :type Boolean) (HitLocation :type "Vector Structure") (HitNormal :type "Vector Structure") (NormalImpulse :type "Vector Structure") (Hit :type "HitResult Structure (by ref)"))
  (`/Engine/EditorBlueprintResources/StandardMacros.DoOnce` false
    (:`Completed`
      (`PrimitiveComponent.SetSimulatePhysics` (`self.StaticMesh1`) true)
      (`PrimitiveComponent.SetSimulatePhysics` (`self.StaticMesh2`) true)
      (`PrimitiveComponent.SetSimulatePhysics` (`self.StaticMesh3`) true)
      (`PrimitiveComponent.SetSimulatePhysics` (`self.e`) true)
      (`PrimitiveComponent.SetSimulatePhysics` (`self.e1`) true)
      (`PrimitiveComponent.SetSimulatePhysics` (`self.e2`) true)
      (`PrimitiveComponent.SetSimulatePhysics` (`self.e3`) true)
      (`PrimitiveComponent.SetSimulatePhysics` (`self.StaticMesh`) true)
      (`PrimitiveComponent.SetSimulatePhysics` (`self.e4`) true)
      (for _array_element (`self.Meshes`)
        (`PrimitiveComponent.SetSimulatePhysics` _array_element true))
      (`NiagaraFunctionLibrary.SpawnSystemAtLocation` "/Game/Realistic_Starter_VFX_Pack_Niagara/Niagara/Destruction/NS_Destruction_Building_01.NS_Destruction_Building_01" (`self.K2_GetActorLocation`)))))

(fn `UserConstructionScript`
  (bind (_boxpershelfminmax_x _boxpershelfminmax_y) (`KismetMathLibrary.BreakVector2D` (`self.BoxPerShelfMinMax`)))
  (bind (_boxminmaxsize_x _boxminmaxsize_y) (`KismetMathLibrary.BreakVector2D` (`self.BoxMinMaxSize`)))
  (bind _stream (`self.Stream`))
  (bind _meshes (`self.Meshes`))
  (bind (_boxminmaxrotation_x _boxminmaxrotation_y) (`KismetMathLibrary.BreakVector2D` (`self.BoxMinMaxRotation`)))
  (bind (_boxminmaxrotation_x_2 _boxminmaxrotation_y_2) (`KismetMathLibrary.BreakVector2D` (`self.BoxMinMaxRotation`)))
  (bind (_boxminmaxrotation_x_3 _boxminmaxrotation_y_3) (`KismetMathLibrary.BreakVector2D` (`self.BoxMinMaxRotation`)))
  (bind (_boxminmaxrotation_x_4 _boxminmaxrotation_y_4) (`KismetMathLibrary.BreakVector2D` (`self.BoxMinMaxRotation`)))
  (bind (_boxpershelfminmax_x_2 _boxpershelfminmax_y_2) (`KismetMathLibrary.BreakVector2D` (`self.BoxPerShelfMinMax`)))
  (bind (_boxminmaxsize_x_2 _boxminmaxsize_y_2) (`KismetMathLibrary.BreakVector2D` (`self.BoxMinMaxSize`)))
  (bind (_boxpershelfminmax_x_3 _boxpershelfminmax_y_3) (`KismetMathLibrary.BreakVector2D` (`self.BoxPerShelfMinMax`)))
  (bind (_boxminmaxsize_x_3 _boxminmaxsize_y_3) (`KismetMathLibrary.BreakVector2D` (`self.BoxMinMaxSize`)))
  (bind (_boxpershelfminmax_x_4 _boxpershelfminmax_y_4) (`KismetMathLibrary.BreakVector2D` (`self.BoxPerShelfMinMax`)))
  (bind (_boxminmaxsize_x_4 _boxminmaxsize_y_4) (`KismetMathLibrary.BreakVector2D` (`self.BoxMinMaxSize`)))
  (bind _width (`self.Width`))
  (bind _returnvalue (`KismetMathLibrary.RandomFloatInRangeFromStream` _boxminmaxsize_x_2 _boxminmaxsize_y_2 _stream))
  (bind _returnvalue_2 (`KismetMathLibrary.RandomFloatInRangeFromStream` _boxminmaxsize_x_4 _boxminmaxsize_y_4 _stream))
  (bind _returnvalue_3 (`KismetMathLibrary.RandomFloatInRangeFromStream` _boxminmaxsize_x_3 _boxminmaxsize_y_3 _stream))
  (bind _returnvalue_4 (`KismetMathLibrary.RandomFloatInRangeFromStream` _boxminmaxsize_x _boxminmaxsize_y _stream))
  (`KismetMathLibrary.SetRandomStreamSeed` _stream (`self.Seed`))
  (bind _output_get (set `self.Amount` (`KismetMathLibrary.FTrunc` (`KismetMathLibrary.RandomFloatInRangeFromStream` _boxpershelfminmax_x_3 _boxpershelfminmax_y_3 _stream))))
  (for _index (range (+ _output_get 1))
    (bind _returnvalue_5 (`AddComponent|NODE_AddStaticMeshComponent-0` :`RelativeTransform` (`KismetMathLibrary.MakeTransform` (`KismetMathLibrary.MakeVector` 0.0 (* _index (/ _width (`KismetMathLibrary.Conv_IntToDouble` _output_get))) 0.0) (`KismetMathLibrary.MakeRotator` 0.0 0.0 (`KismetMathLibrary.RandomFloatInRangeFromStream` _boxminmaxrotation_x_2 _boxminmaxrotation_y_2 _stream)) (`KismetMathLibrary.MakeVector` _returnvalue_3 _returnvalue_3 _returnvalue_3))))
    (`KismetArrayLibrary.Array_Add` _meshes _returnvalue_5))
  (bind _output_get_2 (set `self.Amount` (`KismetMathLibrary.FTrunc` (`KismetMathLibrary.RandomFloatInRangeFromStream` _boxpershelfminmax_x_4 _boxpershelfminmax_y_4 _stream))))
  (for _index_2 (range (+ _output_get_2 1))
    (bind _returnvalue_6 (`AddComponent|NODE_AddStaticMeshComponent-1` :`RelativeTransform` (`KismetMathLibrary.MakeTransform` (`KismetMathLibrary.MakeVector` 0.0 (* _index_2 (/ _width (`KismetMathLibrary.Conv_IntToDouble` _output_get_2))) (`self.ShelfHeight`)) (`KismetMathLibrary.MakeRotator` 0.0 0.0 (`KismetMathLibrary.RandomFloatInRangeFromStream` _boxminmaxrotation_x_3 _boxminmaxrotation_y_3 _stream)) (`KismetMathLibrary.MakeVector` _returnvalue_2 _returnvalue_2 _returnvalue_2))))
    (`KismetArrayLibrary.Array_Add` _meshes _returnvalue_6))
  (bind _output_get_3 (set `self.Amount` (`KismetMathLibrary.FTrunc` (`KismetMathLibrary.RandomFloatInRangeFromStream` _boxpershelfminmax_x_2 _boxpershelfminmax_y_2 _stream))))
  (for _index_3 (range (+ _output_get_3 1))
    (bind _returnvalue_7 (`AddComponent|NODE_AddStaticMeshComponent-3` :`RelativeTransform` (`KismetMathLibrary.MakeTransform` (`KismetMathLibrary.MakeVector` 0.0 (* _index_3 (/ _width (`KismetMathLibrary.Conv_IntToDouble` _output_get_3))) (* (`self.ShelfHeight`) 2.0)) (`KismetMathLibrary.MakeRotator` 0.0 0.0 (`KismetMathLibrary.RandomFloatInRangeFromStream` _boxminmaxrotation_x_4 _boxminmaxrotation_y_4 _stream)) (`KismetMathLibrary.MakeVector` _returnvalue _returnvalue _returnvalue))))
    (`KismetArrayLibrary.Array_Add` _meshes _returnvalue_7))
  (bind _output_get_4 (set `self.Amount` (`KismetMathLibrary.FTrunc` (`KismetMathLibrary.RandomFloatInRangeFromStream` _boxpershelfminmax_x _boxpershelfminmax_y _stream))))
  (for _index_4 (range (+ _output_get_4 1))
    (bind _returnvalue_8 (`AddComponent|NODE_AddStaticMeshComponent-4` :`RelativeTransform` (`KismetMathLibrary.MakeTransform` (`KismetMathLibrary.MakeVector` 0.0 (* _index_4 (/ _width (`KismetMathLibrary.Conv_IntToDouble` _output_get_4))) (* (`self.ShelfHeight`) 3.0)) (`KismetMathLibrary.MakeRotator` 0.0 0.0 (`KismetMathLibrary.RandomFloatInRangeFromStream` _boxminmaxrotation_x _boxminmaxrotation_y _stream)) (`KismetMathLibrary.MakeVector` _returnvalue_4 _returnvalue_4 _returnvalue_4))))
    (`KismetArrayLibrary.Array_Add` _meshes _returnvalue_8)))