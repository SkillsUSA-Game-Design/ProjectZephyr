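; Environment power cell that the player knocks loose by hitting it while boosting or moving fast enough.
; A box overlap casts to TestCharacter, then a DoOnce shifts and rotates the battery, activates lightning particles, shakes the camera, plays an explosion sound and hides the rect light.
; It also increments the PowerManager, then stops the lightning effect after a delay.
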(event `self.Box.OnComponentBeginOverlap`
  (params (OverlappedComponent :type "PrimitiveComponent Object Reference") (OtherActor :type "Actor Object Reference") (OtherComp :type "PrimitiveComponent Object Reference") (OtherBodyIndex :type Integer) (bFromSweep :type Boolean) (SweepResult :type "HitResult Structure (by ref)"))
  (bind _returnvalue (`self.K2_GetActorLocation`))
  (bind _p_stmesh_lightning_v1_25 (`self.P_StMesh_Lightning_V1_25`))
  (bind _astest_character (cast `/Game/TestObjects/TestCharacter` OtherActor))
  (if (or (`/Game/TestObjects/TestCharacter.IsBoosting` _astest_character) (> (`/Game/TestObjects/TestCharacter.Speed` _astest_character) 500.0))
    (`/Engine/EditorBlueprintResources/StandardMacros.DoOnce` false
      (:`Completed`
        (`SceneComponent.K2_SetRelativeLocationAndRotation` (`self.Battery`) (-54.0 0.0 0.0) (struct :`Yaw` -90.0) false false)
        (`ActorComponent.Activate` _p_stmesh_lightning_v1_25 false)
        (`GameplayStatics.PlayWorldCameraShake` "/Game/Blueprints/Character/RMProjectileCameraShake.RMProjectileCameraShake_C" _returnvalue 1000.0 1000.0)
        (`GameplayStatics.PlaySoundAtLocation` "/Game/TurretPack/Sounds/Damage/S_MetalExplosion_B.S_MetalExplosion_B" _returnvalue (struct) 0.8 1.0 0.0 null null null)
        (`SceneComponent.SetVisibility` (`self.RectLight`) false false)
        (`/Game/Blueprints/Environment/PowerSystemManager.Increment` (`self.PowerManager`))
        (`KismetSystemLibrary.Delay` 20.0)
        (`ActorComponent.Deactivate` _p_stmesh_lightning_v1_25)))))

(fn `UserConstructionScript`)