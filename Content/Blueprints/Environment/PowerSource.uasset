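; PowerSource is an environment actor that boosts the TestCharacter upward when it enters the Sphere trigger.
; On BeginPlay it caches the first TestCharacter found in the level.
; An overlap applies a vertical impulse to that character's movement, sets its Flip flag and lowers gravity scale.
; A one-second retriggerable delay then clears Flip and sets a higher, fixed gravity scale rather than restoring the previous value.
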(event `self.ReceiveBeginPlay`
  (bind _outactors (`GameplayStatics.GetAllActorsOfClass` "/Game/TestObjects/TestCharacter.TestCharacter_C"))
  (set `self.PlayerCharacter` (`|GetArrayItem` _outactors)))

(event `self.Sphere.OnComponentBeginOverlap`
  (params (OverlappedComponent :type "PrimitiveComponent Object Reference") (OtherActor :type "Actor Object Reference") (OtherComp :type "PrimitiveComponent Object Reference") (OtherBodyIndex :type Integer) (bFromSweep :type Boolean) (SweepResult :type "HitResult Structure (by ref)"))
  (bind _playercharacter (`self.PlayerCharacter`))
  (bind _charactermovement (`Character.CharacterMovement` _playercharacter))
  (cast `/Game/TestObjects/TestCharacter` OtherActor)
  (`CharacterMovementComponent.AddImpulse` _charactermovement (0.0 0.0 50000.0) false)
  (set `/Game/TestObjects/TestCharacter.Flip` true _playercharacter)
  (set `CharacterMovementComponent.GravityScale` 0.5 _charactermovement)
  (`KismetSystemLibrary.RetriggerableDelay` 1.0)
  (set `/Game/TestObjects/TestCharacter.Flip` false _playercharacter)
  (set `CharacterMovementComponent.GravityScale` 1.5 _charactermovement))

(fn `UserConstructionScript`)