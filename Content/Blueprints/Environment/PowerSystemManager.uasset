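; PowerSystemManager is a manager actor that tracks how many power cells have been activated in the level.
; On BeginPlay it finds every PowerCell and hands it a reference to itself.
; Its Increment event raises the count and fires the 5PowerCellsActivated and 6PowerCellsActivated dispatchers at two milestones.
; Each dispatcher fires at a count one higher than its name indicates.
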(event `self.ReceiveBeginPlay`
  (bind _outactors (`GameplayStatics.GetAllActorsOfClass` "/Game/Blueprints/Environment/PowerCell.PowerCell_C"))
  (for _array_element _outactors
    (set `/Game/Blueprints/Environment/PowerCell.PowerManager` self _array_element)))

(event `Increment`
  (bind _output_get (set `self.PowerCellsActivated` (+ (`self.PowerCellsActivated`) 1)))
  (if (== _output_get 6)
    (`self.5PowerCellsActivated`)
    (elif (== _output_get 7)
      (`self.6PowerCellsActivated`))))

(fn `UserConstructionScript`)