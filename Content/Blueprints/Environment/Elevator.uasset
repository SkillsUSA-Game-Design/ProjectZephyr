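; Elevator actor that travels between its start location and an End offset when a TestCharacter overlaps its Box.
; A Timeline, with play rate set from SecondsToComplete, drives a vector lerp that moves the actor without sweeping.
; A DoOnce blocks retriggering during travel, and on finish a FlipFlop toggles Reverse and resets it, so the next overlap runs the opposite way.
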(event `self.ReceiveBeginPlay`
  (bind _output_get (set `self.StartLocation` (`self.K2_GetActorLocation`)))
  (`TimelineComponent.SetPlayRate` (`self.Timeline_0`) (/ 1.0 (`self.SecondsToComplete`))))

(event `self.Box.OnComponentBeginOverlap`
  (params (OverlappedComponent :type "PrimitiveComponent Object Reference") (OtherActor :type "Actor Object Reference") (OtherComp :type "PrimitiveComponent Object Reference") (OtherBodyIndex :type Integer) (bFromSweep :type Boolean) (SweepResult :type "HitResult Structure (by ref)"))
  (cast `/Game/TestObjects/TestCharacter` OtherActor)
  (`/Engine/EditorBlueprintResources/StandardMacros.DoOnce` false :!label _label
    (:`Completed`
      (if (`self.Reverse`)
        (bind (_direction _newtrack_0) (`Timeline|Timeline_0` :!via `ReverseFromEnd` :!label _label_2)
          (:`Update`
            (`self.K2_SetActorLocation` (`KismetMathLibrary.VLerp` (stale `self.ReceiveBeginPlay` _output_get) (+ (`self.StartLocation`) (`self.End`)) _newtrack_0)))
          (:`Finished`
            (`/Engine/EditorBlueprintResources/StandardMacros.FlipFlop`
              (:`A`
                (set `self.Reverse` true)
                (goto _label :!via `Reset`))
              (:`B`
                (set `self.Reverse` false)
                (goto _label :!via `Reset`)))))
        (else
          (goto _label_2 :!via `PlayFromStart`))))))

(fn `UserConstructionScript`)