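; Single-use health station that sets a TestCharacter's Health to a fixed value when the player presses interact inside its box.
; Box overlap enables the first player controller's input and opens a Gate; leaving disables input and closes it.
; An interact press passes through the open Gate into a DoOnce, which sets Health and toggles the point light's visibility to show it is used.
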(event `self.Box.OnComponentBeginOverlap`
  (params (OverlappedComponent :type "PrimitiveComponent Object Reference") (OtherActor :type "Actor Object Reference") (OtherComp :type "PrimitiveComponent Object Reference") (OtherBodyIndex :type Integer) (bFromSweep :type Boolean) (SweepResult :type "HitResult Structure (by ref)"))
  (bind _astest_character (cast `/Game/TestObjects/TestCharacter` OtherActor))
  (`self.EnableInput` (`GameplayStatics.GetPlayerController` 0))
  (goto _label :!via `Open`))

(event `InputAction|Input_Interact`
  (params (Key :type "Key Structure"))
  (:`Pressed`
    (`/Engine/EditorBlueprintResources/StandardMacros.Gate` true :!label _label
      (:`Exit`
        (`/Engine/EditorBlueprintResources/StandardMacros.DoOnce` false
          (:`Completed`
            (set `/Game/TestObjects/TestCharacter.Health` 99.0 (stale `self.Box.OnComponentBeginOverlap` _astest_character))
            (`SceneComponent.ToggleVisibility` (`self.PointLight`) false)))))))

(event `self.Box.OnComponentEndOverlap`
  (params (OverlappedComponent :type "PrimitiveComponent Object Reference") (OtherActor :type "Actor Object Reference") (OtherComp :type "PrimitiveComponent Object Reference") (OtherBodyIndex :type Integer))
  (cast `/Game/TestObjects/TestCharacter` OtherActor)
  (`self.DisableInput` (`GameplayStatics.GetPlayerController` 0))
  (goto _label :!via `Close`))

(fn `UserConstructionScript`)