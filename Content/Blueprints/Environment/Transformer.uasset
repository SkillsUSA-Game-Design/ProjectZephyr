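; Transformer is an environment actor that explodes when a boosting TestCharacter on one of two specific objectives touches it.
; Sphere overlap and StaticMesh hit events run the same checks into a shared DoOnce.
; It then activates a Niagara effect, destroys the mesh, plays an explosion sound, calls the Destroyed dispatcher, and spawns, enables and initializes a PowerSource_Explosive in its place.
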(event `self.Sphere.OnComponentBeginOverlap`
  (params (OverlappedComponent :type "PrimitiveComponent Object Reference") (OtherActor :type "Actor Object Reference") (OtherComp :type "PrimitiveComponent Object Reference") (OtherBodyIndex :type Integer) (bFromSweep :type Boolean) (SweepResult :type "HitResult Structure (by ref)"))
  (bind _astest_character (cast `/Game/TestObjects/TestCharacter` OtherActor))
  (bind _objective (`/Game/TestObjects/TestCharacter.Objective` _astest_character))
  (if (and (or (`|EnumEquality` _objective "NewEnumerator9") (`|EnumEquality` _objective "NewEnumerator8")) (`/Game/TestObjects/TestCharacter.IsBoosting` _astest_character))
    (`/Engine/EditorBlueprintResources/StandardMacros.DoOnce` false :!label _label
      (:`Completed`
        (`ActorComponent.Activate` (`self.Niagara1`) false)
        (`ActorComponent.K2_DestroyComponent` (`self.StaticMesh`))
        (`GameplayStatics.PlaySoundAtLocation` "/Game/SoundEffects/SuperGridSFX/Cue_Explosions.Cue_Explosions" (`self.K2_GetActorLocation`) (struct) 1.0 1.0 0.0 "/Game/SoundEffects/SoundAttenuation_Loud.SoundAttenuation_Loud" null null)
        (`self.Destroyed`)
        (bind _returnvalue (`|SpawnActorFromClass` "/Game/Blueprints/Environment/PowerSource_Explosive.PowerSource_Explosive_C" (`self.GetTransform`) "AlwaysSpawn" "OverrideRootScale" null null))
        (set `/Game/Blueprints/Environment/PowerSource_Explosive.Enabled` true _returnvalue)
        (`/Game/Blueprints/Environment/PowerSource_Explosive.Init` _returnvalue)))))

(event `self.StaticMesh.OnComponentHit`
  (params (HitComponent :type "PrimitiveComponent Object Reference") (OtherActor :type "Actor Object Reference") (OtherComp :type "PrimitiveComponent Object Reference") (NormalImpulse :type "Vector Structure") (Hit :type "HitResult Structure (by ref)"))
  (bind _astest_character (cast `/Game/TestObjects/TestCharacter` OtherActor))
  (bind _objective (`/Game/TestObjects/TestCharacter.Objective` _astest_character))
  (if (and (or (`|EnumEquality` _objective "NewEnumerator9") (`|EnumEquality` _objective "NewEnumerator8")) (`/Game/TestObjects/TestCharacter.IsBoosting` _astest_character))
    (goto _label)))

(fn `UserConstructionScript`)