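; Lever actor that a TestCharacter activates by pressing Interact inside its box, provided the lever is enabled.
; Box overlaps open and close a gate, which the input press passes through only while Enabled.
; Activation sets IsActivated, swaps the green light for the blue and calls CallActivateEvent.
; An Enable event arms the lever and shows the green light, while BeginPlay matches both lights to initial state.
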(event `self.ReceiveBeginPlay`
  (`SceneComponent.SetVisibility` (`self.GreenLight`) (`self.Enabled`) false)
  (`SceneComponent.SetVisibility` (`self.BlueLight`) (`self.IsActivated`) false))

(event `Enable`
  (set `self.Enabled` true)
  (`SceneComponent.SetVisibility` (`self.GreenLight`) true false)
  (`SceneComponent.SetVisibility` (`self.BlueLight`) false false))

(event `self.Box.OnComponentBeginOverlap`
  (params (OverlappedComponent :type "PrimitiveComponent Object Reference") (OtherActor :type "Actor Object Reference") (OtherComp :type "PrimitiveComponent Object Reference") (OtherBodyIndex :type Integer) (bFromSweep :type Boolean) (SweepResult :type "HitResult Structure (by ref)"))
  (cast `/Game/TestObjects/TestCharacter` OtherActor)
  (goto _label :!via `Open`))

(event `InputAction|Input_Interact` :consume false
  (params (Key :type "Key Structure"))
  (:`Pressed`
    (if (`self.Enabled`)
      (`/Engine/EditorBlueprintResources/StandardMacros.Gate` true :!label _label
        (:`Exit`
          (set `self.IsActivated` true)
          (`SceneComponent.SetVisibility` (`self.GreenLight`) false false)
          (`SceneComponent.SetVisibility` (`self.BlueLight`) true false)
          (`self.ActivateEvent`))))))

(event `self.Box.OnComponentEndOverlap`
  (params (OverlappedComponent :type "PrimitiveComponent Object Reference") (OtherActor :type "Actor Object Reference") (OtherComp :type "PrimitiveComponent Object Reference") (OtherBodyIndex :type Integer))
  (cast `/Game/TestObjects/TestCharacter` OtherActor)
  (goto _label :!via `Close`))

(fn `UserConstructionScript`)