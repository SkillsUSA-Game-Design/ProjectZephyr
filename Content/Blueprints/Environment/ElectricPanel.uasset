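; ElectricPanel is an environment hazard that shocks a TestCharacter entering its Box trigger.
; On overlap it calls the character's ElectricDamageEvent, with a DoOnce that resets after TriggerDelay acting as a cooldown.
; When ShouldMove is set, a Translate timeline started at BeginPlay moves the panel along its up vector by TranslateDistance, with play rate scaled by TranslateTime.
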(event `self.ReceiveBeginPlay`
  (if (`self.ShouldMove`)
    (set `self.StartLocation` (`self.K2_GetActorLocation`))
    (`TimelineComponent.SetPlayRate` (`self.Translate`) (/ 1.0 (`self.TranslateTime`)))
    (bind (_direction _newtrack_0) (`Timeline|Translate` :!via `PlayFromStart`)
      (:`Update`
        (`self.K2_SetActorLocation` (+ (`self.StartLocation`) (* (`self.GetActorUpVector`) (* (`self.TranslateDistance`) _newtrack_0))))))))

(event `self.Box.OnComponentBeginOverlap`
  (params (OverlappedComponent :type "PrimitiveComponent Object Reference") (OtherActor :type "Actor Object Reference") (OtherComp :type "PrimitiveComponent Object Reference") (OtherBodyIndex :type Integer) (bFromSweep :type Boolean) (SweepResult :type "HitResult Structure (by ref)"))
  (bind _astest_character (cast `/Game/TestObjects/TestCharacter` OtherActor))
  (`/Engine/EditorBlueprintResources/StandardMacros.DoOnce` false :!label _label
    (:`Completed`
      (`/Game/TestObjects/TestCharacter.ElectricDamageEvent` _astest_character)
      (`KismetSystemLibrary.Delay` (`self.TriggerDelay`))
      (goto _label :!via `Reset`))))

(fn `UserConstructionScript`)