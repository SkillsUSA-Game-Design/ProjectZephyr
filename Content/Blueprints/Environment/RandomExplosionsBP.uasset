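; Environment actor that spawns Niagara effects, explosions by its name, at random points inside a box volume.
; The construction script sizes the Box component from the BoxExtent variable.
; Once the custom Init event is called, an endless one-second Delay loop adds a new, enlarged Niagara component each pass, converting a random world point into the actor's local space.
; BeginPlay and Tick are unused, and nothing here stops the loop.
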(event `Init`
  (bind _returnvalue (`self.GetTransform`))
  (`KismetSystemLibrary.Delay` 1.0 :!label _label)
  (`AddComponent|NODE_AddNiagaraComponent-0` :`RelativeTransform` (`KismetMathLibrary.MakeTransform` (`KismetMathLibrary.InverseTransformLocation` _returnvalue (`KismetMathLibrary.RandomPointInBoundingBox` (`self.K2_GetActorLocation`) (`self.BoxExtent`))) (.rotation _returnvalue) (10.0 10.0 10.0)))
  (goto _label))

(fn `UserConstructionScript`
  (`BoxComponent.SetBoxExtent` (`self.Box`) (`self.BoxExtent`) true))