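; Enemy turret that tracks the TestCharacter within a sight sphere, fires charged projectiles, and breaks apart when rammed by a boosting or fast-moving player.
; Tick traces to the player, leads the aim point by velocity, and interpolates yaw and pitch on separate meshes.
; A fire delay and Niagara charge-up precede each shot, while close range slows tracking and blocks firing.
; An optional timeline sweeps the aim point when idle.
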(event `self.ReceiveBeginPlay`
  (bind _aimlocation (`self.AimLocation`))
  (bind _outactors (`GameplayStatics.GetAllActorsOfClass` "/Game/TestObjects/TestCharacter.TestCharacter_C"))
  (set `self.PlayerCharacter` (`|GetArrayItem` _outactors))
  (set `self.FireDelayInterp` (`self.FireDelay`))
  (if (`self.IdleAnimation`)
    (`|ExecutionSequence`
      (:`then_0`
        (bind (_direction _newtrack_0) (`Timeline|Timeline_0` :!via `PlayFromStart`)
          (:`Update`
            (`SceneComponent.K2_SetRelativeLocation` _aimlocation (`KismetMathLibrary.MakeVector` (.x (`SceneComponent.RelativeLocation` _aimlocation)) (`KismetMathLibrary.Lerp` 0.0 250.0 _newtrack_0) (.z (`SceneComponent.RelativeLocation` _aimlocation))) false false)))))))

(event `self.ReceiveTick`
  (params (DeltaSeconds :type "Float (single-precision)"))
  (bind _returnvalue_x (`KismetMathLibrary.BreakVector` (`self.GetActorScale3D`)))
  (bind _returnvalue (`self.K2_GetActorLocation`))
  (bind _returnvalue_x_2 (`KismetMathLibrary.BreakVector` (`self.GetActorScale3D`)))
  (bind _turret_mid (`self.Turret_Mid`))
  (bind _turret_top (`self.Turret_Top`))
  (bind _niagara_charge (`self.Niagara_Charge`))
  (bind _barrel_end (`self.Barrel_End`))
  (bind _firedelayinterp (`self.FireDelayInterp`))
  (bind _returnvalue_2 (`KismetMathLibrary.MakeRotFromX` (`KismetMathLibrary.InverseTransformDirection` (`self.GetTransform`) (- (`SceneComponent.K2_GetComponentLocation` (`self.AimLocation`)) (`SceneComponent.K2_GetComponentLocation` (`self.Turret_Top`))))))
  (if (`self.Destroyed`)
    _
    (elif (`self.SeesPlayer`)
      (if (`self.Active`)
        (bind _outhit (`KismetSystemLibrary.LineTraceSingle` (`SceneComponent.K2_GetComponentLocation` (`self.Barrel_End`)) (`self.K2_GetActorLocation` (`self.PlayerCharacter`)) "TraceTypeQuery1" true))
        (bind (_bblockinghit _binitialoverlap _time _distance _location _impactpoint _normal _impactnormal _physmat _hitactor _hitcomponent) (`GameplayStatics.BreakHitResult` _outhit))
        (if _bblockinghit
          (if (< _distance 300.0)
            (set `self.PlayerIsClose` true)
            (else
              (set `self.PlayerIsClose` false)))
          (`SceneComponent.K2_SetWorldLocation` (`self.AimLocation`) (+ (- _location (0.0 0.0 0.0)) (* (`self.GetVelocity` (`self.PlayerCharacter`)) 0.5)) false false)
          (`|ExecutionSequence`
            (:`then_0`
              (`|ExecutionSequence` :!label _label
                (:`then_0`
                  (set `self.TrackingSpeedInterp` (`KismetMathLibrary.FInterpTo` (`self.TrackingSpeedInterp`) (`self.TrackingSpeed`) (`GameplayStatics.GetWorldDeltaSeconds`) 1.0))
                  (`SceneComponent.K2_SetRelativeRotation` _turret_mid (`KismetMathLibrary.RInterpTo` (`SceneComponent.RelativeRotation` _turret_mid) (`KismetMathLibrary.MakeRotator` 0.0 0.0 (.yaw _returnvalue_2)) (`GameplayStatics.GetWorldDeltaSeconds`) (`self.TrackingSpeedInterp`)) false false)
                  (`SceneComponent.K2_SetRelativeRotation` _turret_top (`KismetMathLibrary.RInterpTo` (`SceneComponent.RelativeRotation` _turret_top) (`KismetMathLibrary.MakeRotator` 0.0 (.pitch _returnvalue_2)) (`GameplayStatics.GetWorldDeltaSeconds`) (`self.TrackingSpeedInterp`)) false false))
                (:`then_1`
                  (if (and (stale _output_get_2) (not (`self.PlayerIsClose`)) (<= _firedelayinterp 0.0))
                    (`|ExecutionSequence`
                      (:`then_0`
                        (`/Engine/EditorBlueprintResources/StandardMacros.DoOnce` false :!label _label_2
                          (:`Completed`
                            (`GameplayStatics.SpawnSoundAtLocation` "/Game/SoundEffects/energy_charge_gun_Cue1.energy_charge_gun_Cue1" (`self.K2_GetActorLocation`) (struct) 0.4 (- 1.07 (* _returnvalue_x_2 0.028)) 0.0 null null))))
                      (:`then_1`
                        (bind _output_get (set `self.Charge` (- (`self.Charge`) DeltaSeconds)))
                        (`FXSystemComponent.SetFloatParameter` _niagara_charge "System_Size" (* _output_get 0.75))
                        (if (<= _output_get 0.0)
                          (if (not (`self.PlayerIsClose`))
                            (`|SpawnActorFromClass` "/Game/Blueprints/Turret_Projectile.Turret_Projectile_C" (`KismetMathLibrary.MakeTransform` (`SceneComponent.K2_GetComponentLocation` _barrel_end) (`SceneComponent.K2_GetComponentRotation` _barrel_end) (`KismetMathLibrary.Conv_DoubleToVector` (`self.ProjectileScale`))) "Undefined" "OverrideRootScale" null null)
                            (`ActorComponent.Activate` (`self.Niagara_Fire`) false))
                          (set `self.Charge` (`self.ChargeTime`))
                          (set `self.FireDelayInterp` (`self.FireDelay`))
                          (set `self.TargetLocked` false)
                          (`ActorComponent.Deactivate` _niagara_charge)
                          (`GameplayStatics.SpawnSoundAtLocation` "/Game/SoundEffects/energy_charge_gun_Cue2.energy_charge_gun_Cue2" _returnvalue (struct) 0.75 1.0 3.0 null null)
                          (`GameplayStatics.PlaySoundAtLocation` "/Game/SoundEffects/Lazar_Cue.Lazar_Cue" _returnvalue (struct) 0.5 (- 1.2 (* _returnvalue_x 0.053)) 0.0 null null null)
                          (goto _label_3 :!via `Reset`)
                          (else
                            (`SceneComponent.SetWorldScale3D` (`self.Charge_Test`) (`KismetMathLibrary.Conv_DoubleToVector` (* (* _output_get (/ 1.0 (`self.ChargeTime`))) (`self.ChargeSize`))))))))
                    (else
                      (set `self.FireDelayInterp` (- _firedelayinterp DeltaSeconds))
                      (goto _label_2 :!via `Reset`))))))
            (:`then_1`
              (`/Engine/EditorBlueprintResources/StandardMacros.DoOnce` false :!label _label_3
                (:`Completed`
                  (bind _output_get_2 (set `self.TargetLocked` true))
                  (set `self.Charge` (`self.ChargeTime`))
                  (`ActorComponent.Activate` _niagara_charge false)))))
          (else
            (goto _label)))
        (else
          (if (`self.IdleAnimation`) :!label _label_4
            (goto _label))))
      (else
        (goto _label_4)))))

(event `self.SightTrigger.OnComponentBeginOverlap`
  (params (OverlappedComponent :type "PrimitiveComponent Object Reference") (OtherActor :type "Actor Object Reference") (OtherComp :type "PrimitiveComponent Object Reference") (OtherBodyIndex :type Integer) (bFromSweep :type Boolean) (SweepResult :type "HitResult Structure (by ref)"))
  (cast `/Game/TestObjects/TestCharacter` OtherActor)
  (set `self.SeesPlayer` true))

(event `self.SightTrigger.OnComponentEndOverlap`
  (params (OverlappedComponent :type "PrimitiveComponent Object Reference") (OtherActor :type "Actor Object Reference") (OtherComp :type "PrimitiveComponent Object Reference") (OtherBodyIndex :type Integer))
  (cast `/Game/TestObjects/TestCharacter` OtherActor)
  (set `self.SeesPlayer` false))

(event `self.Sphere_KillRadius.OnComponentBeginOverlap`
  (params (OverlappedComponent :type "PrimitiveComponent Object Reference") (OtherActor :type "Actor Object Reference") (OtherComp :type "PrimitiveComponent Object Reference") (OtherBodyIndex :type Integer) (bFromSweep :type Boolean) (SweepResult :type "HitResult Structure (by ref)"))
  (bind _turret_top (`self.Turret_Top`))
  (bind _returnvalue (`self.K2_GetActorLocation` (`self.PlayerCharacter`)))
  (bind _astest_character (cast `/Game/TestObjects/TestCharacter` OtherActor))
  (bind _isboosting (`/Game/TestObjects/TestCharacter.IsBoosting` _astest_character))
  (if (or _isboosting (> (`/Game/TestObjects/TestCharacter.Speed` _astest_character) 1200.0))
    (`/Engine/EditorBlueprintResources/StandardMacros.DoOnce` false :!label _label_5
      (:`Completed`
        (`AddComponent|NODE_AddNiagaraComponent-0`)
        (set `self.Destroyed` true)
        (`SceneComponent.SetVisibility` (`self.Charge_Test`) false false)
        (`ActorComponent.K2_DestroyComponent` (`self.SM_Turret_A_Base1`))
        (`PrimitiveComponent.SetSimulatePhysics` _turret_top true)
        (`PrimitiveComponent.SetSimulatePhysics` (`self.Turret_Barrel`) true)
        (`PrimitiveComponent.SetSimulatePhysics` (`self.Turret_Mid`) true)
        (`PrimitiveComponent.SetSimulatePhysics` (`self.StaticMesh5`) true)
        (`PrimitiveComponent.SetSimulatePhysics` (`self.StaticMesh6`) true)
        (`GameplayStatics.PlayWorldCameraShake` "/Game/Blueprints/Character/RMExplosionCameraShake.RMExplosionCameraShake_C" _returnvalue 900.0 900.0)
        (`ActorComponent.Deactivate` (`self.Niagara_Charge`))
        (`PrimitiveComponent.SetCollisionEnabled` (`self.StaticMesh2`) "NoCollision")
        (`PrimitiveComponent.SetCollisionEnabled` (`self.SM_Turret_A_Base`) "NoCollision")
        (`GameplayStatics.PlaySoundAtLocation` "/Game/SoundEffects/Exp_Lrg_1_Cue.Exp_Lrg_1_Cue" _returnvalue (struct) 1.2 0.8 0.0 null null null)
        (`GameplayStatics.PlaySoundAtLocation` "/Game/SoundEffects/NoneExplodeMetal2.NoneExplodeMetal2" _returnvalue (struct) 0.8 (`KismetMathLibrary.RandomFloatInRange` 1.0 1.15) 1.0 null null null)
        (`KismetSystemLibrary.Delay` 9.0)
        (`ActorComponent.K2_DestroyComponent` _turret_top)
        (`ActorComponent.K2_DestroyComponent` (`self.Turret_Barrel`))
        (`ActorComponent.K2_DestroyComponent` (`self.Turret_Mid`))
        (`ActorComponent.K2_DestroyComponent` (`self.StaticMesh5`))
        (`ActorComponent.K2_DestroyComponent` (`self.StaticMesh6`))))
    (elif _isboosting
      (`/Engine/EditorBlueprintResources/StandardMacros.DoOnce` false :!label _label_6
        (:`Completed`
          (`GameplayStatics.PlaySoundAtLocation` "/Game/TurretPack/Sounds/Damage/S_MetalExplosion_C.S_MetalExplosion_C" (`self.K2_GetActorLocation`) (struct) 1.0 0.8 0.0 null null null))))))

(event `self.Sphere_CloseRadius.OnComponentBeginOverlap`
  (params (OverlappedComponent :type "PrimitiveComponent Object Reference") (OtherActor :type "Actor Object Reference") (OtherComp :type "PrimitiveComponent Object Reference") (OtherBodyIndex :type Integer) (bFromSweep :type Boolean) (SweepResult :type "HitResult Structure (by ref)"))
  (cast `/Game/TestObjects/TestCharacter` OtherActor)
  (set `self.TrackingSpeed` 1.25)
  (set `self.PlayerIsClose` true))

(event `self.Sphere_CloseRadius.OnComponentEndOverlap`
  (params (OverlappedComponent :type "PrimitiveComponent Object Reference") (OtherActor :type "Actor Object Reference") (OtherComp :type "PrimitiveComponent Object Reference") (OtherBodyIndex :type Integer))
  (cast `/Game/TestObjects/TestCharacter` OtherActor)
  (set `self.TrackingSpeed` 2.2)
  (set `self.PlayerIsClose` false))

(event `self.SM_Turret_A_Base.OnComponentHit`
  (params (HitComponent :type "PrimitiveComponent Object Reference") (OtherActor :type "Actor Object Reference") (OtherComp :type "PrimitiveComponent Object Reference") (NormalImpulse :type "Vector Structure") (Hit :type "HitResult Structure (by ref)"))
  (bind _astest_character (cast `/Game/TestObjects/TestCharacter` OtherActor))
  (bind _speed (`/Game/TestObjects/TestCharacter.Speed` _astest_character))
  (bind _returnvalue (> _speed 150.0))
  (if (or (and (`/Game/TestObjects/TestCharacter.IsBoosting` _astest_character) _returnvalue) (> _speed 1200.0))
    (goto _label_5)
    (elif (not _returnvalue)
      (goto _label_6))))

(fn `UserConstructionScript`
  (`SphereComponent.SetSphereRadius` (`self.SightTrigger`) (`self.SightRadius`) true))