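; ObjectiveChanger is a trigger volume that advances the player's objective when they enter it.
; When active, its box overlap checks that a TestCharacter currently holds the required objective, then replaces it with the new objective.
; The construction script sizes the box from a configurable extents variable, so each placed instance can cover its own area.
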(event `self.Box.OnComponentBeginOverlap`
  (params (OverlappedComponent :type "PrimitiveComponent Object Reference") (OtherActor :type "Actor Object Reference") (OtherComp :type "PrimitiveComponent Object Reference") (OtherBodyIndex :type Integer) (bFromSweep :type Boolean) (SweepResult :type "HitResult Structure (by ref)"))
  (if (`self.Active`)
    (bind _astest_character (cast `/Game/TestObjects/TestCharacter` OtherActor))
    (if (`|EnumEquality` (`/Game/TestObjects/TestCharacter.Objective` _astest_character) (`self.RequiredObjective`))
      (set `/Game/TestObjects/TestCharacter.Objective` (`self.NewObjective`) _astest_character))))

(fn `UserConstructionScript`
  (`BoxComponent.SetBoxExtent` (`self.Box`) (`self.TriggerExtents`) true))