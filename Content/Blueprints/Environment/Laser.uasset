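; Laser hazard actor that damages a TestCharacter when the character hits its beam.
; A hit calls the character's LaserDamageEvent, then a DoOnce disables beam collision and hides both cylinders until RestartDelay elapses and the beam returns.
; The construction script sizes and offsets the outer and thin inner cylinders from LaserLength, so the beam extends from the actor's origin.
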(event `self.Cylinder.OnComponentHit`
  (params (HitComponent :type "PrimitiveComponent Object Reference") (OtherActor :type "Actor Object Reference") (OtherComp :type "PrimitiveComponent Object Reference") (NormalImpulse :type "Vector Structure") (Hit :type "HitResult Structure (by ref)"))
  (bind _cylinder (`self.Cylinder`))
  (bind _astest_character (cast `/Game/TestObjects/TestCharacter` OtherActor))
  (`/Game/TestObjects/TestCharacter.LaserDamageEvent` _astest_character)
  (`/Engine/EditorBlueprintResources/StandardMacros.DoOnce` false :!label _label
    (:`Completed`
      (`PrimitiveComponent.SetCollisionEnabled` _cylinder "NoCollision")
      (`SceneComponent.SetVisibility` _cylinder false false)
      (`SceneComponent.SetVisibility` (`self.Cylinder_Small`) false false)
      (`KismetSystemLibrary.Delay` (`self.RestartDelay`))
      (`PrimitiveComponent.SetCollisionEnabled` _cylinder "QueryAndPhysics")
      (`SceneComponent.SetVisibility` (`self.Cylinder_Small`) true false)
      (`SceneComponent.SetVisibility` _cylinder true false)
      (goto _label :!via `Reset`))))

(fn `UserConstructionScript`
  (bind _laserlength (`self.LaserLength`))
  (bind _cylinder (`self.Cylinder`))
  (bind _returnvalue (* _laserlength 0.01))
  (`SceneComponent.K2_SetRelativeLocation` _cylinder (`KismetMathLibrary.MakeVector` (* _laserlength 0.5)) false false)
  (`SceneComponent.K2_SetRelativeLocation` (`self.Cylinder_Small`) (`KismetMathLibrary.MakeVector` (* _laserlength 0.5)) false false)
  (`SceneComponent.SetWorldScale3D` _cylinder (`KismetMathLibrary.MakeVector` 0.15 0.15 _returnvalue))
  (`SceneComponent.SetWorldScale3D` (`self.Cylinder_Small`) (`KismetMathLibrary.MakeVector` 0.05 0.05 _returnvalue)))