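; Sequencer event Blueprint for the opening cinematic, staging the player character's arrival in a teleport effect.
; Its events hide the player with a meteor sound, spawn an electric aura, then replace it with an explosion and shockwave as the player reappears.
; The arrival leaves a decal at a hardcoded position and a floor fire that deactivates after a delay.
; Charge sound, look-around animation and camera, dialogue and HUD handoff nodes are disconnected.
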(event `SequenceEvent_2`
  (bind _astest_character (cast `/Game/TestObjects/TestCharacter` (`GameplayStatics.GetPlayerPawn` 0)))
  (`Actor.SetActorHiddenInGame` _astest_character true)
  (`GameplayStatics.PlaySound2D` "/Game/SoundEffects/Expansion/Meteor.Meteor" 1.0 0.75 0.0 null null))

(event `SequenceEvent_0`
  (bind _returnvalue (`NiagaraFunctionLibrary.SpawnSystemAtLocation` "/Game/Lightning_Electricity_Pack/Particles/V1_25/P_Electric_Aura.P_Electric_Aura" (+ (`self.TeleportEffectLocation`) (0.0 0.0 -70.0)) (struct) (1.5 1.5 1.5))))

(event `SequenceEvent_1`
  (bind _teleporteffectlocation (`self.TeleportEffectLocation`))
  (`GameplayStatics.PlaySoundAtLocation` "/Game/SoundEffects/Expansion/SW_Explosion_Laser_02_Cue_New.SW_Explosion_Laser_02_Cue_New" _teleporteffectlocation (struct) 0.9 0.6 0.0 "/Game/SoundEffects/SoundAttenuation_DistantLoud.SoundAttenuation_DistantLoud" null null)
  (`NiagaraFunctionLibrary.SpawnSystemAtLocation` "/Game/Blueprints/NS_Electric_Shockwave_Blue_New.NS_Electric_Shockwave_Blue_New" _teleporteffectlocation)
  (bind _astest_character (cast `/Game/TestObjects/TestCharacter` (`GameplayStatics.GetPlayerPawn` 0)))
  (`Actor.SetActorHiddenInGame` _astest_character false)
  (`ActorComponent.K2_DestroyComponent` (stale `SequenceEvent_0` _returnvalue))
  (bind _returnvalue (`NiagaraFunctionLibrary.SpawnSystemAtLocation` "/Game/Realistic_Starter_VFX_Pack_Niagara/Niagara/Fire/NS_Fire_Floor.NS_Fire_Floor" (+ _teleporteffectlocation (0.0 0.0 -50.0)) (struct) (2.0 2.0 1.5)))
  (`GameplayStatics.SpawnDecalAtLocation` "/Game/Materials/M_Decal_Master_Inst.M_Decal_Master_Inst" (128.0 900.0 900.0) (-5251.0 23114.0 4403.0) (struct :`Pitch` 90.0))
  (`KismetSystemLibrary.Delay` 2.0)
  (`ActorComponent.Deactivate` _returnvalue))