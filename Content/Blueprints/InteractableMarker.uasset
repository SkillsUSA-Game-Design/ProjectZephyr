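; Interactable marker actor that appears and animates while a TestCharacter is within its sphere trigger.
; Sphere begin overlap or the Activate event unhides the actor and plays a timeline that offsets its height from the location cached at BeginPlay.
; When the TestCharacter leaves the sphere, the actor hides and the timeline stops.
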(event `self.ReceiveBeginPlay`
  (set `self.InitialLocation` (`self.K2_GetActorLocation`)))

(event `Activate`
  (`self.SetActorHiddenInGame` false :!label _label)
  (bind (_direction _newtrack_0) (`Timeline|Timeline_0` :!label _label_2)
    (:`Update`
      (`self.K2_SetActorLocation` (+ (`self.InitialLocation`) (`KismetMathLibrary.MakeVector` 0.0 0.0 _newtrack_0))))))

(event `self.Sphere.OnComponentBeginOverlap`
  (params (OverlappedComponent :type "PrimitiveComponent Object Reference") (OtherActor :type "Actor Object Reference") (OtherComp :type "PrimitiveComponent Object Reference") (OtherBodyIndex :type Integer) (bFromSweep :type Boolean) (SweepResult :type "HitResult Structure (by ref)"))
  (cast `/Game/TestObjects/TestCharacter` OtherActor)
  (goto _label))

(event `self.Sphere.OnComponentEndOverlap`
  (params (OverlappedComponent :type "PrimitiveComponent Object Reference") (OtherActor :type "Actor Object Reference") (OtherComp :type "PrimitiveComponent Object Reference") (OtherBodyIndex :type Integer))
  (cast `/Game/TestObjects/TestCharacter` OtherActor)
  (`self.SetActorHiddenInGame` true)
  (goto _label_2 :!via `Stop`))

(fn `UserConstructionScript`)