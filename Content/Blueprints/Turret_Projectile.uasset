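; Turret projectile that trails a Niagara effect and explodes on impact, with ribbon width and lifetime scaled by its X scale.
; Tick keeps the effect's end point at the spawn location and destroys the actor once its lifetime expires.
; A gate opened just after BeginPlay lets sphere hits spawn an Explosion, halt the projectile and destroy it shortly after.
; A separate box overlap with TestCharacter plays a world camera shake.
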(event `self.ReceiveBeginPlay`
  (bind _returnvalue_x (`KismetMathLibrary.BreakVector` (`self.GetActorScale3D`)))
  (set `self.InitialLocation` (`self.K2_GetActorLocation`))
  (`FXSystemComponent.SetFloatParameter` (`self.Niagara`) "RibbonWidth" (* _returnvalue_x 2.0))
  (`KismetSystemLibrary.Delay` 0.001)
  (goto _label :!via `Open`))

(event `self.ProjectileMovement.OnProjectileStop`
  (params (ImpactResult :type "HitResult Structure (by ref)")))

(event `self.Sphere1.OnComponentHit`
  (params (HitComponent :type "PrimitiveComponent Object Reference") (OtherActor :type "Actor Object Reference") (OtherComp :type "PrimitiveComponent Object Reference") (NormalImpulse :type "Vector Structure") (Hit :type "HitResult Structure (by ref)"))
  (`/Engine/EditorBlueprintResources/StandardMacros.Gate` true :!label _label
    (:`Exit`
      (`|SpawnActorFromClass` "/Game/Blueprints/Explosion.Explosion_C" (`self.GetTransform`) "Undefined" "OverrideRootScale" null null)
      (`PrimitiveComponent.SetCollisionEnabled` (`self.Sphere1`) "NoCollision")
      (set `ProjectileMovementComponent.MaxSpeed` 0.0 (`self.ProjectileMovement`))
      (`KismetSystemLibrary.Delay` 0.5)
      (`self.K2_DestroyActor`))))

(event `self.ReceiveTick`
  (params (DeltaSeconds :type "Float (single-precision)"))
  (bind _returnvalue_x (`KismetMathLibrary.BreakVector` (`self.GetActorScale3D`)))
  (`FXSystemComponent.SetVectorParameter` (`self.Niagara`) "User.End" (`self.InitialLocation`))
  (if (> (`self.GetGameTimeSinceCreation`) (* _returnvalue_x 3.0))
    (`self.K2_DestroyActor`)))

(event `self.Box.OnComponentBeginOverlap`
  (params (OverlappedComponent :type "PrimitiveComponent Object Reference") (OtherActor :type "Actor Object Reference") (OtherComp :type "PrimitiveComponent Object Reference") (OtherBodyIndex :type Integer) (bFromSweep :type Boolean) (SweepResult :type "HitResult Structure (by ref)"))
  (bind _astest_character (cast `/Game/TestObjects/TestCharacter` OtherActor))
  (`GameplayStatics.PlayWorldCameraShake` "/Game/Blueprints/Character/RMProjectileCameraShake.RMProjectileCameraShake_C" (`self.K2_GetActorLocation` _astest_character) 500.0 500.0))

(fn `UserConstructionScript`)