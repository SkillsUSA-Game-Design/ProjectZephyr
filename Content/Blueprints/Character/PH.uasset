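; Player character Blueprint with target lock, stamina-based sprinting, health and a pause menu.
; Tab toggles a camera-direction sphere trace for a pawn, and Tick turns control rotation toward that target.
; Left Shift sets walk speed and runs RetriggerableDelay loops that drain or restore stamina.
; BeginPlay adds stamina and health widgets, Escape toggles pause, and M applies self-damage, with death only printed.
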(event `self.ReceiveTick`
  (params (DeltaSeconds :type "Float (single-precision)"))
  ;[1 1 1] Set Target Lock Rotation
  (`self.HitTarget`
    (:`then`
      (`Controller.SetControlRotation` (`Pawn.GetController`) (`KismetMathLibrary.FindLookAtRotation` (`self.K2_GetActorLocation`) (`self.K2_GetActorLocation` (`self.HitTarget`)))))
    (:`else`)))

(event `Key|Tab`
  (params (Key :type "Key Structure"))
  (bind _returnvalue (`self.K2_GetActorLocation`))
  ;[1 1 1] Target Lock Trace and Hit
  (:`Pressed`
    (`/Engine/EditorBlueprintResources/StandardMacros.FlipFlop`
      (:`A`
        (bind (_outhit _returnvalue_2) (`KismetSystemLibrary.SphereTraceSingleForObjects` :`Start` _returnvalue :`End` (+ _returnvalue (* (`KismetMathLibrary.GetForwardVector` (`SceneComponent.K2_GetComponentRotation` (`self.FollowCamera`))) 500.0)) :`Radius` 125.0 :`ObjectTypes` (`|MakeArray` "ObjectTypeQuery3" :!type "EObjectTypeQuery Enum") :`DrawDebugType` "ForDuration"))
        (if _returnvalue_2
          (set `self.HitTarget` (`.HitActor` (`GameplayStatics.BreakHitResult` _outhit)))))
      (:`B`
        (set `self.HitTarget` null)))))

(event `Key|LeftShift`
  (params (Key :type "Key Structure"))
  (bind _charactermovement (`self.CharacterMovement`))
  ;[1 1 1] Speed Boost
  (:`Pressed`
    (set `self.isRunning?` true)
    (set `CharacterMovementComponent.MaxWalkSpeed` 2000.0 _charactermovement :!label _label)
    (`KismetSystemLibrary.RetriggerableDelay` 0.2)
    (`self.UseStamina`)
    (if (`self.isRunning?`)
      (goto _label)))
  (:`Released`
    (set `self.isRunning?` false)
    (set `CharacterMovementComponent.MaxWalkSpeed` 1000.0 _charactermovement :!label _label_2)
    (`KismetSystemLibrary.RetriggerableDelay` 0.2)
    (`self.IncreaseStamina`)
    (if (`self.canIncreaseStamina?`)
      (goto _label_2))))

(event `Key|Escape` :paused true
  (params (Key :type "Key Structure"))
  (bind _returnvalue (`GameplayStatics.GetPlayerController` 0))
  ;[1 1 1] Pause Game
  (:`Pressed`
    (`/Engine/EditorBlueprintResources/StandardMacros.FlipFlop`
      (:`A`
        (bind _returnvalue_2 (`|CreateWidget` "/Game/Blueprints/Character/Pause_Menu/Pause_Menu_Widget.Pause_Menu_Widget_C"))
        (`UserWidget.AddToViewport` _returnvalue_2 0)
        (`GameplayStatics.SetGamePaused` true)
        (set `PlayerController.bShowMouseCursor` true _returnvalue))
      (:`B`
        (`Widget.RemoveFromParent` _returnvalue_2)
        (`GameplayStatics.SetGamePaused` false)
        (set `PlayerController.bShowMouseCursor` false _returnvalue)))))

(event `UseStamina`
  ;[1 1 1] Stamina and Damage
  (set `self.stamina` (- (`self.stamina`) 2.0))
  (if (<= (`self.stamina`) 0.0)
    (set `self.isRunning?` false)
    (set `CharacterMovementComponent.MaxWalkSpeed` 1000.0 (`self.CharacterMovement`))
    (else
      (`KismetSystemLibrary.PrintString` (`KismetStringLibrary.Conv_DoubleToString` (`self.stamina`))))))

(event `IncreaseStamina`
  ;[1 1 1] Stamina and Damage
  (set `self.stamina` (+ (`self.stamina`) 2.0))
  (if (>= (`self.stamina`) 100.0)
    (set `self.canIncreaseStamina?` false)
    (else
      (set `self.canIncreaseStamina?` true))))

(event `self.ReceiveBeginPlay`
  ;[1 1 1] Stamina and Damage
  (bind _returnvalue (`|CreateWidget` "/Game/Blueprints/Character/WP_Stamina.WP_Stamina_C" (`GameplayStatics.GetPlayerController` 0)))
  (`UserWidget.AddToViewport` _returnvalue 0)
  (if true
    (bind _returnvalue_2 (`|CreateWidget` "/Game/Blueprints/Character/WP_HealthBar.WP_HealthBar_C" (`GameplayStatics.GetPlayerController` 0)))
    (`UserWidget.AddToViewport` _returnvalue_2 0)))

(event `Key|M`
  (params (Key :type "Key Structure"))
  ;[1 1 1] Stamina and Damage
  (:`Pressed`
    (`GameplayStatics.ApplyDamage` self 10.0)))

(event `self.ReceiveAnyDamage`
  (params (Damage :type "Float (single-precision)") (DamageType :type "DamageType Object Reference") (InstigatedBy :type "Controller Object Reference") (DamageCauser :type "Actor Object Reference"))
  ;[1 1 1] Stamina and Damage
  (set `self.health` (- (`self.health`) Damage))
  (if (<= (`self.health`) 0.0)
    (`KismetSystemLibrary.PrintString` "Dead!")
    (else
      (`KismetSystemLibrary.PrintString` (`KismetStringLibrary.Conv_DoubleToString` (`self.health`))))))

(fn `UserConstructionScript`)

(fn `UseStamina`)