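; Wire task actor that groups several Bp_wire child actors, apparently for a wire puzzle.
; Its construction script casts the child actor of each of its four ChildActor components to Bp_wire and collects them in the Wires array.
; ShuffleEndLocation is an unfinished stub that loops over Wires without doing anything, and the event graph holds no active logic.
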(fn `ShuffleEndLocation`
  (for _ (`self.Wires`)
    _))

(fn `UserConstructionScript`
  (for _array_element (`|MakeArray` (`self.ChildActor1`) (`self.ChildActor2`) (`self.ChildActor3`) (`self.ChildActor`))
    (bind _asbp_wire (cast `/Game/Wire_task/Bp_wire` (`ChildActorComponent.ChildActor` _array_element)))
    (`KismetArrayLibrary.Array_Add` (`self.Wires`) _asbp_wire)))