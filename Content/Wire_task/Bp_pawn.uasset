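; Player pawn for a wire-connection task, in which the mouse drags Bp_wire ends onto other wires.
; Left press traces under the cursor and grabs a wire that passes CanGrab.
; Each tick, the grabbed end follows the cursor ray's intersection with the wire's forward-facing plane.
; Release attaches to any Bp_wire hit, as CanAttach is unused, otherwise resets; camera and cursor setup is unconnected.
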(event `self.ReceiveBeginPlay`)

(event `self.ReceiveTick`
  (params (DeltaSeconds :type "Float (single-precision)"))
  (`self.UpdateGrab`))

(event `StartGrab`
  (bind (_worldlocation _worlddirection) (`PlayerController.DeprojectMousePositionToWorld` (`GameplayStatics.GetPlayerController` 0)))
  (bind (_outhit _returnvalue) (`KismetSystemLibrary.LineTraceSingle` :`Start` _worldlocation :`End` (+ _worldlocation (* _worlddirection 1000.0)) :`TraceChannel` "TraceTypeQuery1" :`DrawDebugType` "ForOneFrame"))
  (if _returnvalue
    (bind (_bblockinghit _binitialoverlap _time _distance _location _impactpoint _normal _impactnormal _physmat _hitactor _hitcomponent) (`GameplayStatics.BreakHitResult` _outhit))
    (bind _asbp_wire (cast `/Game/Wire_task/Bp_wire` _hitactor))
    (if (`/Game/Wire_task/Bp_wire.CanGrab` _asbp_wire _hitcomponent)
      (bind _output_get (set `self.GrabWire` _asbp_wire))
      (`/Game/Wire_task/Bp_wire.StartGrab` _output_get))))

(event `Key|LeftMouseButton`
  (params (Key :type "Key Structure"))
  (:`Pressed`
    (`self.StartGrab`))
  (:`Released`
    (`self.EndGrab`)))

(event `EndGrab`
  (bind (_worldlocation _worlddirection) (`PlayerController.DeprojectMousePositionToWorld` (`GameplayStatics.GetPlayerController` 0)))
  (`self.GrabWire`
    (:`then`
      (bind (_outhit _returnvalue) (`KismetSystemLibrary.LineTraceSingle` :`Start` _worldlocation :`End` (+ _worldlocation (* _worlddirection 1000.0)) :`TraceChannel` "TraceTypeQuery1" :`DrawDebugType` "ForOneFrame"))
      (if _returnvalue
        (bind _asbp_wire (cast `/Game/Wire_task/Bp_wire` (`.HitActor` (`GameplayStatics.BreakHitResult` _outhit)))
          (:`then`
            (if true
              (`/Game/Wire_task/Bp_wire.Attach` (`self.GrabWire`) _asbp_wire)
              (set `self.GrabWire` null)
              (else
                (`self.ResetGrab`))))
          (:`CastFailed`
            (`self.ResetGrab`)))
        (else
          (`self.ResetGrab`))))
    (:`else`
      (`self.ResetGrab`))))

(event `UpdateGrab`
  (bind (_worldlocation _worlddirection) (`PlayerController.DeprojectMousePositionToWorld` (`GameplayStatics.GetPlayerController` 0)))
  (bind _grabwire (`self.GrabWire`)
    (:`then`
      (bind (_t _intersection _returnvalue) (`KismetMathLibrary.LinePlaneIntersection_OriginNormal` _worldlocation (+ _worldlocation (* _worlddirection 1000.0)) (`self.K2_GetActorLocation` _grabwire) (`self.GetActorForwardVector` _grabwire)))
      (if _returnvalue
        (`/Game/Wire_task/Bp_wire.SetEndLocation` _grabwire _intersection)))
    (:`else`)))

(event `ResetGrab`
  (bind _grabwire (`self.GrabWire`)
    (:`then`
      (`/Game/Wire_task/Bp_wire.Reset` _grabwire)
      (set `self.GrabWire` null))
    (:`else`)))

(fn `UserConstructionScript`)