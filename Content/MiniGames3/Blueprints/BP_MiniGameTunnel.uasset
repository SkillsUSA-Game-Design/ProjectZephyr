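; Tunnel minigame on an in-world screen: the player steers to stay centered in a moving tunnel until a progress bar fills.
; Tick smooths input into an offset and animates rings along sine-based paths, recycling them by shifting the array.
; A dynamic material receives ring, position and progress parameters, while a distance check on one ring raises or drains the bar.
; Interaction starts the game and blends the camera; success or cancellation returns it to the player.
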(event `self.ReceiveBeginPlay`
  ;[1 1 1] Init
  (`parent.ReceiveBeginPlay`)
  (bind _returnvalue (`KismetMaterialLibrary.CreateDynamicMaterialInstance` "/Game/MiniGames3/Materials/MI_MiniGameTunnel_Inst.MI_MiniGameTunnel_Inst"))
  (set `self.DMI` _returnvalue))

(event `InitGame`
  (bind _dmi (`self.DMI`))
  (bind _dmi_2 (`self.DMI`))
  ;[1 1 1] Setup game
  (`self.SetupTunnel`)
  (`MaterialInstanceDynamic.SetScalarParameterValue` _dmi "Progress" 0.0)
  (`MaterialInstanceDynamic.SetScalarParameterValue` _dmi "ShowEnabled" 0.0)
  (set `self.BarDelta` (/ (`self.MaxBarValue`) (`self.BarValue`)))
  (set `self.CurrBarValue` 0.0)
  (set `self.Xpos` 0.0)
  (set `self.Ypos` 0.0)
  (set `self.XposNew` 0.0)
  (set `self.YposNew` 0.0)
  (`MaterialInstanceDynamic.SetScalarParameterValue` _dmi_2 "Xpos" (`self.Xpos`))
  (`MaterialInstanceDynamic.SetScalarParameterValue` _dmi_2 "Ypos" (`self.Ypos`)))

(event `self.ReceiveTick`
  (params (DeltaSeconds :type "Float (single-precision)"))
  (bind _returnvalue (`KismetMathLibrary.GetPI`))
  (bind _rightaxis (`self.RightAxis`))
  (bind _tunnel (`self.Tunnel`))
  (bind _forwardaxis (`self.ForwardAxis`))
  (bind _dmi (`self.DMI`))
  (bind (_output_counter _output_counter2) (break `/Game/MiniGames3/Blueprints/Data/F_MG_TunnelRing` (`|GetArrayItem` (`self.Tunnel`) 1)))
  (`parent.ReceiveTick` DeltaSeconds)
  (set `self.DeltaTime` DeltaSeconds)
  (if (`self.IsMiniGameActivated`)
    (`self.CheckTargetAndBar`)
    (if (>= (`self.CurrBarValue`) (`self.MaxBarValue`))
      ;[1 1 1] Success
      (set `self.MiniGameEnabled` false)
      (set `self.IsMiniGameActivated` false)
      (set `self.InputEnable` false)
      (`MaterialInstanceDynamic.SetScalarParameterValue` (`self.DMI`) "ShowEnabled" 1.0)
      (`KismetSystemLibrary.Delay` (`self.DelayTimeWhenComplete`))
      (`self.SetOfflineMaterial`)
      (`self.OnMiniGameSuccess`)
      (`self.BlendCameraFromGameToPlayer` (`self.OverlappedActor`))
      (else
        ;[1 1 1] Check and update position based on user input
        (`|ExecutionSequence`
          (:`then_0`
            (set `self.Xpos` (`KismetMathLibrary.FClamp` (`KismetMathLibrary.FInterpTo` (`self.Xpos`) (`self.XposNew`) (`self.DeltaTime`) 1.0) -0.5 0.5))
            (set `self.Ypos` (`KismetMathLibrary.FClamp` (`KismetMathLibrary.FInterpTo` (`self.Ypos`) (`self.YposNew`) (`self.DeltaTime`) 1.0) -0.25 0.25))
            (`MaterialInstanceDynamic.SetScalarParameterValue` _dmi "Xpos" (`self.Xpos`))
            (`MaterialInstanceDynamic.SetScalarParameterValue` _dmi "Ypos" (`self.Ypos`))
            ;[1 1 1] Update all tunnel rings
            (for (_array_element _array_index) _tunnel
              (bind (_counter _counter2 _scalecounter) (break `/Game/MiniGames3/Blueprints/Data/F_MG_TunnelRing` _array_element))
              (bind (_result1 _result2) (`self.GetCoordinate` _counter _counter2))
              (`MaterialInstanceDynamic.SetVectorParameterValue` (`self.DMI`) (`KismetStringLibrary.Conv_StringToName` (`KismetStringLibrary.Concat_StrStr` "Ring" (`KismetStringLibrary.Conv_IntToString` (+ _array_index 1)))) (make `LinearColor` _result1 _result2 (`KismetMathLibrary.Lerp` 0.51 0.9 _scalecounter) _scalecounter))
              (bind _result (`self.GetClamped` (+ _counter (* (`self.DeltaTime`) (`self.TunnelSpeedX`)))))
              (bind _result_2 (`self.GetClamped` (+ _counter2 (* (`self.DeltaTime`) (`self.TunnelSpeedY`)))))
              (bind (_result_3 _isreset) (`self.GetClamped2` (+ _scalecounter (* (`self.DeltaTime`) (`self.TunnelScaleSpeed`)))))
              (if _isreset
                (`self.ShiftArray`)
                (setmembers `/Game/MiniGames3/Blueprints/Data/F_MG_TunnelRing` :`StructRef` (`|GetArrayItem` (`self.Tunnel`)) :`Counter` (+ _output_counter (/ _returnvalue 12.0)) :`Counter2` (+ _output_counter2 (/ _returnvalue 15.0)) :`ScaleCounter` 0.0)
                (else
                  (setmembers `/Game/MiniGames3/Blueprints/Data/F_MG_TunnelRing` :`StructRef` (`|GetArrayItem` _tunnel _array_index) :`Counter` _result :`Counter2` _result_2 :`ScaleCounter` _result_3)))))
          (:`then_1`
            (if (`self.InputEnable`)
              (`|ExecutionSequence`
                (:`then_0`
                  (if (!= _rightaxis 0.0)
                    (set `self.XposNew` (+ (`self.Xpos`) (* (* _rightaxis -1.0) (`self.MoveSpeed`))))))
                (:`then_1`
                  (if (!= _forwardaxis 0.0)
                    (set `self.YposNew` (+ (`self.Ypos`) (* _forwardaxis (`self.MoveSpeed`)) 0.0))))))))))))

(event `CheckTargetAndBar`
  (bind _currbarvalue (`self.CurrBarValue`))
  (bind (_counter _counter2) (break `/Game/MiniGames3/Blueprints/Data/F_MG_TunnelRing` (`|GetArrayItem` (`self.Tunnel`) 6)))
  ;[1 1 1] Check and update prgoress bar if target inside of tunnel
  (bind (_result1 _result2) (`self.GetCoordinate` _counter _counter2))
  (bind _returnvalue (<= (`KismetMathLibrary.VSize2D` (- (`KismetMathLibrary.MakeVector2D` _result1 _result2) (* (`KismetMathLibrary.MakeVector2D` (`self.Xpos`) (`self.Ypos`)) -4.0))) 0.3))
  (`MaterialInstanceDynamic.SetScalarParameterValue` (`self.DMI`) "OnTarget" (`KismetMathLibrary.SelectFloat` 1.0 0.0 _returnvalue))
  (if _returnvalue
    (set `self.CurrBarValue` (`KismetMathLibrary.FClamp` (+ _currbarvalue (* (`self.BarIncreaseSpeed`) (`self.BarDelta`))) 0.0 0.6))
    (else
      (set `self.CurrBarValue` (`KismetMathLibrary.FClamp` (- _currbarvalue (* (`self.BarDecreaseSpeed`) (`self.BarDelta`))) 0.0 0.6))))
  (`MaterialInstanceDynamic.SetScalarParameterValue` (`self.DMI`) "Progress" (`self.CurrBarValue`)))

(event `self.ForceAction`
  ;[1 1 1] Action
  (if (`self.PlayerOverlapped`)
    (if (not (`self.IsMiniGameActivated`))
      (`self.InitGame`)
      (`PrimitiveComponent.SetMaterial` (`self.MiniGameScreen`) 0 (`self.DMI`))
      (`self.BlendCameraFromPlayerToGame` self (`self.OverlappedActor`))
      (set `self.IsMiniGameActivated` true)
      (set `self.InputEnable` true))))

(event `self.ForceExit`
  ;[1 1 1] Cancel
  (if (and (`self.MiniGameEnabled`) (`self.IsMiniGameActivated`))
    (set `self.IsMiniGameActivated` false)
    (set `self.InputEnable` false)
    (`self.OnMiniGameCanceled`)
    (`self.BlendCameraFromGameToPlayer` (`self.OverlappedActor`))))

(event `self.InteractionBoundBox.OnComponentBeginOverlap`
  (params (OverlappedComponent :type "PrimitiveComponent Object Reference") (OtherActor :type "Actor Object Reference") (OtherComp :type "PrimitiveComponent Object Reference") (OtherBodyIndex :type Integer) (bFromSweep :type Boolean) (SweepResult :type "HitResult Structure (by ref)"))
  ;[1 1 1] Overapping events
  (`self.CheckBeginOverlap` OtherActor))

(event `self.InteractionBoundBox.OnComponentEndOverlap`
  (params (OverlappedComponent :type "PrimitiveComponent Object Reference") (OtherActor :type "Actor Object Reference") (OtherComp :type "PrimitiveComponent Object Reference") (OtherBodyIndex :type Integer))
  ;[1 1 1] Overapping events
  (`self.CheckEndOverlap` OtherActor))

(fn `GetClamped`
  (params (Value :type "Float (double-precision)"))
  (returns (Result :type "Float (double-precision)"))
  (locals (Val :type "Float (double-precision)") (Out :type "Float (double-precision)"))
  ;[1 1 1] Get clamped PI value
  (bind _output_get (set `local.Val` Value))
  (if (>= _output_get (* (`KismetMathLibrary.GetPI`) 2.0))
    (set `local.Out` (- (`local.Val`) (* (`KismetMathLibrary.GetPI`) 2.0)))
    (else
      (set `local.Out` (`local.Val`))))
  (return (`local.Out`)))

(fn `GetClamped2`
  (params (Value :type "Float (double-precision)"))
  (returns (Result :type "Float (double-precision)") (IsReset :type Boolean))
  (locals (Out :type "Float (double-precision)") (Reset :type Boolean))
  ;[1 1 1] Get clamped 0...1 value
  (bind _output_get (set `local.Out` Value))
  (set `local.Reset` false)
  (if (>= _output_get 1.0)
    (set `local.Out` 0.0)
    (set `local.Reset` true))
  (return (`local.Out`) (`local.Reset`)))

(fn `GetCoordinate`
  (params (Counter :type "Float (double-precision)") (Counter2 :type "Float (double-precision)"))
  (returns (Result1 :type "Float (double-precision)") (Result2 :type "Float (double-precision)"))
  ;[1 1 1] Get coordinate by counters
  (return (/ (+ (`KismetMathLibrary.Sin` Counter) (`KismetMathLibrary.Sin` (+ (* (`KismetMathLibrary.GetPI`) 12.0) Counter2))) 2.0) (/ (+ (`KismetMathLibrary.Sin` Counter2) (`KismetMathLibrary.Sin` (+ Counter (* (`KismetMathLibrary.GetPI`) 7.0)))) 2.0)))

(fn `SetupTunnel`
  (locals (Scale :type "Float (double-precision)") (DeltaScale :type "Float (double-precision)") (Counter1 :type "Float (double-precision)") (Counter2 :type "Float (double-precision)"))
  (bind _returnvalue (`KismetMathLibrary.GetPI`))
  ;[1 1 1] Setup tunnel counters
  (set `local.DeltaScale` (/ 1.0 (`KismetMathLibrary.Conv_IntToDouble` (`self.RingsCount`))))
  (set `local.Counter1` (`KismetMathLibrary.RandomFloatInRange` 0.0 _returnvalue))
  (set `local.Counter2` (`KismetMathLibrary.RandomFloatInRange` 0.0 (* _returnvalue 2.0)))
  (`KismetArrayLibrary.Array_Clear` (`self.Tunnel`))
  (for _ (range (`self.RingsCount`))
    (`KismetArrayLibrary.Array_Add` (`self.Tunnel`) (make `/Game/MiniGames3/Blueprints/Data/F_MG_TunnelRing` (`local.Counter1`) (`local.Counter2`) (`local.Scale`)))
    (set `local.Scale` (+ (`local.Scale`) (`local.DeltaScale`)))
    (bind _result (`self.GetClamped` (+ (`local.Counter1`) (/ (`KismetMathLibrary.GetPI`) 12.0))))
    (set `local.Counter1` _result)
    (bind _result_2 (`self.GetClamped` (+ (`local.Counter2`) (/ (`KismetMathLibrary.GetPI`) 15.0))))
    (set `local.Counter2` _result_2)))

(fn `ShiftArray`
  (locals (LastValue :type "/Game/MiniGames3/Blueprints/Data/F_MG_TunnelRing Structure"))
  (bind _tunnel (`self.Tunnel`))
  ;[1 1 1] Shift array from low to height index
  (set `local.LastValue` (`|GetArrayItem` (`self.Tunnel`) 6))
  (for _index (range 6)
    (bind _returnvalue (- 5 _index))
    (`|VariableSetRef` (`|GetArrayItem` _tunnel (+ _returnvalue 1)) (`|GetArrayItem` _tunnel _returnvalue)))
  (`|VariableSetRef` (`|GetArrayItem` _tunnel) (`local.LastValue`)))

(fn `UserConstructionScript`
  (`parent.UserConstructionScript`))