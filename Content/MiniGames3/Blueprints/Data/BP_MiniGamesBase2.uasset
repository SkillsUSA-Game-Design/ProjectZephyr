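; Base Blueprint for in-world mini-game machines, handling player detection, screen state and enter/exit input.
; Custom overlap events track the player, while a looping timer compares facing against an arrow to toggle the key prompt on the idle screen material.
; Interact and cancel inputs call empty ForceAction and ForceExit events meant for overriding.
; Helpers switch idle/offline materials, blend the camera and hide the player; axis inputs store deadzoned values.
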(event `EnableMiniGame`
  ;[1 1 1] Init
  (`PrimitiveComponent.SetMaterial` (`self.MiniGameScreen`) 0 (`self.DMI_Idle`) :!label _label)
  (set `self.MiniGameEnabled` true))

(event `self.ReceiveBeginPlay`
  ;[1 1 1] Init
  (bind _returnvalue (`KismetSystemLibrary.K2_SetTimer` null "CheckPlayerDirection" 0.15 true))
  (set `self.CheckPlayerDirectionHandle` _returnvalue)
  (set `self.PlayerOverlapped` false)
  (set `self.PlayerDetected` false)
  (set `self.IsMiniGameActivated` false)
  (set `self.InputEnable` true)
  (set `self.RightAxis` 0.0)
  (set `self.ForwardAxis` 0.0)
  ;;[1 1 1] Idle material
  (bind _returnvalue_2 (`KismetMaterialLibrary.CreateDynamicMaterialInstance` "/Game/MiniGames3/Materials/MI_MiniGamesIdle_Inst.MI_MiniGamesIdle_Inst"))
  (set `self.DMI_Idle` _returnvalue_2)
  ;;[1 1 1] Offline material
  (bind _returnvalue_3 (`KismetMaterialLibrary.CreateDynamicMaterialInstance` "/Game/MiniGames3/Materials/MI_MiniGameOffline_Inst.MI_MiniGameOffline_Inst"))
  (set `self.DMI_Offline` _returnvalue_3)
  (if (`self.MiniGameEnabled`)
    (goto _label)
    (else
      (`PrimitiveComponent.SetMaterial` (`self.MiniGameScreen`) 0 (`self.DMI_Offline`) :!label _label_2)
      (set `self.MiniGameEnabled` false))))

(event `DisableMiniGame`
  ;[1 1 1] Init
  (goto _label_2))

(event `InputAxis|Input_Forward` :consume false
  (params (AxisValue :type "Float (single-precision)"))
  ;[1 1 1] Controls
  (if (>= (`KismetMathLibrary.Abs` AxisValue) (`self.GamepadSensitivity`))
    (set `self.ForwardAxis` AxisValue)
    (else
      (set `self.ForwardAxis` 0.0))))

(event `CheckBeginOverlap`
  (params (Actor :type "Actor Object Reference"))
  (bind _playerpawn (`self.PlayerPawn`))
  ;[1 1 1] Check overlapped Player
  (if (`KismetSystemLibrary.IsValid` _playerpawn)
    (if (== Actor _playerpawn)
      (set `self.PlayerDetected` true :!label _label_3)
      (set `self.OverlappedActor` Actor))
    (else
      (goto _label_3))))

(event `InputAxis|Input_Right` :consume false
  (params (AxisValue :type "Float (single-precision)"))
  ;[1 1 1] Controls
  (if (>= (`KismetMathLibrary.Abs` AxisValue) (`self.GamepadSensitivity`))
    (set `self.RightAxis` AxisValue)
    (else
      (set `self.RightAxis` 0.0))))

(event `CheckEndOverlap`
  (params (Actor :type "Actor Object Reference"))
  ;[1 1 1] Check overlapped Player
  (if (`self.PlayerDetected`)
    (if (== Actor (`self.OverlappedActor`))
      (set `self.PlayerDetected` false)
      (set `self.PlayerOverlapped` false)
      (set `self.OverlappedActor` null)
      (`MaterialInstanceDynamic.SetScalarParameterValue` (`self.DMI_Idle`) "ShowKey" 0.0))))

(event `InputAction|Input_Interact`
  (params (Key :type "Key Structure"))
  ;[1 1 1] Action
  (:`Pressed`
    (if (`self.MiniGameEnabled`)
      (if (`self.PlayerOverlapped`)
        (`self.ForceAction`)))))

(event `CheckPlayerDirection`
  (bind _overlappedactor (`self.OverlappedActor`))
  (bind _dmi_idle (`self.DMI_Idle`))
  ;[1 1 1] Check if player oriented to Mini Game screen
  (if (`self.PlayerDetected`)
    (`/Engine/EditorBlueprintResources/StandardMacros.IsValid` _overlappedactor
      (:`Is Valid`
        (if (<= (`KismetMathLibrary.DegAcos` (`KismetMathLibrary.Dot_VectorVector` (`SceneComponent.GetForwardVector` (`self.Arrow`)) (`self.GetActorForwardVector` _overlappedactor))) (`self.DetectionAngle`))
          (set `self.PlayerOverlapped` true)
          (`MaterialInstanceDynamic.SetScalarParameterValue` _dmi_idle "ShowKey" 1.0)
          (else
            (set `self.PlayerOverlapped` false)
            (`MaterialInstanceDynamic.SetScalarParameterValue` _dmi_idle "ShowKey" 0.0)))))))

(event `InputAction|Input_Uninteract`
  (params (Key :type "Key Structure"))
  ;[1 1 1] Exit (Cancel) game
  (:`Pressed`
    (if (`self.MiniGameEnabled`)
      (if (`self.PlayerOverlapped`)
        (if (`self.IsMiniGameActivated`)
          (`PrimitiveComponent.SetMaterial` (`self.MiniGameScreen`) 0 (`self.DMI_Idle`))
          (`self.ForceExit`))))))

(event `BlendCameraFromPlayerToGame`
  (params (MiniGame :type "Actor Object Reference") (Player :type "Actor Object Reference"))
  (bind _returnvalue (`GameplayStatics.GetPlayerController` 0))
  ;[1 1 1] Camera transition from Player to Mini Game
  (`self.DisableInput` Player _returnvalue)
  (`PlayerController.SetViewTargetWithBlend` _returnvalue MiniGame 0.0 "VTBlend_Linear" 0.0 false)
  (`self.SetActorHiddenInGame` Player true))

(event `ForceAction`
  ;[0 0.3254 1] Overwritable events
)

(event `SetOfflineMaterial`
  ;[1 1 1] Set Offline material for the screen
  (`PrimitiveComponent.SetMaterial` (`self.MiniGameScreen`) 0 (`self.DMI_Offline`)))

(event `ForceExit`
  ;[0 0.3254 1] Overwritable events
)

(event `BlendCameraFromGameToPlayer`
  (params (Player :type "Actor Object Reference"))
  (bind _returnvalue (`GameplayStatics.GetPlayerController` 0))
  ;[1 1 1] Camera Transition from Mini Game to Player
  (`PlayerController.SetViewTargetWithBlend` _returnvalue Player 0.0 "VTBlend_Linear" 0.0 false)
  (`self.EnableInput` Player _returnvalue)
  (`self.SetActorHiddenInGame` Player false))

(fn `UserConstructionScript`)