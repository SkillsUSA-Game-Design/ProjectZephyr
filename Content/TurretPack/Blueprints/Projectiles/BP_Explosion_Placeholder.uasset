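; BP_Explosion_Placeholder is a self-destroying placeholder explosion effect in the turret pack's projectile Blueprints.
; The construction script gives the sphere a dynamic instance of M_Explosion.
; On BeginPlay, a timeline scales up the sphere, fades its color from yellow to transparent black and dims the point light, then destroys the actor.
; In parallel, a radial force fires one impulse and is removed after a brief delay.
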(event `self.ReceiveBeginPlay`
  (`|ExecutionSequence`
    (:`then_0`
      (bind (_direction _size _color) (`Timeline|Timeline_0` :!via `PlayFromStart`) ; Explosion Animation
        (:`Update`
          (`SceneComponent.SetWorldScale3D` (`self.Sphere`) (`KismetMathLibrary.VLerp` (0.1 0.1 0.1) (8.0 8.0 8.0) _size))
          (`MaterialInstanceDynamic.SetVectorParameterValue` (`self.Material`) "Color" (`KismetMathLibrary.LinearColorLerp` (struct :`R` 1.0 :`G` 0.901284 :`A` 1.0) (struct) _color))
          (`LightComponent.SetIntensity` (`self.PointLight`) (`KismetMathLibrary.Lerp` 30000.0 0.0 _size)))
        (:`Finished`
          (`self.K2_DestroyActor`))))
    (:`then_1`
      (`RadialForceComponent.FireImpulse` (`self.RadialForce`))
      (`KismetSystemLibrary.Delay` 0.1)
      (`ActorComponent.K2_DestroyComponent` (`self.RadialForce`)))))

(fn `UserConstructionScript`
  (bind _sphere (`self.Sphere`))
  (bind _returnvalue (`PrimitiveComponent.CreateDynamicMaterialInstance` _sphere 0 "/Game/TurretPack/Materials/Projectiles/M_Explosion.M_Explosion" "None"))
  (bind _output_get (set `self.Material` _returnvalue))
  (`PrimitiveComponent.SetMaterial` _sphere 0 _output_get))