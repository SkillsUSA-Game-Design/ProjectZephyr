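; BP_Target_Spawner is a placed actor that spawns and respawns BP_TargetPawn targets for the turret pack.
; On play it destroys its preview mesh, waits an initial delay, then spawns a target at its transform, passing destination, health, friendliness and speed.
; A once-per-second poll watches the target and spawns a replacement after a respawn delay once it is gone.
; The construction script applies the friendly material to the preview mesh.
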(event `self.ReceiveBeginPlay`
  (`ActorComponent.K2_DestroyComponent` (`self.StaticMesh`))
  (`KismetSystemLibrary.Delay` (`self.InitialMovement_Delay`))
  (bind _returnvalue (`|SpawnActorFromClass` "/Game/TurretPack/Blueprints/Environment/BP_TargetPawn.BP_TargetPawn_C" (`self.GetTransform`) "Undefined" "OverrideRootScale" null (`self.MoveTo`) (`self.Health`) (`self.Friendly?`) (`self.Speed`) true null :!label _label))
  (`/Engine/EditorBlueprintResources/StandardMacros.IsValid` _returnvalue :!label _label_2
    (:`Is Valid`
      (`KismetSystemLibrary.Delay` 1.0)
      (goto _label_2))
    (:`Is Not Valid`
      (`KismetSystemLibrary.Delay` (`self.Respawn_Delay`))
      (goto _label))))

(fn `UserConstructionScript`
  (if (`self.Friendly?`)
    (`PrimitiveComponent.SetMaterial` (`self.StaticMesh`) 0 "/Game/TurretPack/Materials/Environment/MI_Target_Friendly.MI_Target_Friendly")))