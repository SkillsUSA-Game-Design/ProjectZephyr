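; Pushable button actor that plays a press animation and sound when the player interacts with it nearby.
; A box overlap with TestCharacter opens and closes a gate on the Interact input, so presses register only within range.
; The Button_Animation graph lerps the mesh between its starting transform and an inset one captured at BeginPlay, using one timeline to push in and another played in reverse to return.
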(event `self.ReceiveBeginPlay`
  (bind (_returnvalue_location _returnvalue_rotation _returnvalue_scale) (`KismetMathLibrary.BreakTransform` (`SceneComponent.GetRelativeTransform` (`self.Button`))))
  (set `self.Out Position` (`KismetMathLibrary.MakeTransform` _returnvalue_location _returnvalue_rotation _returnvalue_scale))
  (set `self.In Position` (`KismetMathLibrary.MakeTransform` (- _returnvalue_location (0.0 10.0 0.0)) _returnvalue_rotation _returnvalue_scale))
  (`self.EnableInput` (`GameplayStatics.GetPlayerController` 0)))

(event `InputAction|Input_Interact`
  (params (Key :type "Key Structure"))
  ;[1 1 1] Button Interaction (Push Button)
  (:`Pressed`
    (`/Engine/EditorBlueprintResources/StandardMacros.Gate` true :!label _label
      (:`Exit`
        (`GameplayStatics.PlaySoundAtLocation` "/Game/SoundEffects/Expansion/Split/Sounds_IP/Button.Button" (`self.K2_GetActorLocation`) (struct) 1.0 1.0 0.0 null null null)
        (bind (_direction _button_in) (`Timeline|Button In` :!via `PlayFromStart`)
          (:`Update`
            (`SceneComponent.K2_SetRelativeTransform` (`self.Button`) (`KismetMathLibrary.TLerp` (`self.Out Position`) (`self.In Position`) _button_in) false false))
          (:`Finished`
            (bind (_direction_2 _button_in_2) (`Timeline|Button_Out` :!via `ReverseFromEnd`)
              (:`Update`
                (`SceneComponent.K2_SetRelativeTransform` (`self.Button`) (`KismetMathLibrary.TLerp` (`self.Out Position`) (`self.In Position`) _button_in_2) false false)))))))))

(event `self.Box.OnComponentBeginOverlap`
  (params (OverlappedComponent :type "PrimitiveComponent Object Reference") (OtherActor :type "Actor Object Reference") (OtherComp :type "PrimitiveComponent Object Reference") (OtherBodyIndex :type Integer) (bFromSweep :type Boolean) (SweepResult :type "HitResult Structure (by ref)"))
  ;[1 1 1] Button Interaction (Push Button)
  (cast `/Game/TestObjects/TestCharacter` OtherActor)
  (goto _label :!via `Open`))

(event `self.Box.OnComponentEndOverlap`
  (params (OverlappedComponent :type "PrimitiveComponent Object Reference") (OtherActor :type "Actor Object Reference") (OtherComp :type "PrimitiveComponent Object Reference") (OtherBodyIndex :type Integer))
  ;[1 1 1] Button Interaction (Push Button)
  (cast `/Game/TestObjects/TestCharacter` OtherActor)
  (goto _label :!via `Close`))

(fn `UserConstructionScript`)