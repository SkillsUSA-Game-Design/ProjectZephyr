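; Projectile actor from a lightning electricity effects pack that launches forward on begin play via a velocity impulse on its physics Sphere.
; On the first hit it stops physics and collision and spawns a Niagara hit effect tinted blue through user color parameters.
; A timeline then drives the size parameter of the Energy effect before the actor destroys itself.
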(event `self.ReceiveBeginPlay`
  (`PrimitiveComponent.AddImpulse` (`self.Sphere`) (* (`SceneComponent.GetForwardVector` (`self.Sphere`)) (`self.Speed`)) "None" true))

(event `self.ReceiveHit`
  (params (MyComp :type "PrimitiveComponent Object Reference") (Other :type "Actor Object Reference") (OtherComp :type "PrimitiveComponent Object Reference") (bSelfMoved :type Boolean) (HitLocation :type "Vector Structure") (HitNormal :type "Vector Structure") (NormalImpulse :type "Vector Structure") (Hit :type "HitResult Structure (by ref)"))
  (bind _sphere (`self.Sphere`))
  (bind (_returnvalue_location _returnvalue_rotation) (`KismetMathLibrary.BreakTransform` (`SceneComponent.K2_GetComponentToWorld` (`self.Sphere`))))
  (`/Engine/EditorBlueprintResources/StandardMacros.DoOnce` false
    (:`Completed`
      (`PrimitiveComponent.SetSimulatePhysics` _sphere false)
      (`PrimitiveComponent.SetCollisionEnabled` _sphere "NoCollision")
      (bind _returnvalue (`NiagaraFunctionLibrary.SpawnSystemAtLocation` "/Game/Lightning_Electricity_Pack/Particles/V1_4/P_Hit_v1_4.P_Hit_v1_4" _returnvalue_location _returnvalue_rotation))
      (`FXSystemComponent.SetColorParameter` _returnvalue "User.color" (struct :`G` 0.23074 :`B` 1.0 :`A` 1.0))
      (`FXSystemComponent.SetColorParameter` _returnvalue "User.color_02" (struct :`R` 0.005986 :`G` 0.367294 :`B` 1.0 :`A` 1.0))
      (bind (_direction _end) (`Timeline|Timeline_0` :!via `PlayFromStart`)
        (:`Update`
          (`FXSystemComponent.SetFloatParameter` (`self.Energy`) "User.System_Size" _end))
        (:`Finished`
          (`self.K2_DestroyActor`))))))

(fn `UserConstructionScript`)