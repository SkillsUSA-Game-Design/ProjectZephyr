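; Looping punch effect actor from the lightning and electricity pack that moves a sphere and fires a Punch effect.
; After an initial FirstDelay, the Movement timeline drives the sphere along its relative X axis.
; At the end of the forward stroke, Punch activates just ahead of the sphere with matching rotation.
; The same timeline then reverses at a slower rate and restarts after a pause, branching on its direction.
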(event `Again`
  (bind _punch (`self.Punch`))
  (bind _sphere (`self.Sphere`))
  (bind (_returnvalue_location _returnvalue_rotation) (`KismetMathLibrary.BreakTransform` (`SceneComponent.K2_GetComponentToWorld` _sphere)))
  (`TimelineComponent.SetPlayRate` (`self.Movement`) 1.0 :!label _label)
  (bind (_direction _newtrack_0) (`Timeline|Movement` :!via `PlayFromStart` :!label _label_2)
    (:`Update`
      (`SceneComponent.K2_SetRelativeLocation` (`self.Sphere`) (`KismetMathLibrary.MakeVector` _newtrack_0) false false))
    (:`Finished`
      (if (`|EnumEquality` _direction "Forward")
        (`SceneComponent.K2_SetWorldLocationAndRotation` _punch (+ (* (`SceneComponent.GetForwardVector` _sphere) 10.0) _returnvalue_location) _returnvalue_rotation false false)
        (`ActorComponent.Activate` _punch true)
        (`KismetSystemLibrary.Delay` 0.5)
        (`self.Reverse`)
        (else
          (`KismetSystemLibrary.Delay` 1.0)
          (`self.Again`))))))

(event `self.ReceiveBeginPlay`
  (`KismetSystemLibrary.Delay` (`self.FirstDelay`))
  (goto _label))

(event `Reverse`
  (`TimelineComponent.SetPlayRate` (`self.Movement`) 0.3)
  (goto _label_2 :!via `ReverseFromEnd`))

(fn `UserConstructionScript`)