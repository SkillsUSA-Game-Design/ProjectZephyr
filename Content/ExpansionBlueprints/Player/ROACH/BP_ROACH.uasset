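; BP_ROACH is the player's ROACH companion actor, which can hover beside the player character.
; While Following is set, Tick eases it toward a raised offset to the target's right and matches the TestCharacter spring arm's rotation.
; BeginPlay targets the player, but nothing connected in this graph turns Following on.
; Enable and Disable show or hide it and toggle its box collision.
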(event `self.ReceiveTick`
  (params (DeltaSeconds :type "Float (single-precision)"))
  (bind _target (`self.Target`))
  (bind (_returnvalue_x _returnvalue_y _returnvalue_z) (`KismetMathLibrary.BreakVector` (`self.GetActorRightVector` _target)))
  ;[1 1 1] Set Roach Location and Rotation
  (if (`self.Following`)
    (`self.K2_SetActorLocation` (`KismetMathLibrary.VInterpTo` (`self.K2_GetActorLocation`) (+ (`self.K2_GetActorLocation` _target) (`KismetMathLibrary.MakeVector` (* _returnvalue_x 75.0) (* _returnvalue_y 75.0) (+ _returnvalue_z 50.0))) DeltaSeconds))
    (bind _astest_character (cast `/Game/TestObjects/TestCharacter` (`GameplayStatics.GetPlayerCharacter` 0)))
    (`self.K2_SetActorRotation` (`SpringArmComponent.GetTargetRotation` (`/Game/TestObjects/TestCharacter.SpringArm` _astest_character)))))

(event `self.ReceiveBeginPlay`
  ;[1 1 1] Lock Roach location on spawn, will change based on story beats
  (set `self.Target` (`GameplayStatics.GetPlayerCharacter` 0)))

(event `/Game/ExpansionBlueprints/Interface/BPI_Enable_Disable.Enable`
  ;[1 1 1] Spawn ROACH
  (`self.SetActorHiddenInGame` false)
  (`PrimitiveComponent.SetCollisionEnabled` (`self.Box`) "QueryAndPhysics"))

(event `/Game/ExpansionBlueprints/Interface/BPI_Enable_Disable.Disable`
  ;[1 1 1] DeSpawn ROACH
  (`self.SetActorHiddenInGame` true)
  (`PrimitiveComponent.SetCollisionEnabled` (`self.Box`) "NoCollision"))

(fn `UserConstructionScript`)