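; Waypoint actor that scripts the ROACH companion's movement away from the player, back to them, or on to a linked next location.
; LocationType sets behaviour flags in the construction script, and Enable runs the matching moves with optional teleport-in, despawn and placeholder printed dialogue.
; Fast looping timers interpolate ROACH's position and rotation with speed ramps, toggle its follow tick, and can enable the next location to form a chain.
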(event `/Game/ExpansionBlueprints/Interface/BPI_Enable_Disable.Disable`
  ;[1 1 1] Disable/Destroy
  (`self.K2_DestroyActor`))

(event `self.ReceiveBeginPlay`
  ;[1 1 1] GetReference to Roach
  (bind _returnvalue (`GameplayStatics.GetActorOfClass` "/Game/ExpansionBlueprints/Player/ROACH/BP_ROACH.BP_ROACH_C"))
  (set `self.ROACH` _returnvalue))

(event `/Game/ExpansionBlueprints/Interface/BPI_Enable_Disable.Enable`
  ;[1 1 1] Enable Independent Roach Movement
  (bind _asbp_roach (cast `/Game/ExpansionBlueprints/Player/ROACH/BP_ROACH` (`self.ROACH`)))
  (`|ExecutionSequence`
    (:`then_0`
      ;[1 1 1] Roach Leaves Player
      (if (`self.Roach Leave Player`)
        (set `/Game/ExpansionBlueprints/Player/ROACH/BP_ROACH.Following` false _asbp_roach)
        (`self.SetActorTickEnabled` _asbp_roach false)
        (bind _returnvalue (`KismetSystemLibrary.K2_SetTimerDelegate` (delegate `RoatToDestination`) 0.001 true))))
    (:`then_1`
      ;[1 1 1] Roach Joins Player
      (if (`self.Roach Join Player`)
        (if (`self.SpawnAtLocation`)
          (`self.K2_SetActorLocation` _asbp_roach (`self.K2_GetActorLocation`) false false)
          (message `/Game/ExpansionBlueprints/Interface/BPI_Enable_Disable.Enable` _asbp_roach))
        (bind _astest_character (cast `/Game/TestObjects/TestCharacter` (`GameplayStatics.GetPlayerCharacter` 0)))
        (bind _returnvalue_2 (`KismetSystemLibrary.K2_SetTimerDelegate` (delegate `RoachToPlayer`) 0.001 true))
        (set `self.TimeToPlayer` (`GameplayStatics.GetUnpausedTimeSeconds`))))
    (:`then_2`
      ;[1 1 1] Roach Moves to Next Location
      (if (not (`self.Roach Leave Player`))
        (if (`self.GoToNextLocation`) :!label _label
          (if (`self.SpawnAtLocation`)
            (`self.K2_SetActorLocation` _asbp_roach (`self.K2_GetActorLocation`) false false)
            (message `/Game/ExpansionBlueprints/Interface/BPI_Enable_Disable.Enable` _asbp_roach))
          (set `self.TimeToDestination` (`GameplayStatics.GetWorldDeltaSeconds`))
          (bind _returnvalue_3 (`KismetSystemLibrary.K2_SetTimerDelegate` (delegate `RoachToNextLocation`) 0.001 true)))))
    (:`then_3`
      ;[1 1 1] Despawn At Location
      (if (`self.DespawnAtLocation`)
        (if (== (`self.K2_GetActorLocation` _asbp_roach) (`self.K2_GetActorLocation`) :`ErrorTolerance` 50.0)
          (`KismetSystemLibrary.Delay` (`self.DespawnDelay`))
          (message `/Game/ExpansionBlueprints/Interface/BPI_Enable_Disable.Disable` _asbp_roach))))
    (:`then_4`
      ;[1 1 1] PlayDialogue (Place Holder, will change with addition of UI/Audio Voice Lines
      (if (`self.PlayDialogue`)
        (`KismetSystemLibrary.PrintString` (`|GetArrayItem` (`self.VoiceLines`) (`self.LineIndex`)) true true (struct :`G` 0.66 :`B` 1.0 :`A` 1.0) (`self.LineDuration`))
        (set `self.LineIndex` (+ (`self.LineIndex`) 1))
        (bind _returnvalue_4 (`KismetSystemLibrary.K2_SetTimerDelegate` (delegate `DisplayDialogue`) (`self.LineDuration`) true))))))

(event `RoatToDestination`
  ;[1 1 1] Roach Leaves Player
  (bind _returnvalue (`self.K2_GetActorLocation` (stale `/Game/ExpansionBlueprints/Interface/BPI_Enable_Disable.Enable` _asbp_roach)))
  (`self.K2_SetActorLocation` (stale `/Game/ExpansionBlueprints/Interface/BPI_Enable_Disable.Enable` _asbp_roach) (`KismetMathLibrary.VInterpTo` _returnvalue (`self.K2_GetActorLocation`) (`GameplayStatics.GetWorldDeltaSeconds`) (`self.SpeedToDestination`)) false false)
  (`self.K2_SetActorRotation` (stale `/Game/ExpansionBlueprints/Interface/BPI_Enable_Disable.Enable` _asbp_roach) (`KismetMathLibrary.RInterpTo` (`self.K2_GetActorRotation` (stale `/Game/ExpansionBlueprints/Interface/BPI_Enable_Disable.Enable` _asbp_roach)) (`KismetMathLibrary.FindLookAtRotation` (`self.K2_GetActorLocation` (stale `/Game/ExpansionBlueprints/Interface/BPI_Enable_Disable.Enable` _asbp_roach)) (`self.K2_GetActorLocation`)) (`GameplayStatics.GetWorldDeltaSeconds`) 5.0) false)
  (if (== (`self.K2_GetActorLocation`) _returnvalue :`ErrorTolerance` 100.0)
    (set `self.SpeedToNextDestination` 0.1)
    (`KismetSystemLibrary.K2_ClearAndInvalidateTimerHandle` (stale `/Game/ExpansionBlueprints/Interface/BPI_Enable_Disable.Enable` _returnvalue))
    (if (`self.GoToNextLocation`)
      (goto _label))
    (elif (not (< (- (`GameplayStatics.GetWorldDeltaSeconds`) (`self.TimeToDestination`)) 2.0))
      (set `self.SpeedToNextDestination` (* (`self.SpeedToNextDestination`) 1.01)))))

(event `RoachToPlayer`
  ;[1 1 1] Roach Joins Player
  (bind _target (`/Game/ExpansionBlueprints/Player/ROACH/BP_ROACH.Target` (stale `/Game/ExpansionBlueprints/Interface/BPI_Enable_Disable.Enable` _asbp_roach)))
  (bind (_returnvalue_x _returnvalue_y _returnvalue_z) (`KismetMathLibrary.BreakVector` (`self.GetActorRightVector` _target)))
  (bind _returnvalue (+ (`self.K2_GetActorLocation` _target) (`KismetMathLibrary.MakeVector` (* _returnvalue_x 50.0) (* _returnvalue_y 50.0) (+ _returnvalue_z 100.0))))
  (`self.K2_SetActorLocation` (stale `/Game/ExpansionBlueprints/Interface/BPI_Enable_Disable.Enable` _asbp_roach) (`KismetMathLibrary.VInterpTo` (`self.K2_GetActorLocation` (stale `/Game/ExpansionBlueprints/Interface/BPI_Enable_Disable.Enable` _asbp_roach)) _returnvalue (`GameplayStatics.GetWorldDeltaSeconds`) (`self.SpeedToPlayer`)) false false)
  (bind (_returnvalue_x_2 _returnvalue_y_2) (`KismetMathLibrary.BreakVector` (`KismetMathLibrary.Vector_GetAbs` (- (`self.K2_GetActorLocation` (stale `/Game/ExpansionBlueprints/Interface/BPI_Enable_Disable.Enable` _asbp_roach)) _returnvalue))))
  (if (and (<= _returnvalue_x_2 300.0) (<= _returnvalue_y_2 300.0))
    (`self.K2_SetActorRotation` (stale `/Game/ExpansionBlueprints/Interface/BPI_Enable_Disable.Enable` _asbp_roach) (`KismetMathLibrary.RInterpTo` (`self.K2_GetActorRotation` (stale `/Game/ExpansionBlueprints/Interface/BPI_Enable_Disable.Enable` _asbp_roach)) (`SpringArmComponent.GetTargetRotation` (`/Game/TestObjects/TestCharacter.SpringArm` (stale `/Game/ExpansionBlueprints/Interface/BPI_Enable_Disable.Enable` _astest_character))) (`GameplayStatics.GetWorldDeltaSeconds`) (`self.RoachRotationSpeed`)) false)
    (else
      (`self.K2_SetActorRotation` (stale `/Game/ExpansionBlueprints/Interface/BPI_Enable_Disable.Enable` _asbp_roach) (`KismetMathLibrary.RInterpTo` (`self.K2_GetActorRotation` (stale `/Game/ExpansionBlueprints/Interface/BPI_Enable_Disable.Enable` _asbp_roach)) (`KismetMathLibrary.FindLookAtRotation` (`self.K2_GetActorLocation` (stale `/Game/ExpansionBlueprints/Interface/BPI_Enable_Disable.Enable` _asbp_roach)) (`self.K2_GetActorLocation` (stale `/Game/ExpansionBlueprints/Interface/BPI_Enable_Disable.Enable` _astest_character))) (`GameplayStatics.GetWorldDeltaSeconds`) 5.0) false)))
  (if (== (`self.K2_GetActorLocation` (stale `/Game/ExpansionBlueprints/Interface/BPI_Enable_Disable.Enable` _asbp_roach)) _returnvalue :`ErrorTolerance` 2.0)
    (`KismetSystemLibrary.K2_ClearAndInvalidateTimerHandle` (stale `/Game/ExpansionBlueprints/Interface/BPI_Enable_Disable.Enable` _returnvalue_2))
    (set `/Game/ExpansionBlueprints/Player/ROACH/BP_ROACH.Following` true (stale `/Game/ExpansionBlueprints/Interface/BPI_Enable_Disable.Enable` _asbp_roach))
    (`self.SetActorTickEnabled` (stale `/Game/ExpansionBlueprints/Interface/BPI_Enable_Disable.Enable` _asbp_roach) true)
    (elif (>= (- (`GameplayStatics.GetUnpausedTimeSeconds`) (`self.TimeToPlayer`)) 2.0)
      (set `self.SpeedToPlayer` (* (`self.SpeedToPlayer`) 1.001))
      (set `self.RoachRotationSpeed` (* (`self.RoachRotationSpeed`) 1.001)))))

(event `RoachToNextLocation`
  ;[1 1 1] Roach Moves to Next Location
  (`self.K2_SetActorLocation` (stale `/Game/ExpansionBlueprints/Interface/BPI_Enable_Disable.Enable` _asbp_roach) (`KismetMathLibrary.VInterpTo` (`self.K2_GetActorLocation` (stale `/Game/ExpansionBlueprints/Interface/BPI_Enable_Disable.Enable` _asbp_roach)) (`self.K2_GetActorLocation` (`self.NextLocation`)) (`GameplayStatics.GetWorldDeltaSeconds`) (`self.SpeedToNextDestination`)) false false)
  (`self.K2_SetActorRotation` (stale `/Game/ExpansionBlueprints/Interface/BPI_Enable_Disable.Enable` _asbp_roach) (`KismetMathLibrary.RInterpTo` (`self.K2_GetActorRotation` (stale `/Game/ExpansionBlueprints/Interface/BPI_Enable_Disable.Enable` _asbp_roach)) (`KismetMathLibrary.FindLookAtRotation` (`self.K2_GetActorLocation` (stale `/Game/ExpansionBlueprints/Interface/BPI_Enable_Disable.Enable` _asbp_roach)) (`self.K2_GetActorLocation` (`self.NextLocation`))) (`GameplayStatics.GetWorldDeltaSeconds`) 5.0) false)
  (if (== (`self.K2_GetActorLocation` (stale `/Game/ExpansionBlueprints/Interface/BPI_Enable_Disable.Enable` _asbp_roach)) (`self.K2_GetActorLocation` (`self.NextLocation`)) :`ErrorTolerance` 50.0)
    (`KismetSystemLibrary.K2_ClearAndInvalidateTimerHandle` (stale `/Game/ExpansionBlueprints/Interface/BPI_Enable_Disable.Enable` _returnvalue_3))
    (if (`self.DespawnAtLocation`)
      (message `/Game/ExpansionBlueprints/Interface/BPI_Enable_Disable.Disable` (stale `/Game/ExpansionBlueprints/Interface/BPI_Enable_Disable.Enable` _asbp_roach))
      (set `self.SpeedToNextDestination` 0.1)
      (else
        (message `/Game/ExpansionBlueprints/Interface/BPI_Enable_Disable.Enable` (`self.NextLocation`))))
    (elif (not (< (- (`GameplayStatics.GetWorldDeltaSeconds`) (`self.TimeToDestination`)) 2.0))
      (set `self.SpeedToNextDestination` (* (`self.SpeedToNextDestination`) 1.05)))))

(event `DisplayDialogue`
  ;[1 1 1] PlayDialogue (Place Holder, will change with addition of UI/Audio Voice Lines
  (`KismetSystemLibrary.PrintString` (`|GetArrayItem` (`self.VoiceLines`) (`self.LineIndex`)) true true (struct :`G` 0.66 :`B` 1.0 :`A` 1.0) (`self.LineDuration`))
  (bind _output_get (set `self.LineIndex` (+ (`self.LineIndex`) 1)))
  (if (== _output_get (`KismetArrayLibrary.Array_Length` (`self.VoiceLines`)))
    (`KismetSystemLibrary.K2_ClearAndInvalidateTimerHandle` (stale `/Game/ExpansionBlueprints/Interface/BPI_Enable_Disable.Enable` _returnvalue_4))))

(fn `UserConstructionScript`
  (switch `/Game/ExpansionBlueprints/Player/ROACH/ExtraFiles/Enum_ROACH_Locations` (`self.Location Type`)
    (:`NewEnumerator0`
      (set `self.Roach Leave Player` true)
      (set `self.Roach Join Player` false)
      (set `self.GoToNextLocation` false))
    (:`NewEnumerator1`
      (set `self.Roach Join Player` true)
      (set `self.Roach Leave Player` false)
      (set `self.GoToNextLocation` false))
    (:`NewEnumerator2`
      (set `self.GoToNextLocation` true)
      (set `self.Roach Join Player` false)
      (set `self.Roach Leave Player` false))
    (:`NewEnumerator3`
      (set `self.Roach Leave Player` true)
      (set `self.GoToNextLocation` true)
      (set `self.Roach Join Player` false))
    (:`NewEnumerator4`
      (set `self.Roach Leave Player` false)
      (set `self.Roach Join Player` false)
      (set `self.GoToNextLocation` false))))