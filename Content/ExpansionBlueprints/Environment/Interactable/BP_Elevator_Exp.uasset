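; BP_Elevator_Exp is an interactable elevator that travels between its starting location and an End offset.
; A box overlap permits interaction, and Enable and Disable interface events switch the elevator on or off.
; Interact runs a timeline, rate-scaled by SecondsToComplete, that lerps the actor's location.
; A DoOnce blocks retriggering until the move finishes, when a FlipFlop toggles the direction for the next trip.
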(event `self.Box.OnComponentEndOverlap`
  (params (OverlappedComponent :type "PrimitiveComponent Object Reference") (OtherActor :type "Actor Object Reference") (OtherComp :type "PrimitiveComponent Object Reference") (OtherBodyIndex :type Integer))
  ;[1 1 1] Enable interaction when standing on platform
  (set `self.can interact` false))

(event `/Game/ExpansionBlueprints/Interface/BPI_Enable_Disable.Enable`
  ;[1 1 1] Enable/Disable Interface Events
  (set `self.Enabled` true))

(event `self.Box.OnComponentBeginOverlap`
  (params (OverlappedComponent :type "PrimitiveComponent Object Reference") (OtherActor :type "Actor Object Reference") (OtherComp :type "PrimitiveComponent Object Reference") (OtherBodyIndex :type Integer) (bFromSweep :type Boolean) (SweepResult :type "HitResult Structure (by ref)"))
  ;[1 1 1] Enable interaction when standing on platform
  (set `self.can interact` true))

(event `/Game/ExpansionBlueprints/Interface/BPI_Enable_Disable.Disable`
  ;[1 1 1] Enable/Disable Interface Events
  (set `self.Enabled` false))

(event `self.ReceiveBeginPlay`
  ;[1 1 1] Initialize Starting Point and Timeline Duration
  (bind _output_get (set `self.StartLocation` (`self.K2_GetActorLocation`)))
  (`TimelineComponent.SetPlayRate` (`self.Timeline_0`) (/ 1.0 (`self.SecondsToComplete`))))

(event `/Game/ExpansionBlueprints/Interface/Interact.Interact`
  (params (Player :type "/Game/TestObjects/TestCharacter Object Reference"))
  ;[1 1 1] Move Elevator when Interacted With
  (if (`self.Enabled`)
    (if (`self.can interact`)
      (set `self.can interact` false)
      (`/Engine/EditorBlueprintResources/StandardMacros.DoOnce` false :!label _label
        (:`Completed`
          (if (`self.Reverse`)
            (bind (_direction _newtrack_0) (`Timeline|Timeline_0` :!via `ReverseFromEnd` :!label _label_2)
              (:`Update`
                (`self.K2_SetActorLocation` (`KismetMathLibrary.VLerp` (stale `self.ReceiveBeginPlay` _output_get) (+ (`self.StartLocation`) (`self.End`)) _newtrack_0)))
              (:`Finished`
                (set `self.can interact` true)
                (`/Engine/EditorBlueprintResources/StandardMacros.FlipFlop`
                  (:`A`
                    (set `self.Reverse` true)
                    (goto _label :!via `Reset`))
                  (:`B`
                    (set `self.Reverse` false)
                    (goto _label :!via `Reset`)))))
            (else
              (goto _label_2 :!via `PlayFromStart`))))))))

(fn `UserConstructionScript`)