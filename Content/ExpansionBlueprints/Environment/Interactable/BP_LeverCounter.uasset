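; BP_LeverCounter is an order-checking counter for a lever puzzle that triggers other actors once solved.
; AddtoCounter records each value passed in, while Enable counts calls until the required sequence length is reached.
; A matching sequence sends enable and disable messages to two actor lists, while a mismatch resets the recorded order and count.
; An alternative per-step check is left disconnected, so validation happens only at the end.
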(event `/Game/ExpansionBlueprints/Interface/BPI_Enable_Disable.Enable`
  (bind _output_get (set `self.LeverCheck` (+ (`self.LeverCheck`) 1)))
  (if (> _output_get (- (`KismetArrayLibrary.Array_Length` (`self.LeverOrderCorrect`)) 1))
    (if (`KismetArrayLibrary.Array_Identical` (`self.LevelOrderCurrent`) (`self.LeverOrderCorrect`))
      (for _array_element (`self.EnabledActor`)
        (message `/Game/ExpansionBlueprints/Interface/BPI_Enable_Disable.Enable` _array_element))
      (for _array_element_2 (`self.DisableActor`)
        (message `/Game/ExpansionBlueprints/Interface/BPI_Enable_Disable.Disable` _array_element_2))
      (else
        (set `self.LevelOrderCurrent` (`self.LeverClear`))
        (set `self.LeverCheck` 0)))))

(event `/Game/ExpansionBlueprints/Environment/Interactable/Additional_Files/BPI_LeverPuzzle.AddToCounter`
  (params (NewParam :type Integer))
  (`KismetArrayLibrary.Array_Add` (`self.LevelOrderCurrent`) NewParam))

(fn `UserConstructionScript`)