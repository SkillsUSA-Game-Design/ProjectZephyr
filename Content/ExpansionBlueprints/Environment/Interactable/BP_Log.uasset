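; BP_Log is an interactable audio log pickup that shows a transcript on screen, then destroys itself.
; On interact it hides its mesh, disables collision and creates a widget.
; A delay loop steps through the Transcript lines at a fixed interval, then removes the widget and the actor.
; The sound playback branch is not connected, so no audio plays.
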(event `/Game/ExpansionBlueprints/Interface/Interact.Interact`
  (params (Player :type "/Game/TestObjects/TestCharacter Object Reference"))
  (if (not (`self.IsPlaying?`))
    (`self.PlayAudioLog`)))

(event `PlayAudioLog`
  ;[1 1 1] Start playing
  (`PrimitiveComponent.SetCollisionEnabled` (`self.StaticMesh`) "NoCollision")
  (`self.SetActorHiddenInGame` true)
  (set `self.TextLine` 0)
  (set `self.IsPlaying?` true)
  (bind _returnvalue (`|CreateWidget` "/Game/ExpansionBlueprints/Environment/Interactable/AudioLogWidget.AudioLogWidget_C"))
  (`UserWidget.AddToViewport` _returnvalue 0)
  (set `/Game/ExpansionBlueprints/Environment/Interactable/AudioLogWidget.MyText` (`|GetArrayItem` (`self.Transcript`) (`self.TextLine`)) _returnvalue :!label _label)
  (`KismetSystemLibrary.Delay` (`self.DelayBetweenLines (seconds)`))
  (if (== (- (`KismetArrayLibrary.Array_Length` (`self.Transcript`)) 1) (`self.TextLine`))
    (`self.StopAudioLog`)
    (else
      (`/Engine/EditorBlueprintResources/StandardMacros.IncrementInt` (`self.TextLine`)
        (:`  `
          (goto _label))))))

(event `StopAudioLog`
  ;[1 1 1] Stop Playing
  (set `self.IsPlaying?` false)
  (`Widget.RemoveFromParent` (stale `PlayAudioLog` _returnvalue))
  (`self.K2_DestroyActor`))

(fn `UserConstructionScript`)