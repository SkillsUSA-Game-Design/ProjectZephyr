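; Radial lock minigame on an interactable screen: the player rotates three linked rings in quarter turns to align with a random solver position.
; A looping timer polls the axes to select and turn rings, with each move also turning other rings.
; InitGame scrambles from the solved state using those same moves.
; Timelines animate dynamic material parameters for rotation and the solve, which reports success and returns the camera to the player.
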(event `self.ReceiveBeginPlay`
  ;[1 1 1] Init
  (`parent.ReceiveBeginPlay`)
  (bind _returnvalue (`KismetMaterialLibrary.CreateDynamicMaterialInstance` "/Game/MiniGames3/Materials/MI_MiniGameRadial_Inst.MI_MiniGameRadial_Inst"))
  (set `self.DMI` _returnvalue)
  (bind _returnvalue_2 (`KismetSystemLibrary.K2_SetTimer` null "CheckContorls" 0.05 true))
  (set `self.ControlsTimeHandle` _returnvalue_2)
  (bind _returnvalue_3 (`KismetSystemLibrary.K2_SetTimer` null "UpdateDecor" 0.1 true))
  (set `self.DecorTimeHandle` _returnvalue_3))

(event `InitGame`
  (bind _dmi (`self.DMI`))
  (bind _solverpos (`self.SolverPos`))
  ;[1 1 1] Setup game
  (bind _output_get (set `self.SolverPos` (`KismetMathLibrary.RandomIntegerInRange` 0 3)))
  (`self.SetupSolver` _output_get)
  (set `self.Selector` 0)
  (`self.SetupSelector`)
  (set `self.Ring1_Index` _solverpos)
  (set `self.Ring2_Index` _solverpos)
  (bind _output_get_2 (set `self.Ring3_Index` _solverpos))
  (bind _angle (`self.GetRotAngleByIndex` _output_get_2))
  (bind _output_get_3 (set `self.Ring1_Rot` _angle))
  (bind _output_get_4 (set `self.Ring2_Rot` _output_get_3))
  (set `self.Ring3_Rot` _output_get_4)
  (`self.PreRollRings`)
  (`MaterialInstanceDynamic.SetScalarParameterValue` _dmi "Ring1_Rot" (`self.Ring1_Rot`))
  (`MaterialInstanceDynamic.SetScalarParameterValue` _dmi "Ring2_Rot" (`self.Ring2_Rot`))
  (`MaterialInstanceDynamic.SetScalarParameterValue` _dmi "Ring3_Rot" (`self.Ring3_Rot`))
  (`MaterialInstanceDynamic.SetScalarParameterValue` _dmi "Flasher" 0.0)
  (`MaterialInstanceDynamic.SetScalarParameterValue` _dmi "ShowUnblocked" 0.0)
  (set `self.IsRotation` false))

(event `SetupSelector`
  (bind _dmi (`self.DMI`))
  ;[1 1 1] Mark selected ring
  (`MaterialInstanceDynamic.SetScalarParameterValue` _dmi "Ring1_Sel" 0.0)
  (`MaterialInstanceDynamic.SetScalarParameterValue` _dmi "Ring2_Sel" 0.0)
  (`MaterialInstanceDynamic.SetScalarParameterValue` _dmi "Ring3_Sel" 0.0)
  (`MaterialInstanceDynamic.SetScalarParameterValue` _dmi (`KismetStringLibrary.Conv_StringToName` (`KismetStringLibrary.Concat_StrStr` "Ring" (`KismetStringLibrary.Conv_IntToString` (+ (`self.Selector`) 1)) "_Sel")) 1.0))

(event `CheckContorls`
  (bind _dmi (`self.DMI`))
  (bind _rightaxis (`self.RightAxis`))
  (bind _forwardaxis (`self.ForwardAxis`))
  (bind _dmi_2 (`self.DMI`))
  ;[1 1 1] Controls
  (if (`self.InputEnable`)
    (if (`self.IsMiniGameActivated`)
      (`|ExecutionSequence`
        (:`then_0`
          (if (!= _rightaxis 0.0)
            (if (`self.RightAxisEnable`)
              (set `self.RightAxisEnable` false)
              (set `self.InputEnable` false)
              (set `self.RotationDirection` (* (`KismetMathLibrary.SignOfFloat` _rightaxis) -1.0))
              (`self.CalcRingRotation` (`self.Selector`))
              (set `self.IsRotation` true)
              (bind (_direction _newtrack_0) (`Timeline|Timeline_0` :!via `PlayFromStart`)
                (:`Update`
                  (`MaterialInstanceDynamic.SetScalarParameterValue` (`self.DMI`) "Ring1_Rot" (`KismetMathLibrary.Lerp` (`self.Ring1_FromRot`) (`self.Ring1_ToRot`) _newtrack_0))
                  (`MaterialInstanceDynamic.SetScalarParameterValue` (`self.DMI`) "Ring2_Rot" (`KismetMathLibrary.Lerp` (`self.Ring2_FromRot`) (`self.Ring2_ToRot`) _newtrack_0))
                  (`MaterialInstanceDynamic.SetScalarParameterValue` (`self.DMI`) "Ring3_Rot" (`KismetMathLibrary.Lerp` (`self.Ring3_FromRot`) (`self.Ring3_ToRot`) _newtrack_0)))
                (:`Finished`
                  (set `self.Ring1_Rot` (`self.Ring1_ToRot`))
                  (set `self.Ring2_Rot` (`self.Ring2_ToRot`))
                  (set `self.Ring3_Rot` (`self.Ring3_ToRot`))
                  (set `self.IsRotation` false)
                  (if (and (== (`self.Ring1_Index`) (`self.SolverPos`)) (== (`self.Ring2_Index`) (`self.SolverPos`)) (== (`self.Ring3_Index`) (`self.SolverPos`)))
                    (`MaterialInstanceDynamic.SetScalarParameterValue` _dmi_2 "Ring1_Sel" 1.0)
                    (`MaterialInstanceDynamic.SetScalarParameterValue` _dmi_2 "Ring2_Sel" 1.0)
                    (`MaterialInstanceDynamic.SetScalarParameterValue` _dmi_2 "Ring3_Sel" 1.0)
                    (`MaterialInstanceDynamic.SetScalarParameterValue` _dmi_2 "Flasher" 1.0)
                    ;;[1 1 1] Draw solver from start to end
                    (switch `int` (`self.SolverPos`)
                      (:`0`
                        (set `self.Solver_Xfrom` 0.46)
                        (set `self.Solver_Xto` 0.46)
                        (set `self.Solver_XSizeFrom` 0.08)
                        (set `self.Solver_XSizeTo` 0.08)
                        (set `self.Solver_Yfrom` 0.07)
                        (set `self.Solver_Yto` 0.07)
                        (set `self.Solver_YSizeFrom` 0.02)
                        (set `self.Solver_YSizeTo` 0.18)
                        (bind (_direction_2 _newtrack_0_2) (`Timeline|Timeline_1` :!via `PlayFromStart` :!label _label)
                          (:`Update`
                            (`MaterialInstanceDynamic.SetScalarParameterValue` _dmi "Solver_XO" (`KismetMathLibrary.Lerp` (`self.Solver_Xfrom`) (`self.Solver_Xto`) _newtrack_0_2))
                            (`MaterialInstanceDynamic.SetScalarParameterValue` _dmi "Solver_YO" (`KismetMathLibrary.Lerp` (`self.Solver_Yfrom`) (`self.Solver_Yto`) _newtrack_0_2))
                            (`MaterialInstanceDynamic.SetScalarParameterValue` _dmi "Solver_XSize" (`KismetMathLibrary.Lerp` (`self.Solver_XSizeFrom`) (`self.Solver_XSizeTo`) _newtrack_0_2))
                            (`MaterialInstanceDynamic.SetScalarParameterValue` _dmi "Solver_YSize" (`KismetMathLibrary.Lerp` (`self.Solver_YSizeFrom`) (`self.Solver_YSizeTo`) _newtrack_0_2)))
                          (:`Finished`
                            ;;[1 1 1] Success
                            (set `self.MiniGameEnabled` false)
                            (set `self.IsMiniGameActivated` false)
                            (set `self.InputEnable` false)
                            (`MaterialInstanceDynamic.SetScalarParameterValue` (`self.DMI`) "ShowUnblocked" 1.0)
                            (`KismetSystemLibrary.Delay` (`self.DelayTimeWhenComplete`))
                            (`self.SetOfflineMaterial`)
                            (`self.OnMiniGameSuccess`)
                            (`self.BlendCameraFromGameToPlayer` (`self.OverlappedActor`)))))
                      (:`1`
                        (set `self.Solver_Xfrom` 0.685)
                        (set `self.Solver_Xto` 0.525)
                        (set `self.Solver_XSizeFrom` 0.02)
                        (set `self.Solver_XSizeTo` 0.18)
                        (set `self.Solver_Yfrom` 0.234)
                        (set `self.Solver_Yto` 0.234)
                        (set `self.Solver_YSizeFrom` 0.08)
                        (set `self.Solver_YSizeTo` 0.08)
                        (goto _label :!via `PlayFromStart`))
                      (:`2`
                        (set `self.Solver_Xfrom` 0.46)
                        (set `self.Solver_Xto` 0.46)
                        (set `self.Solver_XSizeFrom` 0.08)
                        (set `self.Solver_XSizeTo` 0.08)
                        (set `self.Solver_Yfrom` 0.459)
                        (set `self.Solver_Yto` 0.299)
                        (set `self.Solver_YSizeFrom` 0.02)
                        (set `self.Solver_YSizeTo` 0.18)
                        (goto _label :!via `PlayFromStart`))
                      (:`3`
                        (set `self.Solver_Xfrom` 0.295)
                        (set `self.Solver_Xto` 0.295)
                        (set `self.Solver_XSizeFrom` 0.02)
                        (set `self.Solver_XSizeTo` 0.18)
                        (set `self.Solver_Yfrom` 0.234)
                        (set `self.Solver_Yto` 0.234)
                        (set `self.Solver_YSizeFrom` 0.08)
                        (set `self.Solver_YSizeTo` 0.08)
                        (goto _label :!via `PlayFromStart`)))
                    (else
                      (set `self.InputEnable` true))))))
            (else
              (set `self.RightAxisEnable` true))))
        (:`then_1`
          (if (!= _forwardaxis 0.0)
            (if (`self.ForwardAxisEnable`)
              (set `self.ForwardAxisEnable` false)
              (set `self.Selector` (`KismetMathLibrary.Clamp` (- (`self.Selector`) (`KismetMathLibrary.FTrunc` (`KismetMathLibrary.SignOfFloat` _forwardaxis))) 0 2))
              (`self.SetupSelector`))
            (else
              (set `self.ForwardAxisEnable` true))))))))

(event `self.ForceAction`
  ;[1 1 1] Action
  (if (`self.PlayerOverlapped`)
    (if (not (`self.IsMiniGameActivated`))
      (`self.InitGame`)
      (`PrimitiveComponent.SetMaterial` (`self.MiniGameScreen`) 0 (`self.DMI`))
      (`self.BlendCameraFromPlayerToGame` self (`self.OverlappedActor`))
      (set `self.IsMiniGameActivated` true)
      (set `self.InputEnable` true))))

(event `UpdateDecor`
  (bind _dmi (`self.DMI`))
  ;[1 1 1] Update Decor
  (if (`self.IsMiniGameActivated`)
    (`MaterialInstanceDynamic.SetScalarParameterValue` _dmi "DecorText4" (`KismetMathLibrary.Conv_IntToDouble` (`KismetMathLibrary.RandomIntegerInRange` 0 31)))
    (if (`self.IsRotation`)
      (`MaterialInstanceDynamic.SetScalarParameterValue` _dmi "DecorText1" (`KismetMathLibrary.Conv_IntToDouble` (`KismetMathLibrary.RandomIntegerInRange` 0 31)))
      (`MaterialInstanceDynamic.SetScalarParameterValue` _dmi "DecorText2" (`KismetMathLibrary.Conv_IntToDouble` (`KismetMathLibrary.RandomIntegerInRange` 0 31)))
      (`MaterialInstanceDynamic.SetScalarParameterValue` _dmi "DecorText3" (`KismetMathLibrary.Conv_IntToDouble` (`KismetMathLibrary.RandomIntegerInRange` 0 31))))))

(event `self.InteractionBoundBox.OnComponentBeginOverlap`
  (params (OverlappedComponent :type "PrimitiveComponent Object Reference") (OtherActor :type "Actor Object Reference") (OtherComp :type "PrimitiveComponent Object Reference") (OtherBodyIndex :type Integer) (bFromSweep :type Boolean) (SweepResult :type "HitResult Structure (by ref)"))
  ;[1 1 1] Overlap events
  (`self.CheckBeginOverlap` OtherActor))

(event `self.InteractionBoundBox.OnComponentEndOverlap`
  (params (OverlappedComponent :type "PrimitiveComponent Object Reference") (OtherActor :type "Actor Object Reference") (OtherComp :type "PrimitiveComponent Object Reference") (OtherBodyIndex :type Integer))
  ;[1 1 1] Overlap events
  (`self.CheckEndOverlap` OtherActor))

(event `CalcRingRotation`
  (params (SelectorIndex :type Integer))
  (bind _rotationdirection (`self.RotationDirection`))
  (bind _ring1_rot (`self.Ring1_Rot`))
  (bind _rotationdirection_2 (`self.RotationDirection`))
  (bind _ring3_rot (`self.Ring3_Rot`))
  (bind _returnvalue (* (`self.RotationDirection`) -1.0))
  ;[1 1 1] Calculate From To rotation for all rings
  (switch `int` SelectorIndex
    (:`0`
      (bind (_index _fromangle _toangle) (`self.GetRotIndex` (`self.Ring1_Index`) _returnvalue (`self.Ring1_Rot`)))
      (set `self.Ring1_Index` _index)
      (set `self.Ring1_FromRot` _fromangle)
      (set `self.Ring1_ToRot` _toangle)
      (bind (_index_2 _fromangle_2 _toangle_2) (`self.GetRotIndex` (`self.Ring3_Index`) _returnvalue (`self.Ring3_Rot`)))
      (set `self.Ring3_Index` _index_2)
      (set `self.Ring3_FromRot` _fromangle_2)
      (set `self.Ring3_ToRot` _toangle_2)
      (bind (_index_3 _fromangle_3 _toangle_3) (`self.GetRotIndex` (`self.Ring2_Index`) _returnvalue (`self.Ring2_Rot`)))
      (set `self.Ring2_Index` _index_3)
      (set `self.Ring2_FromRot` _fromangle_3)
      (set `self.Ring2_ToRot` _toangle_3))
    (:`1`
      (bind (_index_4 _fromangle_4 _toangle_4) (`self.GetRotIndex` (`self.Ring2_Index`) (* _rotationdirection_2 -1.0) (`self.Ring2_Rot`)))
      (set `self.Ring2_Index` _index_4)
      (set `self.Ring2_FromRot` _fromangle_4)
      (set `self.Ring2_ToRot` _toangle_4)
      (bind (_index_5 _fromangle_5 _toangle_5) (`self.GetRotIndex` (`self.Ring1_Index`) _rotationdirection_2 (`self.Ring1_Rot`)))
      (set `self.Ring1_Index` _index_5)
      (set `self.Ring1_FromRot` _fromangle_5)
      (set `self.Ring1_ToRot` _toangle_5)
      (set `self.Ring3_FromRot` _ring3_rot)
      (set `self.Ring3_ToRot` _ring3_rot))
    (:`2`
      (bind (_index_6 _fromangle_6 _toangle_6) (`self.GetRotIndex` (`self.Ring3_Index`) (* _rotationdirection -1.0) (`self.Ring3_Rot`)))
      (set `self.Ring3_Index` _index_6)
      (set `self.Ring3_FromRot` _fromangle_6)
      (set `self.Ring3_ToRot` _toangle_6)
      (bind (_index_7 _fromangle_7 _toangle_7) (`self.GetRotIndex` (`self.Ring2_Index`) _rotationdirection (`self.Ring2_Rot`)))
      (set `self.Ring2_Index` _index_7)
      (set `self.Ring2_FromRot` _fromangle_7)
      (set `self.Ring2_ToRot` _toangle_7)
      (set `self.Ring1_FromRot` _ring1_rot)
      (set `self.Ring1_ToRot` _ring1_rot))))

(event `self.ForceExit`
  ;[1 1 1] Cancel
  (if (and (`self.MiniGameEnabled`) (`self.IsMiniGameActivated`))
    (set `self.IsMiniGameActivated` false)
    (set `self.InputEnable` false)
    (`self.OnMiniGameCanceled`)
    (`self.BlendCameraFromGameToPlayer` (`self.OverlappedActor`))))

(fn `GetRotAngleByIndex`
  (params (Index :type Integer))
  (returns (Angle :type "Float (double-precision)"))
  (locals (OutAngle :type "Float (double-precision)"))
  ;[1 1 1] Return rotation valuse by index
  (switch `int` Index
    (:`0`
      (set `local.OutAngle` 0.0))
    (:`1`
      (set `local.OutAngle` 0.75))
    (:`2`
      (set `local.OutAngle` 0.5))
    (:`3`
      (set `local.OutAngle` 0.25)))
  (return (`local.OutAngle`)))

(fn `GetRotIndex`
  (params (CurrIndex :type Integer) (Sign :type "Float (double-precision)") (InAngle :type "Float (double-precision)"))
  (returns (Index :type Integer) (FromAngle :type "Float (double-precision)") (ToAngle :type "Float (double-precision)"))
  (locals (OutIndex :type Integer) (OutAngle :type "Float (double-precision)") (OutFromAngle :type "Float (double-precision)"))
  (bind _outindex (`local.OutIndex`))
  (if (== InAngle 1.0)
    (set `local.OutFromAngle` 0.0)
    (else
      (set `local.OutFromAngle` InAngle)))
  (bind _output_get (set `local.OutIndex` (+ CurrIndex (`KismetMathLibrary.FTrunc` Sign))))
  (if (> _output_get 3)
    (set `local.OutIndex` 0)
    (elif (< _output_get 0)
      (set `local.OutIndex` 3)))
  (if (and (== CurrIndex 0) (== _outindex 1))
    (set `local.OutFromAngle` 1.0))
  (bind _angle (`self.GetRotAngleByIndex` (`local.OutIndex`)))
  (set `local.OutAngle` _angle)
  (if (and (== _outindex 0) (== CurrIndex 1))
    (set `local.OutAngle` 1.0))
  (return (`local.OutIndex`) (`local.OutFromAngle`) (`local.OutAngle`)))

(fn `PreRollRings`
  (locals (Count :type Integer))
  ;[1 1 1] Randomly pre roll ring on start game. For variations
  (set `local.Count` (`KismetMathLibrary.RandomIntegerInRange` 1 2))
  (set `self.RotationDirection` (`KismetMathLibrary.SelectFloat` 1.0 -1.0 (>= (`KismetMathLibrary.RandomIntegerInRange` 0 10) 5)))
  (for _ (range (+ (`local.Count`) 1))
    (`self.CalcRingRotation` 0)
    (set `self.Ring1_Rot` (`self.Ring1_ToRot`) :!label _label)
    (set `self.Ring2_Rot` (`self.Ring2_ToRot`))
    (set `self.Ring3_Rot` (`self.Ring3_ToRot`)))
  (set `local.Count` (`KismetMathLibrary.RandomIntegerInRange` 1 2))
  (set `self.RotationDirection` (`KismetMathLibrary.SelectFloat` 1.0 -1.0 (>= (`KismetMathLibrary.RandomIntegerInRange` 0 10) 5)))
  (for _ (range (+ (`local.Count`) 1))
    (`self.CalcRingRotation` 1)
    (goto _label))
  (set `local.Count` (`KismetMathLibrary.RandomIntegerInRange` 1 3))
  (set `self.RotationDirection` (`KismetMathLibrary.SelectFloat` 1.0 -1.0 (>= (`KismetMathLibrary.RandomIntegerInRange` 0 10) 5)))
  (for _ (range (+ (`local.Count`) 1))
    (`self.CalcRingRotation` 2)
    (goto _label)))

(fn `SetupSolver`
  (params (Position :type Integer))
  (locals (XO :type "Float (double-precision)") (YO :type "Float (double-precision)") (Xsize :type "Float (double-precision)") (Ysize :type "Float (double-precision)"))
  (bind _dmi (`self.DMI`))
  ;[1 1 1] Setup coords solver by index
  (switch `int` Position
    (:`0`
      (set `local.XO` 0.46)
      (set `local.YO` 0.07)
      (set `local.Xsize` 0.08)
      (set `local.Ysize` 0.02))
    (:`1`
      (set `local.XO` 0.685)
      (set `local.YO` 0.234)
      (set `local.Xsize` 0.02)
      (set `local.Ysize` 0.08))
    (:`2`
      (set `local.XO` 0.46)
      (set `local.YO` 0.459)
      (set `local.Xsize` 0.08)
      (set `local.Ysize` 0.02))
    (:`3`
      (set `local.XO` 0.295)
      (set `local.YO` 0.234)
      (set `local.Xsize` 0.02)
      (set `local.Ysize` 0.08)))
  (`MaterialInstanceDynamic.SetScalarParameterValue` _dmi "Solver_XO" (`local.XO`))
  (`MaterialInstanceDynamic.SetScalarParameterValue` _dmi "Solver_YO" (`local.YO`))
  (`MaterialInstanceDynamic.SetScalarParameterValue` _dmi "Solver_XSize" (`local.Xsize`))
  (`MaterialInstanceDynamic.SetScalarParameterValue` _dmi "Solver_YSize" (`local.Ysize`)))

(fn `UserConstructionScript`
  (`parent.UserConstructionScript`))