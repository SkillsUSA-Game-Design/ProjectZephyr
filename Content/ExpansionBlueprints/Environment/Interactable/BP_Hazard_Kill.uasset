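; BP_Hazard_Kill is an environmental hazard volume that damages actors entering its box, in one-time, continuous or kill mode.
; The construction script turns the HazardType selection into mode flags that the overlap event checks.
; One-time applies Damage once, while kill applies a large fixed amount.
; Continuous damages immediately and on a looping timer until overlap ends, toggling a ContinuousDamage flag on the TestCharacter found by class.
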(event `self.Box.OnComponentEndOverlap`
  (params (OverlappedComponent :type "PrimitiveComponent Object Reference") (OtherActor :type "Actor Object Reference") (OtherComp :type "PrimitiveComponent Object Reference") (OtherBodyIndex :type Integer))
  ;[1 0.3947 0] Apply Continuous Damage
  (set `/Game/TestObjects/TestCharacter.ContinuousDamage` false (stale `self.Box.OnComponentBeginOverlap` _returnvalue))
  (`KismetSystemLibrary.K2_ClearAndInvalidateTimerHandle` (stale `self.Box.OnComponentBeginOverlap` _returnvalue_2)))

(event `self.Box.OnComponentBeginOverlap`
  (params (OverlappedComponent :type "PrimitiveComponent Object Reference") (OtherActor :type "Actor Object Reference") (OtherComp :type "PrimitiveComponent Object Reference") (OtherBodyIndex :type Integer) (bFromSweep :type Boolean) (SweepResult :type "HitResult Structure (by ref)"))
  ;[0 1 0.1986] Select Action Based on Hazard Type
  (bind _returnvalue (`GameplayStatics.GetActorOfClass` "/Game/TestObjects/TestCharacter.TestCharacter_C"))
  (if (`self.OneTime`)
    ;[1 0.9286 0] Apply Damage Once
    (`GameplayStatics.ApplyDamage` OtherActor (`self.Damage`))
    (elif (`self.Continuous`)
      ;[1 0.3947 0] Apply Continuous Damage
      (set `/Game/TestObjects/TestCharacter.ContinuousDamage` true _returnvalue)
      (`GameplayStatics.ApplyDamage` OtherActor (`self.Damage`) null null "/Game/ExpansionBlueprints/Environment/Interactable/Additional_Files/Continuous.Continuous_C")
      (bind _returnvalue_2 (`KismetSystemLibrary.K2_SetTimerDelegate` (delegate `DamageTick`) (`self.ContinuousInterval`) true))
      (elif (`self.Kill`)
        ;[1 0 0.06489] Kill Player
        (`GameplayStatics.ApplyDamage` OtherActor 99.0)))))

(event `DamageTick`
  ;[1 0.3947 0] Apply Continuous Damage
  (`GameplayStatics.ApplyDamage` (stale `self.Box.OnComponentBeginOverlap` OtherActor) (`self.Damage`) null null "/Game/ExpansionBlueprints/Environment/Interactable/Additional_Files/Continuous.Continuous_C"))

(fn `UserConstructionScript`
  (switch `/Game/ExpansionBlueprints/Environment/Interactable/Additional_Files/Hazard_Kill` (`self.HazardType`)
    (:`NewEnumerator0`
      (set `self.OneTime` true)
      (set `self.Continuous` false)
      (set `self.Kill` false))
    (:`NewEnumerator1`
      (set `self.OneTime` false)
      (set `self.Continuous` true)
      (set `self.Kill` false))
    (:`NewEnumerator2`
      (set `self.OneTime` false)
      (set `self.Continuous` false)
      (set `self.Kill` true))))