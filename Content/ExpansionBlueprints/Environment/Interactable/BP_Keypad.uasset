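; Interactable code keypad that opens a linked Door when the player enters the matching KeypadCode.
; Its collision box registers it on TestCharacter, and LookAt blends to a close-up camera, hides the player mesh, locks movement and resets the display to placeholder dots.
; Child-actor buttons receive a keypad reference; Press handles digits, backspace and confirm.
; A correct code opens the door and restores the player view, while a wrong one clears the entry.
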(event `LookAt`
  (bind _enteredcode (`self.EnteredCode`))
  ;[1 1 1] On interact, do move camera to show close up keypad, and reset keypad display
  (`PlayerController.SetViewTargetWithBlend` (`GameplayStatics.GetPlayerController` 0) (`ActorComponent.GetOwner` (`self.Camera`)) 0.4 "VTBlend_Linear" 0.0 false)
  (bind _astest_character (cast `/Game/TestObjects/TestCharacter` (`GameplayStatics.GetPlayerCharacter` 0)))
  (`SceneComponent.SetVisibility` (`Character.Mesh` _astest_character) false false)
  (`Controller.SetIgnoreMoveInput` (`GameplayStatics.GetPlayerController` 0) true)
  (`TextRenderComponent.K2_SetText` _enteredcode (`KismetSystemLibrary.MakeLiteralText` (`KismetTextLibrary.Conv_StringToText` (`KismetStringLibrary.GetSubstring` "...................." 0 (`KismetStringLibrary.Len` (`self.KeypadCode`))))))
  (`TextRenderComponent.SetTextRenderColor` _enteredcode (make `Color` 200 200 200 255))
  (bind _output_get (set `self.ButtonsArray` (`|MakeArray` (`self.Button0`) (`self.Button1`) (`self.Button2`) (`self.Button3`) (`self.Button4`) (`self.Button5`) (`self.Button6`) (`self.Button7`) (`self.Button8`) (`self.Button9`) (`self.ButtonBack`) (`self.ButtonEnter`))))
  (for _array_element _output_get
    (bind _asbp_keypad_button (cast `/Game/ExpansionBlueprints/Environment/Interactable/BP_KeypadButton` (`ChildActorComponent.ChildActor` _array_element)))
    (set `/Game/ExpansionBlueprints/Environment/Interactable/BP_KeypadButton.KeypadActorRef` self _asbp_keypad_button)))

(event `self.CollisionBox.OnComponentBeginOverlap`
  (params (OverlappedComponent :type "PrimitiveComponent Object Reference") (OtherActor :type "Actor Object Reference") (OtherComp :type "PrimitiveComponent Object Reference") (OtherBodyIndex :type Integer) (bFromSweep :type Boolean) (SweepResult :type "HitResult Structure (by ref)"))
  ;[1 1 1] Send self to player if colliding
  (if (== OtherActor (`GameplayStatics.GetPlayerPawn` 0))
    (bind _astest_character (cast `/Game/TestObjects/TestCharacter` OtherActor))
    (set `/Game/TestObjects/TestCharacter.Keypad Ref` self _astest_character)))

(event `self.CollisionBox.OnComponentEndOverlap`
  (params (OverlappedComponent :type "PrimitiveComponent Object Reference") (OtherActor :type "Actor Object Reference") (OtherComp :type "PrimitiveComponent Object Reference") (OtherBodyIndex :type Integer))
  ;[1 1 1] Null Keypad Reference when Exiting view
  (if (== OtherActor (`GameplayStatics.GetPlayerPawn` 0))
    (bind _astest_character (cast `/Game/TestObjects/TestCharacter` OtherActor))
    (set `/Game/TestObjects/TestCharacter.Keypad Ref` null _astest_character)))

(event `Press`
  (params (Value :type Text) (`Is Confirm?` :type Boolean) (`Is Back?` :type Boolean))
  (bind _enteredcode (`self.EnteredCode`))
  ;[1 1 1] On Key Press
  (if (`KismetStringLibrary.EqualEqual_StrStr` (`KismetTextLibrary.Conv_TextToString` (`TextRenderComponent.Text` (`self.EnteredCode`))) (`KismetStringLibrary.GetSubstring` "...................." 0 (`KismetStringLibrary.Len` (`self.KeypadCode`))))
    (`TextRenderComponent.K2_SetText` (`self.EnteredCode`) Value)
    (elif (`self.CanEnter?`)
      (if `Is Back?`
        (`self.Backspace`)
        (elif `Is Confirm?`
          (`self.Enter`)
          (elif (< (`KismetStringLibrary.Len` (`KismetTextLibrary.Conv_TextToString` (`TextRenderComponent.Text` (`self.EnteredCode`)))) (`KismetStringLibrary.Len` (`self.KeypadCode`)))
            (`TextRenderComponent.SetTextRenderColor` (`self.EnteredCode`) (make `Color` 255 255 255 255))
            (`TextRenderComponent.K2_SetText` _enteredcode (`KismetTextLibrary.Conv_StringToText` (`KismetStringLibrary.Concat_StrStr` (`KismetTextLibrary.Conv_TextToString` (`TextRenderComponent.Text` _enteredcode)) (`KismetTextLibrary.Conv_TextToString` Value))))))))))

(event `LookAway`
  ;[1 1 1] Exit Camera View
  (`PlayerController.SetViewTargetWithBlend` (`GameplayStatics.GetPlayerController` 0) (`ActorComponent.GetOwner` (`/Game/TestObjects/TestCharacter.Camera` (cast `/Game/TestObjects/TestCharacter` (`GameplayStatics.GetPlayerPawn` 0) :!pure true))) 0.4 "VTBlend_Linear" 0.0 false)
  (`SceneComponent.SetVisibility` (`Character.Mesh` (`GameplayStatics.GetPlayerCharacter` 0)) true false)
  (`Controller.SetIgnoreMoveInput` (`GameplayStatics.GetPlayerController` 0) false))

(event `Enter`
  ;[1 1 1] Enter
  (if (== (`self.KeypadCode`) (`KismetTextLibrary.Conv_TextToString` (`TextRenderComponent.Text` (`self.EnteredCode`))))
    (`PlayerController.SetViewTargetWithBlend` (`GameplayStatics.GetPlayerController` 0) (`ActorComponent.GetOwner` (`/Game/TestObjects/TestCharacter.Camera` (cast `/Game/TestObjects/TestCharacter` (`GameplayStatics.GetPlayerPawn` 0) :!pure true))) 0.4 "VTBlend_Linear" 0.0 false)
    (`/Game/ExpansionBlueprints/Environment/Interactable/BP_Door.Open` (`self.Door`))
    (`SceneComponent.SetVisibility` (`Character.Mesh` (`GameplayStatics.GetPlayerCharacter` 0)) true false)
    (`Controller.SetIgnoreMoveInput` (`GameplayStatics.GetPlayerController` 0) false)
    (else
      (`TextRenderComponent.K2_SetText` (`self.EnteredCode`) (`KismetSystemLibrary.MakeLiteralText` (`KismetTextLibrary.Conv_StringToText` ""))))))

(event `Backspace`
  (bind _returnvalue (`KismetTextLibrary.Conv_TextToString` (`TextRenderComponent.Text` (`self.EnteredCode`))))
  ;[1 1 1] Enter
  ;;[1 1 1] Backspace
  (`TextRenderComponent.K2_SetText` (`self.EnteredCode`) (`KismetTextLibrary.Conv_StringToText` (`KismetStringLibrary.GetSubstring` _returnvalue 0 (- (`KismetStringLibrary.Len` _returnvalue) 1)))))

(fn `UserConstructionScript`
  (`TextRenderComponent.SetTextRenderColor` (`self.EnteredCode`) (make `Color` 200 200 200 255)))