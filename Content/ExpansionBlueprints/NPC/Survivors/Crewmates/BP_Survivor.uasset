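; BP_Survivor is a crewmate survivor NPC that can be shown or hidden and plays timed dialogue when interacted with.
; Enable and Disable toggle actor visibility together with capsule collision.
; Interact, gated by DoOnce so it runs only once, creates a dialogue widget and steps through the Dialogue array using a looping Delay of LineDuration.
; EndDialogue removes the widget after the last line.
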(event `/Game/ExpansionBlueprints/Interface/BPI_Enable_Disable.Enable`
  (`self.SetActorHiddenInGame` false)
  (`PrimitiveComponent.SetCollisionEnabled` (`self.CapsuleComponent`) "QueryAndPhysics"))

(event `/Game/ExpansionBlueprints/Interface/BPI_Enable_Disable.Disable`
  (`self.SetActorHiddenInGame` true)
  (`PrimitiveComponent.SetCollisionEnabled` (`self.CapsuleComponent`) "NoCollision"))

(event `/Game/ExpansionBlueprints/Interface/Interact.Interact`
  (params (Player :type "/Game/TestObjects/TestCharacter Object Reference"))
  (`/Engine/EditorBlueprintResources/StandardMacros.DoOnce` false
    (:`Completed`
      (bind _returnvalue (`|CreateWidget` "/Game/ExpansionBlueprints/NPC/Survivors/Widgets/Widget_Dialogue.Widget_Dialogue_C"))
      (`UserWidget.AddToViewport` _returnvalue 0)
      (set `/Game/ExpansionBlueprints/NPC/Survivors/Widgets/Widget_Dialogue.Dialogue` (`|GetArrayItem` (`self.Dialogue`) (`self.DialogeLineNumber`)) _returnvalue :!label _label)
      (`KismetSystemLibrary.Delay` (`self.LineDuration`))
      (if (== (- (`KismetArrayLibrary.Array_Length` (`self.Dialogue`)) 1) (`self.DialogeLineNumber`))
        (`self.EndDialogue`)
        (else
          (`/Engine/EditorBlueprintResources/StandardMacros.IncrementInt` (`self.DialogeLineNumber`)
            (:`  `
              (goto _label))))))))

(event `EndDialogue`
  (`Widget.RemoveFromParent` (stale `/Game/ExpansionBlueprints/Interface/Interact.Interact` _returnvalue)))

(fn `UserConstructionScript`)