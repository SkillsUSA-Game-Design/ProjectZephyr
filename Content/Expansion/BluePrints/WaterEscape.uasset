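; WaterEscape is an overlap-driven actor that starts a moving element, likely rising water in an escape sequence, and damages a TestCharacter on later contact.
; When the character's WaterV flag is unset, an overlap activates InterpToMovement, destroys the Box1 component and sets the flag.
; Overlaps with the flag already set call the character's GrinderDamageEvent, so the character's state separates trigger from hazard.
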(event `self.ReceiveActorBeginOverlap`
  (params (OtherActor :type "Actor Object Reference"))
  (bind _astest_character (cast `/Game/TestObjects/TestCharacter` OtherActor))
  (if (`/Game/TestObjects/TestCharacter.WaterV` _astest_character)
    (bind _astest_character_2 (cast `/Game/TestObjects/TestCharacter` OtherActor))
    (`/Game/TestObjects/TestCharacter.GrinderDamageEvent` _astest_character_2)
    (else
      (`ActorComponent.Activate` (`self.InterpToMovement`) false)
      (`ActorComponent.K2_DestroyComponent` (`self.Box1`))
      (bind _astest_character_3 (cast `/Game/TestObjects/TestCharacter` OtherActor))
      (set `/Game/TestObjects/TestCharacter.WaterV` true _astest_character_3))))

(fn `UserConstructionScript`)