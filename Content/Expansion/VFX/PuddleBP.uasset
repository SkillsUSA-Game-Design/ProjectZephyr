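; PuddleBP is a decal actor that places a randomized puddle on the ground for visual variety.
; All logic runs in the Construction Script, which creates a dynamic material instance on the decal and sets its puddle texture to one of two random choices.
; It then gives the decal an independent random scale on each axis and a random yaw, with pitch fixed for downward projection.
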(fn `UserConstructionScript`
  (bind _returnvalue (`KismetMathLibrary.RandomFloatInRange` 0.3 0.7))
  (bind _decal (`self.Decal`))
  ;[1 1 1] Setting Random Puddle Texture
  (bind _returnvalue_2 (`DecalComponent.CreateDynamicMaterialInstance` (`self.Decal`)))
  (`MaterialInstanceDynamic.SetTextureParameterValue` _returnvalue_2 "Puddle Texture" (select `int` (`KismetMathLibrary.RandomInteger` 2) :`0` (`self.Texture 1`) :`1` (`self.Texture 2`)))
  ;[1 1 1] Set Random Scale
  (`SceneComponent.SetRelativeScale3D` _decal (`KismetMathLibrary.MakeVector` _returnvalue _returnvalue _returnvalue))
  ;[1 1 1] Set Random Rotation
  (`SceneComponent.K2_SetRelativeRotation` _decal (`KismetMathLibrary.MakeRotator` 0.0 -90.0 (`KismetMathLibrary.RandomFloatInRange` 0.0 360.0)) false false))