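; Homing turret missile that flies with launch sound and smoke trail, explodes on impact, and self-destructs after a timeout.
; BeginPlay passes the homing target and acceleration to ProjectileMovement and excludes the instigator from damage.
; Tick detects impacts with a short forward line trace, then once spawns an explosion, applies radial damage and pushes physics objects.
; The spent missile hides, stops, detaches its effects and homing target, then destroys itself after a delay.
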(event `self.ReceiveBeginPlay`
  (bind _projectilemovement (`self.ProjectileMovement`))
  (`|ExecutionSequence`
    (:`then_0`
      (`KismetSystemLibrary.Delay` (`self.AutoDeathTimer`))
      (`/Engine/EditorBlueprintResources/StandardMacros.IsValid` self
        (:`Is Valid`
          (`self.K2_DestroyActor`))))
    (:`then_1`
      (`KismetArrayLibrary.Array_Add` (`self.IgnoreActors_Damage`) (`self.GetInstigator`))
      (set `ProjectileMovementComponent.HomingTargetComponent` (`self.HomingTarget`) _projectilemovement)
      (set `ProjectileMovementComponent.HomingAccelerationMagnitude` (`self.HomingAccelerationMagnitude`) _projectilemovement)
      (bind _returnvalue (`GameplayStatics.SpawnSoundAttached` (`self.MissileLaunchSound`) (`self.SM_Turret_A_Missile`) "None" (0.0 0.0 0.0) (struct) "KeepRelativeOffset" false 1.0 1.0 0.0 null null))
      (set `self.LaunchSound` _returnvalue)
      (bind _returnvalue_2 (`GameplayStatics.SpawnEmitterAttached` "/Game/ZEPHYR/TurretPack/Effects/P_RocketSmoke.P_RocketSmoke" (`self.SM_Turret_A_Missile`) "None" (`SceneComponent.RelativeLocation` (`self.Arrow`)) (struct) (1.0 1.0 1.0) "KeepRelativeOffset" false))
      (set `self.SmokeEmmitter` _returnvalue_2))))

(event `self.ReceiveTick`
  (params (DeltaSeconds :type "Float (single-precision)"))
  (bind _homingtarget (`self.HomingTarget`))
  (bind _sm_turret_a_missile (`self.SM_Turret_A_Missile`))
  (bind _launchsound (`self.LaunchSound`))
  (bind _smokeemmitter (`self.SmokeEmmitter`))
  (bind _returnvalue (`SceneComponent.K2_GetComponentLocation` _sm_turret_a_missile))
  (bind (_outhit _returnvalue_2) (`KismetSystemLibrary.LineTraceSingle` :`Start` _returnvalue :`End` (+ _returnvalue (* (`SceneComponent.GetForwardVector` _sm_turret_a_missile) 100.0)) :`TraceChannel` "TraceTypeQuery1" :`TraceColor` (struct :`R` 1.0 :`G` 0.998104 :`A` 1.0) :`TraceHitColor` (struct) :`DrawTime` 0.05))
  (if _returnvalue_2
    (`/Engine/EditorBlueprintResources/StandardMacros.DoOnce` false
      (:`Completed`
        (bind (_bblockinghit _binitialoverlap _time _distance _location _impactpoint _normal _impactnormal _physmat _hitactor _hitcomponent) (`GameplayStatics.BreakHitResult` _outhit))
        (`|SpawnActorFromClass` "/Game/ZEPHYR/TurretPack/Blueprints/Projectiles/BP_Explosion_Placeholder.BP_Explosion_Placeholder_C" (`KismetMathLibrary.MakeTransform` _location) "AlwaysSpawn" "OverrideRootScale" (`self.GetOwner`) null)
        (if (`SceneComponent.IsSimulatingPhysics` _hitcomponent "None")
          (`PrimitiveComponent.AddImpulse` _hitcomponent (* (`SceneComponent.GetForwardVector` (`self.SM_Turret_A_Missile`)) 300.0) "None" true))
        (`GameplayStatics.ApplyRadialDamage` (`self.Damage`) _location 800.0 null (`self.IgnoreActors_Damage`) null null)
        (`/Engine/EditorBlueprintResources/StandardMacros.IsValid` _launchsound
          (:`Is Valid`
            (`SceneComponent.K2_DetachFromComponent` _launchsound "KeepWorld" "KeepWorld" "KeepWorld" true))
          (:`Is Not Valid`
            _))
        (`GameplayStatics.PlaySoundAtLocation` "/Game/ZEPHYR/TurretPack/Sounds/Damage/SC_Explosion.SC_Explosion" _location (struct) 1.0 1.0 0.0 null null null)
        (`SceneComponent.K2_DetachFromComponent` _smokeemmitter "KeepWorld" "KeepWorld" "KeepWorld" true)
        (`ActorComponent.Deactivate` _smokeemmitter)
        (`ActorComponent.Deactivate` (`self.ProjectileMovement`))
        (`/Engine/EditorBlueprintResources/StandardMacros.IsValid` _homingtarget
          (:`Is Valid`
            (`SceneComponent.K2_DetachFromComponent` _homingtarget "KeepWorld" "KeepWorld" "KeepWorld" true))
          (:`Is Not Valid`
            _))
        (`SceneComponent.SetVisibility` (`self.SM_Turret_A_Missile`) false false)
        (`SceneComponent.SetVisibility` (`self.PointLight`) false false)
        (`KismetSystemLibrary.Delay` 5.0)
        (`self.K2_DestroyActor`)))))

(fn `UserConstructionScript`)