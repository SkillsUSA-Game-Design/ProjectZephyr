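; Minigun turret bullet projectile with randomized speed and a configurable color on its mesh material and point light, self-destroyed after a timeout.
; Hits on anything but the instigator, matched by display name, spawn sparks along the mirrored ricochet direction and fading bullet-hole and heat decals.
; Physics-simulating targets get a velocity-scaled impulse and attached decals, others get world-placed decals.
; The bullet then destroys itself and applies damage.
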(event `self.ReceiveBeginPlay`
  ;[1 1 1] Kill Self if alive for more than "Auto Death Timer" seconds
  (`KismetSystemLibrary.Delay` (`self.AutoDeathTimer`))
  (`/Engine/EditorBlueprintResources/StandardMacros.IsValid` self
    (:`Is Valid`
      (`self.K2_DestroyActor`))))

(event `self.SM_Bullet.OnComponentHit`
  (params (HitComponent :type "PrimitiveComponent Object Reference") (OtherActor :type "Actor Object Reference") (OtherComp :type "PrimitiveComponent Object Reference") (NormalImpulse :type "Vector Structure") (Hit :type "HitResult Structure (by ref)"))
  (bind (_bblockinghit _binitialoverlap _time _distance _location _impactpoint _normal _impactnormal _physmat _hitactor _hitcomponent) (`GameplayStatics.BreakHitResult` Hit))
  (bind _sm_bullet (`self.SM_Bullet`))
  (bind _impactpoint_2 (`self.ImpactPoint`))
  (bind _impactpoint_3 (`self.ImpactPoint`))
  (bind _returnvalue (`SceneComponent.K2_GetComponentLocation` _sm_bullet))
  (bind _returnvalue_2 (`KismetMathLibrary.Conv_VectorToRotator` (`self.ImpactNormal`)))
  (bind _returnvalue_3 (`KismetMathLibrary.Conv_VectorToRotator` (`self.ImpactNormal`)))
  (if (not (`KismetStringLibrary.EqualEqual_StrStr` (`KismetSystemLibrary.GetDisplayName` (`self.GetInstigator`)) (`KismetSystemLibrary.GetDisplayName` OtherActor)))
    (set `self.BulletCollisionHit` true)
    (set `self.ImpactPoint` _impactpoint)
    (set `self.Hit Location` _location)
    (set `self.Normal` _normal)
    (set `self.ImpactNormal` _impactnormal)
    (set `self.HitActor` _hitactor)
    (set `self.HitComponent` _hitcomponent)
    ;[1 1 1] Hit Events
    (`GameplayStatics.SpawnEmitterAtLocation` "/Game/ZEPHYR/TurretPack/Effects/P_Bullet_Sparks.P_Bullet_Sparks" (`self.Hit Location`) (`KismetMathLibrary.FindLookAtRotation` (+ (`self.Normal`) _impactpoint_2) (+ _impactpoint_2 (`KismetMathLibrary.MirrorVectorByNormal` (- (+ _returnvalue (* (`SceneComponent.GetForwardVector` _sm_bullet) 10.0)) _returnvalue) (`self.ImpactNormal`)))) (3.0 3.0 3.0) false)
    (if (`SceneComponent.IsSimulatingPhysics` (`self.HitComponent`) "None")
      (`PrimitiveComponent.AddImpulseAtLocation` (`self.HitComponent`) (* (`self.GetVelocity`) (`self.PhysicsImpulse_Intensity`)) (`self.ImpactPoint`) "None")
      (bind _returnvalue_4 (`GameplayStatics.SpawnDecalAttached` "/Game/ZEPHYR/TurretPack/Materials/Projectiles/M_Decal_BulletHole.M_Decal_BulletHole" (10.0 10.0 10.0) (`self.HitComponent`) "None" (`self.ImpactPoint`) _returnvalue_3 "KeepWorldPosition" 10.0))
      (`DecalComponent.SetFadeOut` _returnvalue_4 5.0 5.0 false)
      (bind _returnvalue_5 (`GameplayStatics.SpawnDecalAttached` "/Game/ZEPHYR/TurretPack/Materials/Projectiles/M_Decal_BulletHeat.M_Decal_BulletHeat" (10.0 10.0 10.0) (`self.HitComponent`) "None" (`self.ImpactPoint`) _returnvalue_3 "KeepWorldPosition" 2.5))
      (`DecalComponent.SetFadeOut` _returnvalue_5 0.0 2.5 false)
      (else
        (bind _returnvalue_6 (`GameplayStatics.SpawnDecalAtLocation` "/Game/ZEPHYR/TurretPack/Materials/Projectiles/M_Decal_BulletHole.M_Decal_BulletHole" (10.0 10.0 10.0) _impactpoint_3 _returnvalue_2 10.0))
        (`DecalComponent.SetFadeOut` _returnvalue_6 5.0 5.0 false)
        (bind _returnvalue_7 (`GameplayStatics.SpawnDecalAtLocation` "/Game/ZEPHYR/TurretPack/Materials/Projectiles/M_Decal_BulletHeat.M_Decal_BulletHeat" (10.0 10.0 10.0) _impactpoint_3 _returnvalue_2 2.5))
        (`DecalComponent.SetFadeOut` _returnvalue_7 0.0 2.5 false)))
    (`self.K2_DestroyActor`)
    (`GameplayStatics.ApplyDamage` (`self.HitActor`) (`self.Damage`))))

(fn `UserConstructionScript`
  (bind _sm_bullet (`self.SM_Bullet`))
  (bind _color (`self.Color`))
  ;[1 1 1] Change Projectile Color
  (set `ProjectileMovementComponent.InitialSpeed` (* (`self.Speed`) (`KismetMathLibrary.RandomFloatInRange` 0.9 1.1)) (`self.Projectile`))
  (bind _returnvalue (`PrimitiveComponent.CreateDynamicMaterialInstance` _sm_bullet 0 (`PrimitiveComponent.GetMaterial` _sm_bullet 0) "None"))
  (`MaterialInstanceDynamic.SetVectorParameterValue` _returnvalue "Color" _color)
  (`LightComponent.SetLightColor` (`self.PointLight`) _color true)
  (`PrimitiveComponent.SetMaterial` _sm_bullet 0 _returnvalue))